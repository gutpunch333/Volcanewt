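; Birthday cake boss enemy: a three-tier turret tank that shoots BP_TurretBullet at the nearest visible BP_Volcanewt.
; Each tick it picks a target by sphere overlap and line of sight, then turns each tier at its own speed with pitch-clamped barrels.
; Each tier fires once its cooldown ends and a dot product shows it faces the target.
; Non-EnemyUnit damage lowers health, destroying top and middle tier bodies at thresholds; the death branch is empty.
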(event `self.ReceiveBeginPlay`
  (set `self.CurrentHealth` (`self.MaxHealth`)))

(event `self.ReceiveTick`
  (params (DeltaSeconds :type "Float (single-precision)"))
  ;[1 1 1] Rotates to player and fires turrets
  (`self.FindTarget`)
  (`self.Target`
    (:`then`
      (`self.UpdateBottomTurretRotation` DeltaSeconds)
      (`self.UpdateFireBottom`)
      (`self.UpdateMiddleTurretRotation` DeltaSeconds)
      (`self.UpdateFireMiddle`)
      (`self.UpdateTopTurretRotation` DeltaSeconds)
      (`self.UpdateFireTop`)
      (`KismetSystemLibrary.PrintString` (`KismetStringLibrary.Conv_DoubleToString` (`self.CurrentHealth`))))
    (:`else`)))

(event `FireTop`
  ;[1 1 1] Fire each turret
  (set `self.TimeOfLastFireTop` (`KismetSystemLibrary.GetGameTimeInSeconds`))
  (`|SpawnActorFromClass` "/Game/Enemies/ProjectilesEtc/BP_TurretBullet.BP_TurretBullet_C" (`SceneComponent.K2_GetComponentToWorld` (`self.TopLayerFirePoint1`)) "AlwaysSpawn" "MultiplyWithRoot" null null)
  (`|SpawnActorFromClass` "/Game/Enemies/ProjectilesEtc/BP_TurretBullet.BP_TurretBullet_C" (`SceneComponent.K2_GetComponentToWorld` (`self.TopFireLocationL`)) "AlwaysSpawn" "MultiplyWithRoot" null null))

(event `self.ReceiveAnyDamage`
  (params (Damage :type "Float (single-precision)") (DamageType :type "DamageType Object Reference") (InstigatedBy :type "Controller Object Reference") (DamageCauser :type "Actor Object Reference"))
  ;[1 1 1] Boss health manager
  (if (not (`self.ActorHasTag` DamageCauser "EnemyUnit"))
    (set `self.CurrentHealth` (- (`self.CurrentHealth`) Damage))
    (if (<= (`self.CurrentHealth`) 1250.0)
      (`ActorComponent.K2_DestroyComponent` (`self.Tank_body_layer3_low`)))
    (if (<= (`self.CurrentHealth`) 500.0)
      (`ActorComponent.K2_DestroyComponent` (`self.Tank_body_layer2_low`)))
    (if (<= (`self.CurrentHealth`) 0.0)
      _)))

(event `FireMiddle`
  ;[1 1 1] Fire each turret
  (set `self.TimeOfLastFireMid` (`KismetSystemLibrary.GetGameTimeInSeconds`))
  (`GameplayStatics.PlaySoundAtLocation` "/Game/Audio/SoundEffects/shootFree.shootFree" (`self.K2_GetActorLocation`) (struct) 1.0 1.0 0.0 null null null null)
  (`|SpawnActorFromClass` "/Game/Enemies/ProjectilesEtc/BP_TurretBullet.BP_TurretBullet_C" (`SceneComponent.K2_GetComponentToWorld` (`self.MiddleLayerFirePoint`)) "AlwaysSpawn" "MultiplyWithRoot" null null))

(event `FireBottom`
  ;[1 1 1] Fire each turret
  (set `self.TimeOfLastFireBottom` (`KismetSystemLibrary.GetGameTimeInSeconds`))
  (`GameplayStatics.PlaySoundAtLocation` "/Game/Audio/SoundEffects/shootFree.shootFree" (`self.K2_GetActorLocation`) (struct) 1.0 1.0 0.0 null null null null)
  (`|SpawnActorFromClass` "/Game/Enemies/ProjectilesEtc/BP_TurretBullet.BP_TurretBullet_C" (`SceneComponent.K2_GetComponentToWorld` (`self.BottomLayerFirePoint`)) "AlwaysSpawn" "MultiplyWithRoot" null null))

(fn `FindTarget`
  (locals (BestDistance :type "Float (double-precision)") (CurrentDistance :type "Float (double-precision)") (BestTarget :type "Actor Object Reference") (CurrentTarget :type "Actor Object Reference"))
  ;[1 1 1] Determines best target and ensures it can be seen
  (set `local.BestDistance` (+ (`self.SensingRange`) 1.0))
  (bind _outactors (`KismetSystemLibrary.SphereOverlapActors` (`self.K2_GetActorLocation`) (`self.SensingRange`) (`|MakeArray` "ObjectTypeQuery3" :!type "EObjectTypeQuery Enum") "/Game/Player/BP_Volcanewt.BP_Volcanewt_C"))
  (for _array_element _outactors
    (bind _output_get (set `local.CurrentTarget` _array_element))
    (bind _output_get_2 (set `local.CurrentDistance` (`self.GetDistanceTo` _output_get self)))
    (if (or (< _output_get_2 (`local.BestDistance`)) (not (`KismetSystemLibrary.IsValid` (`local.BestTarget`))))
      (bind _result (`/Game/Blueprints/Libraries_and_Interfaces/MuhFunctionLibrary.HasLineOfSight` (`SceneComponent.K2_GetComponentLocation` (`self.Tank_body_layer_1_low`)) (`self.K2_GetActorLocation` (`local.CurrentTarget`)) (`|MakeArray` self (`local.CurrentTarget`) :!type "Actor Object Reference")))
      (if _result
        (set `local.BestTarget` (`local.CurrentTarget`))
        (set `local.BestDistance` (`local.CurrentDistance`)))))
  (set `self.Target` (`local.BestTarget`)))

(fn `UpdateBottomTurretRotation`
  (params (DeltaSeconds :type "Float (double-precision)"))
  (locals (NewRotation :type "Rotator Structure" :default (struct)) (NewRotationBarrelBot :type "Rotator Structure" :default (struct)))
  ;[1 1 1] Turret rotation (left and right only)
  (bind _output_get (set `local.NewRotation` (`KismetMathLibrary.RInterpTo_Constant` (`SceneComponent.K2_GetComponentRotation` (`self.Tank_body_layer_1_low`)) (`KismetMathLibrary.FindLookAtRotation` (`SceneComponent.K2_GetComponentLocation` (`self.Tank_body_layer_1_low`)) (`self.K2_GetActorLocation` (`self.Target`))) (`local.DeltaSeconds`) (`self.BottomRotationSpeed`))))
  (`SceneComponent.K2_SetWorldRotation` (`self.Tank_body_layer_1_low`) (`KismetMathLibrary.MakeRotator` (.roll _output_get) (`KismetMathLibrary.ClampAngle` (.pitch _output_get)) (.yaw _output_get)) false false)
  ;[1 1 1] Barrel rotation (up and down only)
  (bind _output_get_2 (set `local.NewRotationBarrelBot` (`KismetMathLibrary.RInterpTo_Constant` (`SceneComponent.K2_GetComponentRotation` (`self.Tank_layer1_cannon_low`)) (`KismetMathLibrary.FindLookAtRotation` (`SceneComponent.K2_GetComponentLocation` (`self.Tank_layer1_cannon_low`)) (`self.K2_GetActorLocation` (`self.Target`))) (`local.DeltaSeconds`) (`self.BottomRotationSpeed`))))
  (`SceneComponent.K2_SetWorldRotation` (`self.Tank_layer1_cannon_low`) (`KismetMathLibrary.MakeRotator` (.pitch _output_get) (`KismetMathLibrary.ClampAngle` (.pitch _output_get_2) -45.0 45.0) (.yaw _output_get)) false false))

(fn `UpdateFireBottom`
  ;[1 1 1 1 24] Checks if turret has cooldown and is facing target, fires if both are true
  (if (> (- (`KismetSystemLibrary.GetGameTimeInSeconds`) (`self.TimeOfLastFireBottom`)) (`self.RateOfFireBottom`))
    (if (> (`KismetMathLibrary.Dot_VectorVector` (`KismetMathLibrary.GetDirectionUnitVector` (`SceneComponent.K2_GetComponentLocation` (`self.Tank_body_layer_1_low`)) (`self.K2_GetActorLocation` (`self.Target`))) (`SceneComponent.GetForwardVector` (`self.Tank_body_layer_1_low`))) 0.99)
      (`self.FireBottom`)
      (`KismetSystemLibrary.PrintString` "Firing bottom"))))

(fn `UpdateFireMiddle`
  ;[1 1 1 1 24] Checks if turret has cooldown and is facing target, fires if both are true
  (if (> (- (`KismetSystemLibrary.GetGameTimeInSeconds`) (`self.TimeOfLastFireMid`)) (`self.RateOfFireMid`))
    (if (> (`KismetMathLibrary.Dot_VectorVector` (`KismetMathLibrary.GetDirectionUnitVector` (`SceneComponent.K2_GetComponentLocation` (`self.Tank_body_layer2_low`)) (`self.K2_GetActorLocation` (`self.Target`))) (`SceneComponent.GetForwardVector` (`self.MiddleTurretRotation`))) 0.99)
      (`self.FireMiddle`)
      (`KismetSystemLibrary.PrintString` "Firing mid"))))

(fn `UpdateFireTop`
  ;[1 1 1 1 24] Checks if turret has cooldown and is facing target, fires if both are true
  (if (> (- (`KismetSystemLibrary.GetGameTimeInSeconds`) (`self.TimeOfLastFireTop`)) (`self.RateOfFireTop`))
    (if (> (`KismetMathLibrary.Dot_VectorVector` (`KismetMathLibrary.GetDirectionUnitVector` (`SceneComponent.K2_GetComponentLocation` (`self.Tank_body_layer3_low`)) (`self.K2_GetActorLocation` (`self.Target`))) (`SceneComponent.GetForwardVector` (`self.Tank_body_layer3_low`))) 0.99)
      (`self.FireTop`)
      (`KismetSystemLibrary.PrintString` "Firing top "))))

(fn `UpdateMiddleTurretRotation`
  (params (DeltaSeconds :type "Float (double-precision)"))
  (locals (NewRotation :type "Rotator Structure" :default (struct)) (NewRotationBarrel :type "Rotator Structure" :default (struct)))
  ;[1 1 1] Comment
  (bind _output_get (set `local.NewRotation` (`KismetMathLibrary.RInterpTo_Constant` (`SceneComponent.K2_GetComponentRotation` (`self.Tank_body_layer2_low`)) (`KismetMathLibrary.FindLookAtRotation` (`SceneComponent.K2_GetComponentLocation` (`self.Tank_body_layer2_low`)) (`self.K2_GetActorLocation` (`self.Target`))) (`local.DeltaSeconds`) (`self.MiddleRotationSpeed`))))
  (`SceneComponent.K2_SetWorldRotation` (`self.Tank_body_layer2_low`) (`KismetMathLibrary.MakeRotator` (.roll _output_get) (`KismetMathLibrary.ClampAngle` (.pitch _output_get)) (.yaw _output_get)) false false)
  ;[1 1 1] Barrel rotation (up and down only)
  (bind _output_get_2 (set `local.NewRotationBarrel` (`KismetMathLibrary.RInterpTo_Constant` (`SceneComponent.K2_GetComponentRotation` (`self.Tank_cannon_layer2_low`)) (`KismetMathLibrary.FindLookAtRotation` (`SceneComponent.K2_GetComponentLocation` (`self.Tank_cannon_layer2_low`)) (`self.K2_GetActorLocation` (`self.Target`))) (`local.DeltaSeconds`) (`self.MiddleRotationSpeed`))))
  (`SceneComponent.K2_SetWorldRotation` (`self.Tank_cannon_layer2_low`) (`KismetMathLibrary.MakeRotator` (.roll _output_get) (`KismetMathLibrary.ClampAngle` (.pitch _output_get_2) -45.0 45.0) (.yaw _output_get)) false false))

(fn `UpdateTopTurretRotation`
  (params (DeltaSeconds :type "Float (double-precision)"))
  (locals (NewRotation :type "Rotator Structure" :default (struct)) (NewRotationBarrels :type "Rotator Structure" :default (struct)))
  (bind _tank_turret_low (`self.Tank_turret_low`))
  ;[1 1 1] Turret rotation (left and right)
  (bind _output_get (set `local.NewRotation` (`KismetMathLibrary.RInterpTo_Constant` (`SceneComponent.K2_GetComponentRotation` (`self.Tank_body_layer3_low`)) (`KismetMathLibrary.FindLookAtRotation` (`SceneComponent.K2_GetComponentLocation` (`self.Tank_body_layer3_low`)) (`self.K2_GetActorLocation` (`self.Target`))) (`local.DeltaSeconds`) (`self.TopRotationSpeed`))))
  (`SceneComponent.K2_SetWorldRotation` (`self.Tank_body_layer3_low`) (`KismetMathLibrary.MakeRotator` (.roll _output_get) (`KismetMathLibrary.ClampAngle` (.pitch _output_get)) (.yaw _output_get)) false false)
  ;[1 1 1] Barrel rotation (up and down only)
  (bind _output_get_2 (set `local.NewRotationBarrels` (`KismetMathLibrary.RInterpTo_Constant` (`SceneComponent.K2_GetComponentRotation` _tank_turret_low) (`KismetMathLibrary.FindLookAtRotation` (`SceneComponent.K2_GetComponentLocation` _tank_turret_low) (`self.K2_GetActorLocation` (`self.Target`))) (`local.DeltaSeconds`) (`self.TopRotationSpeed`))))
  (`SceneComponent.K2_SetWorldRotation` (`self.TopLayerFirePoint1`) (`KismetMathLibrary.MakeRotator` (.roll _output_get) (`KismetMathLibrary.ClampAngle` (.pitch _output_get_2) -45.0 45.0) (.yaw _output_get)) false false)
  (`SceneComponent.K2_SetWorldRotation` (`self.TopLayerFirePoint2`) (`KismetMathLibrary.MakeRotator` (.roll _output_get) (`KismetMathLibrary.ClampAngle` (.pitch _output_get_2) -45.0 45.0) (.yaw _output_get)) false false)
  (`SceneComponent.K2_SetWorldRotation` (`self.TopLayerFirePoint3`) (`KismetMathLibrary.MakeRotator` (.roll _output_get) (`KismetMathLibrary.ClampAngle` (.pitch _output_get_2) -45.0 45.0) (.yaw _output_get)) false false)
  (`SceneComponent.K2_SetWorldRotation` (`self.TopLayerFirePoint4`) (`KismetMathLibrary.MakeRotator` (.roll _output_get) (`KismetMathLibrary.ClampAngle` (.pitch _output_get_2) -45.0 45.0) (.yaw _output_get)) false false)
  (`SceneComponent.K2_SetWorldRotation` (`self.TopLayerFirePoint5`) (`KismetMathLibrary.MakeRotator` (.roll _output_get) (`KismetMathLibrary.ClampAngle` (.pitch _output_get_2) -45.0 45.0) (.yaw _output_get)) false false)
  (`SceneComponent.K2_SetWorldRotation` (`self.TopLayerFirePoint6`) (`KismetMathLibrary.MakeRotator` (.roll _output_get) (`KismetMathLibrary.ClampAngle` (.pitch _output_get_2) -45.0 45.0) (.yaw _output_get)) false false))

(fn `UserConstructionScript`)