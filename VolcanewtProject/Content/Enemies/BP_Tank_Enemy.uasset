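; Tank enemy that chases and shoots at the Volcanewt player and is destroyed by any damage.
; Pawn sensing sets an AI blackboard flag once the player is seen.
; AttackPlayer sphere-traces forward and, if it hits the player, spawns a projectile at the spawn point with a shot sound.
; Taking damage plays a boom, reports the enemy's monetary value to the game mode and destroys the actor.
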(event `self.ReceiveAnyDamage`
  (params (Damage :type "Float (single-precision)") (DamageType :type "DamageType Object Reference") (InstigatedBy :type "Controller Object Reference") (DamageCauser :type "Actor Object Reference"))
  ;[1 1 1 1 100] Destroys Enemy
  (`GameplayStatics.PlaySoundAtLocation` "/Game/Audio/SoundEffects/stompBoom.stompBoom" (`self.K2_GetActorLocation`) (struct) 0.4 1.1 0.15 null null null null)
  (bind _asbpgm_volcanewt (cast `/Game/Blueprints/BPGM_Volcanewt` (`GameplayStatics.GetGameMode`)))
  (`/Game/Blueprints/BPGM_Volcanewt.EnemyDestroyed` _asbpgm_volcanewt (`self.EnemyMonetaryValue`))
  (`self.K2_DestroyActor`))

(event `self.PawnSensing.OnSeePawn`
  (params (Pawn :type "Pawn Object Reference"))
  ;[1 1 1 1 30] On seeing the player, follow them (copied from basic/helicopter enemy script)
  (cast `/Game/Player/BP_Volcanewt` Pawn)
  (`BlackboardComponent.SetValueAsBool` (`AIBlueprintHelperLibrary.GetBlackboard` (`AIBlueprintHelperLibrary.GetAIController` self)) "hasSeenPlayer?" true))

(event `AttackPlayer`
  (bind _returnvalue (`self.K2_GetActorLocation`))
  ;[1 1 1] Enemy attack code (same used in helicopter enemy)
  ;;[1 1 1] Radius for attacking player
  (bind (_outhit _returnvalue_2) (`KismetSystemLibrary.SphereTraceSingleForObjects` _returnvalue (+ _returnvalue (* (`KismetMathLibrary.GetForwardVector` (`self.K2_GetActorRotation`)) 1500.0)) 400.0 (`|MakeArray` "ObjectTypeQuery3" :!type "EObjectTypeQuery Enum")))
  (if _returnvalue_2
    (cast `/Game/Player/BP_Volcanewt` (`.HitActor` (`GameplayStatics.BreakHitResult` _outhit)))
    (`GameplayStatics.PlaySoundAtLocation` "/Game/Audio/SoundEffects/shootFree.shootFree" (`self.K2_GetActorLocation`) (struct) 1.0 1.0 0.0 null null null null)
    (`|SpawnActorFromClass` "/Game/Enemies/ProjectilesEtc/TestProjectile.TestProjectile_C" (`SceneComponent.K2_GetComponentToWorld` (`self.spawn proj loc`)) "AlwaysSpawn" "MultiplyWithRoot" null null)))

(fn `UserConstructionScript`)