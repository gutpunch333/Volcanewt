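; Enemy bus actor that drives along a randomly chosen BP_Road spline.
; On BeginPlay it hides its cube, picks one road from all BP_Road actors, then shows itself and opens a movement gate after a random delay under a second.
; Tick advances its distance by the road's RoadSpeed, snaps location and rotation to the spline, and wraps to zero past the end.
; DestroyBus removes the actor.
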(event `DestroyBus`
  (`self.K2_DestroyActor`))

(event `Attach To Road`
  (bind _allroadsarray (`self.AllRoadsArray`))
  ;[0.3297 0.3626 1] Getting a random road from the array and attaching self to it
  (bind _asbp_road (cast `/Game/Blueprints/BP_Road` (`|GetArrayItem` _allroadsarray (`KismetMathLibrary.RandomInteger` (`KismetArrayLibrary.Array_Length` _allroadsarray)))))
  (set `self.RoadRef` _asbp_road))

(event `self.ReceiveBeginPlay`
  ;[0.3297 0.3626 1] Settting invisible, Getting all roads, creating an array of them, then calling Attach to Road
  (`SceneComponent.SetVisibility` (`self.Cube`) false false)
  (bind _outactors (`GameplayStatics.GetAllActorsOfClass` "/Game/Blueprints/BP_Road.BP_Road_C"))
  (set `self.AllRoadsArray` _outactors)
  (`self.Attach To Road`)
  (set `self.StartingBusDistance` 0.0) ; When spawning, likely need to find the nearest point on the spline to the player, and set the starting distane to that. Else, the Bus may immediately respawn
  ;[1 0.381 0.09741] Randomized begin movement timing
  (`KismetSystemLibrary.Delay` (`KismetMathLibrary.RandomFloatInRange` 0.0 1.0))
  (`self.UnlockMovement`))

(event `self.ReceiveTick`
  (params (DeltaSeconds :type "Float (single-precision)"))
  (bind _roadref (`self.RoadRef`))
  (bind (_returnvalue_location _returnvalue_rotation) (`KismetMathLibrary.BreakTransform` (`SplineComponent.GetTransformAtDistanceAlongSpline` (`/Game/Blueprints/BP_Road.Spline` _roadref) (`self.BusDistance`) "World" false)))
  ;[0.2838 1 0.2025] Per tick, updating the distance of the bus along the associated road spline
  (`/Engine/EditorBlueprintResources/StandardMacros.Gate` true :!label _label
    (:`Exit`
      (set `self.BusDistance` (+ (* DeltaSeconds (`/Game/Blueprints/BP_Road.RoadSpeed` _roadref)) (`self.BusDistance`)))
      (`self.K2_SetActorTransform` (`KismetMathLibrary.MakeTransform` _returnvalue_location _returnvalue_rotation))
      ;[0.2838 1 0.2025] If bus beyond the end of the spline, reset it to the start of the spline
      (if (> (`self.BusDistance`) (`SplineComponent.GetSplineLength` (`/Game/Blueprints/BP_Road.Spline` (`self.RoadRef`))))
        (set `self.BusDistance` 0.0)))))

(event `UnlockMovement`
  ;[1 0.381 0.09741] Sets bus visible and opens movement gate
  (`SceneComponent.SetVisibility` (`self.Cube`) true false)
  (goto _label :!via `Open`))

(fn `UserConstructionScript`)