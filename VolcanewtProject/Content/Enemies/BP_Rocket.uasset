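; Homing rocket projectile that chases actors tagged "Newt" and destroys itself on a hit or after about seven seconds.
; BeginPlay re-runs LockOn every half second, feeding FindHomingTarget's closest match to the projectile movement and a Niagara target parameter.
; The search keeps its best distance between calls, so the target switches only for a closer distance.
; Hit applies damage only when the hit component compares equal to the player pawn.
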(event `self.ReceiveHit`
  (params (MyComp :type "PrimitiveComponent Object Reference") (Other :type "Actor Object Reference") (OtherComp :type "PrimitiveComponent Object Reference") (bSelfMoved :type Boolean) (HitLocation :type "Vector Structure") (HitNormal :type "Vector Structure") (NormalImpulse :type "Vector Structure") (Hit :type "HitResult Structure (by ref)"))
  (if (== OtherComp (`GameplayStatics.GetPlayerPawn` 0))
    (`KismetSystemLibrary.Delay` 0.1)
    (`GameplayStatics.ApplyDamage` Other 25.0)
    (`self.K2_DestroyActor`)
    (else
      (`self.K2_DestroyActor`))))

(event `self.Sphere.OnComponentHit`
  (params (HitComponent :type "PrimitiveComponent Object Reference") (OtherActor :type "Actor Object Reference") (OtherComp :type "PrimitiveComponent Object Reference") (NormalImpulse :type "Vector Structure") (Hit :type "HitResult Structure (by ref)"))
  (`KismetSystemLibrary.PrintString` "Ouchie"))

(event `Lock On`
  (bind _homingtarget (`self.Find Homing Target`))
  (set `ProjectileMovementComponent.HomingTargetComponent` _homingtarget (`self.ProjectileMovement`))
  (`GameplayStatics.GetAllActorsOfClass` "/Game/Player/BP_Volcanewt.BP_Volcanewt_C")
  (`NiagaraComponent.SetVariableVec3` (`self.Niagara`) "Target" (`SceneComponent.K2_GetComponentLocation` _homingtarget))
  (`KismetSystemLibrary.Delay` 7.0)
  (`self.K2_DestroyActor`))

(event `self.ReceiveBeginPlay`
  (`self.Lock On` :!label _label)
  (`KismetSystemLibrary.Delay` 0.5)
  (goto _label))

(fn `Find Homing Target`
  (returns (HomingTarget :type "SceneComponent Object Reference"))
  (bind _outactors (`GameplayStatics.GetAllActorsOfClassWithTag` "/Script/Engine.Actor" "Newt"))
  (for _array_element _outactors
    (bind _returnvalue (`KismetMathLibrary.VSize` (- (`self.K2_GetActorLocation` _array_element) (`self.K2_GetActorLocation`))))
    (if (< _returnvalue (`self.NewtDistance`))
      (set `self.NewtDistance` _returnvalue)
      (set `self.HomingTarget` _array_element)))
  (return (`self.GetComponentByClass` (`self.HomingTarget`) "/Script/Engine.SceneComponent")))

(fn `UserConstructionScript`)