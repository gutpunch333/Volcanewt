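; BP_NC3_SquadSpawn is an enemy spawner that creates a squad of soldiers at its own location.
; BeginPlay starts a fast looping timer that increments NumSoldiers with each spawn, choosing regular soldiers first, then laser soldiers, up to a fixed cap.
; The rocket soldier branch is unreachable behind the laser threshold check.
; Reaching the cap only clears the Looping variable, leaving the timer itself running.
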(event `self.ReceiveBeginPlay`
  (bind _output_get (set `self.Looping` true))
  (`KismetSystemLibrary.K2_SetTimerDelegate` (delegate `Spawn Enemy`) 0.1 _output_get))

(event `Spawn Enemy`
  (if (>= (`self.NumSoldiers`) 13)
    (set `self.Looping` false)
    (elif (>= (`self.NumSoldiers`) 8)
      (`|SpawnActorFromClass` "/Game/Enemies/BP_LaserSoldier.BP_LaserSoldier_C" (`KismetMathLibrary.Conv_VectorToTransform` (`self.K2_GetActorLocation`)) "Undefined" "MultiplyWithRoot" null null)
      (`/Engine/EditorBlueprintResources/StandardMacros.IncrementInt` (`self.NumSoldiers`))
      (elif (>= (`self.NumSoldiers`) 9)
        (`|SpawnActorFromClass` "/Game/Enemies/BP_RocketSoldier.BP_RocketSoldier_C" (`KismetMathLibrary.Conv_VectorToTransform` (`self.K2_GetActorLocation`)) "Undefined" "MultiplyWithRoot" null null)
        (`/Engine/EditorBlueprintResources/StandardMacros.IncrementInt` (`self.NumSoldiers`))
        (else
          (`|SpawnActorFromClass` "/Game/Enemies/BP_Soldier.BP_Soldier_C" (`KismetMathLibrary.Conv_VectorToTransform` (`self.K2_GetActorLocation`)) "Undefined" "MultiplyWithRoot" null null)
          (`/Engine/EditorBlueprintResources/StandardMacros.IncrementInt` (`self.NumSoldiers`)))))))

(fn `UserConstructionScript`)