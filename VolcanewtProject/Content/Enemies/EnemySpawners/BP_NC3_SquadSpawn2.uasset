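; BP_NC3_SquadSpawn2 is an enemy spawner that fills a fixed mixed squad of basic, laser and rocket soldiers at its own location.
; BeginPlay starts a very short looping timer whose each tick spawns one of each type still under its individual cap.
; At the squad total it only clears the Looping variable, so the timer itself is never cleared and keeps firing without spawning.
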(event `self.ReceiveBeginPlay`
  (bind _output_get (set `self.Looping` true))
  (`KismetSystemLibrary.K2_SetTimerDelegate` (delegate `Spawn Enemy`) 0.001 _output_get))

(event `Spawn Enemy`
  (if (>= (`self.NumSoldiers`) 13)
    (set `self.Looping` false)
    (else
      (`|ExecutionSequence`
        (:`then_0`
          (if (not (>= (`self.NumBasics`) 5))
            (`|SpawnActorFromClass` "/Game/Enemies/BP_Soldier.BP_Soldier_C" (`KismetMathLibrary.Conv_VectorToTransform` (`self.K2_GetActorLocation`)) "Undefined" "MultiplyWithRoot" null null)
            (`/Engine/EditorBlueprintResources/StandardMacros.IncrementInt` (`self.NumSoldiers`)
              (:`  `
                (`/Engine/EditorBlueprintResources/StandardMacros.IncrementInt` (`self.NumBasics`))))))
        (:`then_1`
          (if (not (>= (`self.NumLasers`) 3))
            (`|SpawnActorFromClass` "/Game/Enemies/BP_LaserSoldier.BP_LaserSoldier_C" (`KismetMathLibrary.Conv_VectorToTransform` (`self.K2_GetActorLocation`)) "Undefined" "MultiplyWithRoot" null null)
            (`/Engine/EditorBlueprintResources/StandardMacros.IncrementInt` (`self.NumSoldiers`)
              (:`  `
                (`/Engine/EditorBlueprintResources/StandardMacros.IncrementInt` (`self.NumLasers`))))))
        (:`then_2`
          (if (not (>= (`self.NumRockets`) 6))
            (`|SpawnActorFromClass` "/Game/Enemies/BP_RocketSoldier.BP_RocketSoldier_C" (`KismetMathLibrary.Conv_VectorToTransform` (`self.K2_GetActorLocation`)) "Undefined" "MultiplyWithRoot" null null)
            (`/Engine/EditorBlueprintResources/StandardMacros.IncrementInt` (`self.NumSoldiers`)
              (:`  `
                (`/Engine/EditorBlueprintResources/StandardMacros.IncrementInt` (`self.NumRockets`))))))))))

(fn `UserConstructionScript`)