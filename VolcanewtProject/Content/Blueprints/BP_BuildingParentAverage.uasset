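; Parent Blueprint for a destructible building that carries a monetary value and crumbles when its health runs out.
; Any damage spawns a money UI actor, then reduces remaining health with a Niagara hit effect.
; At zero health it notifies BPGM_Volcanewt, removes the static mesh, crumbles the physics-enabled Geometry Collection and plays a sound.
; Construction sets health and dynamic materials, but the timeline fade-out and actor destroy are unconnected.
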(event `self.ReceiveBeginPlay`
  (set `self.TotalHealth` (`self.Current Health`)))

(event `self.ReceiveAnyDamage`
  (params (Damage :type "Float (single-precision)") (DamageType :type "DamageType Object Reference") (InstigatedBy :type "Controller Object Reference") (DamageCauser :type "Actor Object Reference"))
  (bind _current_health (`self.Current Health`))
  (bind _gc_component (`self.GC_Component`))
  (bind _returnvalue (<= _current_health 0.0))
  ;[1 1 1] Checks if the building has any health, if above 0 itlll do damage stuff
  (`self.SpawnMoneyUI`)
  (if (not _returnvalue)
    (set `self.Current Health` (- _current_health Damage))
    (`/Game/Blueprints/Libraries_and_Interfaces/MuhFunctionLibrary.SpawnNiagaraAtActor` self "/Game/Textures/NPS_BuildingDamage.NPS_BuildingDamage")
    (if _returnvalue
      (bind _asbpgm_volcanewt (cast `/Game/Blueprints/BPGM_Volcanewt` (`GameplayStatics.GetGameMode`)))
      (`/Game/Blueprints/BPGM_Volcanewt.BuildingDestroyed` _asbpgm_volcanewt (`self.MonetaryValue`) self)
      (`ActorComponent.K2_DestroyComponent` (`self.Static Mesh Component`))
      ;[1 1 1] Sets physics to mesh and breaks apart the separate geometry mesh
      (`PrimitiveComponent.SetSimulatePhysics` _gc_component true)
      (`GeometryCollectionComponent.CrumbleCluster` _gc_component 0)
      (`GeometryCollectionComponent.CrumbleCluster` _gc_component 1)
      ;[1 1 1] Sound :)
      (`GameplayStatics.PlaySoundAtLocation` (`self.Destuction SFX`) (`self.K2_GetActorLocation`) (struct) 1.0 1.0 0.0 null null null null))))

(event `SpawnMoneyUI`
  (bind _returnvalue_location (`KismetMathLibrary.BreakTransform` (`self.GetTransform`)))
  ;[1 1 1] Spawn Money UI
  (`|SpawnActorFromClass` "/Game/Blueprints/BP_MoneyUISpawner.BP_MoneyUISpawner_C" (`KismetMathLibrary.MakeTransform` (+ _returnvalue_location (0.0 0.0 10.0))) "AlwaysSpawn" "MultiplyWithRoot" null (`self.MonetaryValue`) (`KismetMathLibrary.FTrunc` (stale `self.ReceiveAnyDamage` Damage)) (`KismetMathLibrary.FTrunc` (`self.TotalHealth`)) (`KismetMathLibrary.FTrunc` (`self.Current Health`)) null))

(fn `UserConstructionScript`
  (bind _max_health (`self.Max Health`))
  (bind _gc_component (`self.GC_Component`))
  (bind _returnvalue (`PrimitiveComponent.CreateDynamicMaterialInstance` _gc_component 1 "/Game/Enemies/EnemyAssets/lambert1.lambert1" "None"))
  (set `self.DynamicMaterialInstanceIndex1` _returnvalue)
  (bind _returnvalue_2 (`PrimitiveComponent.CreateDynamicMaterialInstance` _gc_component 0 "/Game/Enemies/EnemyAssets/lambert1.lambert1" "None"))
  (set `self.DynamicMaterialInstanceIndex0` _returnvalue_2)
  (set `self.Current Health` _max_health)
  (set `self.TotalHealth` _max_health))