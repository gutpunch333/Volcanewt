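; Destructible apartment building actor that loses health on damage, crumbling a Geometry Collection and spawning damage particles.
; Construction registers Chaos master and anchor fields; each non-lethal hit lowers the anchor with remaining health and re-crumbles the cluster.
; When another equal hit would deplete health, it reports its monetary value to the Volcanewt GameMode, plays rubble sound, fades dynamic materials via timeline, then destroys itself.
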(event `self.ReceiveBeginPlay`
  (set `self.bCanBeDamaged` true)
  (bind _asbpgm_volcanewt (cast `/Game/Blueprints/BPGM_Volcanewt` (`GameplayStatics.GetGameMode`)))
  (set `self.As BPGM Volcanewt` _asbpgm_volcanewt)
  ;[1 1 1] A variable consistent across all building actors is established
  (bind _asbp_building_parent (cast `/Game/Blueprints/BP_BuildingParent` (`ChildActorComponent.ChildActor` (`self.BP_BuildingParent`))))
  (set `/Game/Blueprints/BP_BuildingParent.MonetaryValue` (`self.ApartmentBuildingMV`) _asbp_building_parent))

(event `self.ReceiveAnyDamage`
  (params (Damage :type "Float (single-precision)") (DamageType :type "DamageType Object Reference") (InstigatedBy :type "Controller Object Reference") (DamageCauser :type "Actor Object Reference"))
  (bind _returnvalue (- (`self.SmallBuildingHealth`) Damage))
  (bind _returnvalue_2 (<= _returnvalue 0.0))
  ;[1 1 1] Checks if the building has any health, if above 0 itlll do damage stuff
  (if (not _returnvalue_2)
    (set `self.SmallBuildingHealth` _returnvalue)
    (`self.DecreaseBuildingStructure` 0.0)
    (`/Game/Blueprints/Libraries_and_Interfaces/MuhFunctionLibrary.SpawnNiagaraAtActor` self "/Game/Textures/NPS_BuildingDamage.NPS_BuildingDamage")
    (if _returnvalue_2
      (bind _asbpgm_volcanewt (cast `/Game/Blueprints/BPGM_Volcanewt` (`GameplayStatics.GetGameMode`)))
      (`/Game/Blueprints/BPGM_Volcanewt.BuildingDestroyed` _asbpgm_volcanewt (`self.ApartmentBuildingMV`) self)
      ;[1 1 1 1 1000] Sound :)
      (`GameplayStatics.PlaySoundAtLocation` "/Game/Audio/SoundEffects/rocks.rocks" (`self.K2_GetActorLocation`) (struct) 0.75 1.4 2.7 null null null null)
      ;;[1 1 1] Lerping the dynamic materials' parameter values to fade the building out
      (`KismetSystemLibrary.Delay` 1.0)
      (bind (_direction _fadealpha) (`Timeline|Timeline` :!via `PlayFromStart`)
        (:`Update`
          (bind _returnvalue_3 (`KismetMathLibrary.Lerp` 1.0 0.0 _fadealpha))
          (`MaterialInstanceDynamic.SetScalarParameterValue` (`self.DynamicMaterialInstanceIndex1`) "fadeOut" _returnvalue_3)
          (`MaterialInstanceDynamic.SetScalarParameterValue` (`self.DynamicMaterialInstanceIndex0`) "fadeOut" _returnvalue_3))
        (:`Finished`
          (`KismetSystemLibrary.Delay` 7.0)
          (`self.K2_DestroyActor`))))))

(event `DecreaseBuildingStructure`
  (params (Damage :type "Float (double-precision)"))
  (bind (_returnvalue_x _returnvalue_y) (`KismetMathLibrary.BreakVector` (`self.K2_GetActorLocation`)))
  (bind _initializationfields (`GeometryCollectionComponent.InitializationFields` (`self.GC_ApartmentBuilding2`)))
  (bind _returnvalue (- 500.0 (- 900.0 (* 900.0 (/ (`self.SmallBuildingHealth`) 250.0)))))
  (`PrimitiveComponent.SetSimulatePhysics` (`self.GC_ApartmentBuilding2`) true)
  (`SceneComponent.K2_SetWorldTransform` (`Actor.RootComponent` (`self.As BP Custom Anchor`)) (`KismetMathLibrary.MakeTransform` (`KismetMathLibrary.MakeVector` _returnvalue_x _returnvalue_y _returnvalue) (struct) (`self.GetActorScale3D`)) false false)
  (`KismetArrayLibrary.Array_Remove` _initializationfields 1)
  (`KismetArrayLibrary.Array_Add` _initializationfields (`self.As BP Custom Anchor`))
  (`GeometryCollectionComponent.CrumbleCluster` (`self.GC_ApartmentBuilding2`) 1)
  (`KismetSystemLibrary.PrintString` (`KismetStringLibrary.Conv_DoubleToString` _returnvalue)))

(fn `UserConstructionScript`
  (bind _gc_apartmentbuilding2 (`self.GC_ApartmentBuilding2`))
  (bind _initializationfields (`GeometryCollectionComponent.InitializationFields` (`self.GC_ApartmentBuilding2`)))
  ;[1 1 1] Creating and setting references to Dynamic Material instances
  (bind _returnvalue (`PrimitiveComponent.CreateDynamicMaterialInstance` _gc_apartmentbuilding2 1 "/Game/Buildings/lambert1.lambert1" "None"))
  (set `self.DynamicMaterialInstanceIndex1` _returnvalue)
  (bind _returnvalue_2 (`PrimitiveComponent.CreateDynamicMaterialInstance` _gc_apartmentbuilding2 0 "/Game/Buildings/lambert1.lambert1" "None"))
  (set `self.DynamicMaterialInstanceIndex0` _returnvalue_2)
  (bind _asbp_chaos_master (cast `/Game/ChaosDestruction/BP_ChaosMaster` (`ChildActorComponent.ChildActor` (`self.BP_ChaosMaster`))))
  (`KismetArrayLibrary.Array_Add` _initializationfields _asbp_chaos_master)
  ;[1 1 1] Sets the anchor field to the geometry collision component and sets a variable for the anchor field to be referenced later
  (bind _asbp_custom_anchor (cast `` (`ChildActorComponent.ChildActor` (`self.BP_CustomAnchor`)))
    (:`then`
      (bind _output_get (set `self.As BP Custom Anchor` _asbp_custom_anchor))
      (`KismetArrayLibrary.Array_Add` _initializationfields _output_get)
      (`GeometryCollectionComponent.CrumbleCluster` (`self.GC_ApartmentBuilding2`) 1))
    (:`CastFailed`
      (`KismetSystemLibrary.PrintString` "Nopers"))))