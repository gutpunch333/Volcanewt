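; BP_SmallStore is a destructible small store building in the Volcanewt game.
; On BeginPlay it caches the BPGM_Volcanewt game mode and registers itself there by its monetary value.
; Any damage reduces its health; at zero or below it reports its value and reference to the game mode as destroyed, then destroys itself.
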(event `self.ReceiveBeginPlay`
  (bind _asbpgm_volcanewt (cast `/Game/Blueprints/BPGM_Volcanewt` (`GameplayStatics.GetGameMode`)))
  (bind _output_get (set `self.As BPGM Volcanewt` _asbpgm_volcanewt))
  (`/Game/Blueprints/BPGM_Volcanewt.Register Building` _output_get (`self.SmallStoreMV`)))

(event `self.ReceiveAnyDamage`
  (params (Damage :type "Float (single-precision)") (DamageType :type "DamageType Object Reference") (InstigatedBy :type "Controller Object Reference") (DamageCauser :type "Actor Object Reference"))
  (bind _smallstorehealth (`self.SmallStoreHealth`))
  (set `self.SmallStoreHealth` (- _smallstorehealth Damage))
  (if (<= _smallstorehealth 0.0)
    (`/Game/Blueprints/BPGM_Volcanewt.BuildingDestroyed` (`self.As BPGM Volcanewt`) (`self.SmallStoreMV`) self)
    (`self.K2_DestroyActor`)))

(fn `UserConstructionScript`)