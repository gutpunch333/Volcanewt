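; BP_Pylon is a destructible pylon that controls BP_Mechanewt's health gates in the boss fight.
; When its health runs out, it disables damage on all pylons and refreshes their green-sphere indicators.
; It then uses the pylon count to open gates, lower the boss's health floor and trigger a DPS or final-stand phase before destroying itself.
; ChargeUp only refreshes the indicators, without re-enabling damage.
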(event `self.ReceiveBeginPlay`
  (bind _as_bp_mechanewt (`self.As BP Mechanewt`))
  (bind _returnvalue (`GameplayStatics.GetActorOfClass` "/Game/Blueprints/Enemies/Mechanewt/BP_Mechanewt.BP_Mechanewt_C"))
  (set `self.As BP Mechanewt` _returnvalue)
  (bind _outactors (`GameplayStatics.GetAllActorsOfClass` "BP_Pylon_C"))
  (set `self.All Pylons Array` _outactors)
  (set `/Game/Blueprints/Enemies/Mechanewt/BP_Mechanewt.HealthGate1` true _as_bp_mechanewt)
  (set `/Game/Blueprints/Enemies/Mechanewt/BP_Mechanewt.HealthGate2` true _as_bp_mechanewt)
  (set `/Game/Blueprints/Enemies/Mechanewt/BP_Mechanewt.HealthGate3` true _as_bp_mechanewt)
  (set `self.bCanBeDamaged` true)
  (`self.ColorChanger`))

(event `RemoveHealthGate`
  (bind _as_bp_mechanewt (`self.As BP Mechanewt`))
  (bind _as_bp_mechanewt_2 (`self.As BP Mechanewt`))
  (bind _as_bp_mechanewt_3 (`self.As BP Mechanewt`))
  ;[1 1 1] Removing Health Gate when Pylon is destroyed
  (if (>= (`KismetArrayLibrary.Array_Length` (`self.All Pylons Array`)) 3)
    (set `/Game/Blueprints/Enemies/Mechanewt/BP_Mechanewt.HealthGate1` false _as_bp_mechanewt_3)
    (set `/Game/Blueprints/Enemies/Mechanewt/BP_Mechanewt.HealthGate2` true _as_bp_mechanewt_3)
    (set `/Game/Blueprints/Enemies/Mechanewt/BP_Mechanewt.HealthGate3` true _as_bp_mechanewt_3)
    (set `Actor.bCanBeDamaged` true _as_bp_mechanewt_3)
    (set `/Game/Blueprints/Enemies/Mechanewt/BP_Mechanewt.HealthGateLowest` 4000.0 _as_bp_mechanewt_3)
    (`SceneComponent.SetVisibility` (`self.Capsule`) false false)
    (`/Game/Blueprints/Enemies/Mechanewt/BP_Mechanewt.DPSPhase` _as_bp_mechanewt_3)
    (`self.K2_DestroyActor`)
    (elif (== (`KismetArrayLibrary.Array_Length` (`self.All Pylons Array`)) 2)
      (set `/Game/Blueprints/Enemies/Mechanewt/BP_Mechanewt.HealthGate1` false _as_bp_mechanewt)
      (set `/Game/Blueprints/Enemies/Mechanewt/BP_Mechanewt.HealthGate2` false _as_bp_mechanewt)
      (set `/Game/Blueprints/Enemies/Mechanewt/BP_Mechanewt.HealthGate3` true _as_bp_mechanewt)
      (set `Actor.bCanBeDamaged` true _as_bp_mechanewt)
      (set `/Game/Blueprints/Enemies/Mechanewt/BP_Mechanewt.HealthGateLowest` 2000.0 _as_bp_mechanewt)
      (`SceneComponent.SetVisibility` (`self.Capsule`) false false)
      (`/Game/Blueprints/Enemies/Mechanewt/BP_Mechanewt.DPSPhase` _as_bp_mechanewt)
      (`self.K2_DestroyActor`)
      (elif (== (`KismetArrayLibrary.Array_Length` (`self.All Pylons Array`)) 1)
        (set `/Game/Blueprints/Enemies/Mechanewt/BP_Mechanewt.HealthGate1` false _as_bp_mechanewt_2)
        (set `/Game/Blueprints/Enemies/Mechanewt/BP_Mechanewt.HealthGate2` false _as_bp_mechanewt_2)
        (set `Actor.bCanBeDamaged` true _as_bp_mechanewt_2)
        (set `/Game/Blueprints/Enemies/Mechanewt/BP_Mechanewt.HealthGate3` false _as_bp_mechanewt_2)
        (set `/Game/Blueprints/Enemies/Mechanewt/BP_Mechanewt.HealthGateLowest` 0.0 _as_bp_mechanewt_2)
        (`SceneComponent.SetVisibility` (`self.Capsule`) false false)
        (`/Game/Blueprints/Enemies/Mechanewt/BP_Mechanewt.FinalStandPhase` _as_bp_mechanewt_2)
        (`self.K2_DestroyActor`)
        (else
          (`self.K2_DestroyActor`))))))

(event `self.ReceiveAnyDamage`
  (params (Damage :type "Float (single-precision)") (DamageType :type "DamageType Object Reference") (InstigatedBy :type "Controller Object Reference") (DamageCauser :type "Actor Object Reference"))
  ;[1 1 1] Health Manager
  (if (`self.bCanBeDamaged`)
    (set `self.Attacking Actor` DamageCauser)
    (bind _output_get (set `self.CurrentHealth` (- (`self.CurrentHealth`) Damage)))
    (if (<= _output_get 0.0)
      (`self.UpdatePylonCount`)
      (else
        (`KismetSystemLibrary.PrintString` (`KismetStringLibrary.Conv_DoubleToString` (`self.CurrentHealth`)))))))

(event `UpdatePylonCount`
  ;[1 1 1] Remove Pylon from Array when one is destroyed
  (bind _outactors (`GameplayStatics.GetAllActorsOfClass` "BP_Pylon_C"))
  (bind _output_get (set `self.All Pylons Array` _outactors))
  (bind _result (`/Engine/EditorBlueprintResources/StandardMacros.DecrementInt` (`KismetArrayLibrary.Array_Length` _outactors))
    (:`  `
      (for _array_element _output_get
        (set `Actor.bCanBeDamaged` false _array_element)
        (`self.ColorChanger` _array_element)
        (`KismetSystemLibrary.PrintString` (`KismetStringLibrary.Conv_IntToString` _result))
        (`KismetSystemLibrary.LogString` "Pylons"))
      (`self.RemoveHealthGate`))))

(event `ChargeUp`
  ;[1 1 1] Charge Up (when Mechanewt becomes invincible)
  (`KismetSystemLibrary.PrintString` "Invincible")
  (bind _outactors (`GameplayStatics.GetAllActorsOfClass` "BP_Pylon_C"))
  (for _array_element _outactors
    (`self.ColorChanger` _array_element)
    (`KismetSystemLibrary.PrintString` "Back to green")))

(event `ColorChanger`
  ;[1 1 1] Switches between color spheres depending on whether pylon can be damaged
  (bind _outactors (`GameplayStatics.GetAllActorsOfClass` "BP_Pylon_C"))
  (for _array_element _outactors
    (if (`Actor.bCanBeDamaged` _array_element)
      (`SceneComponent.SetVisibility` (`/Game/Blueprints/Enemies/Mechanewt/BP_Pylon.GreenSphere` _array_element) true false)
      (`KismetSystemLibrary.PrintString` "Green now")
      (else
        (`SceneComponent.SetVisibility` (`/Game/Blueprints/Enemies/Mechanewt/BP_Pylon.GreenSphere` _array_element) false false)
        (`KismetSystemLibrary.PrintString` "Red now")))))

(fn `UserConstructionScript`)