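; BP_Pylon is a destructible enemy pylon, a child actor of BP_Mechanewt, that controls that enemy's three health gates.
; On BeginPlay it enables all gates and snapshots every pylon in the level.
; Damage depleting its health sets gates by that snapshot's count, makes the Mechanewt damageable, calls HealthGates and destroys the pylon.
; UpdatePylonCount only forwards to RemoveHealthGate, so the stored count is never refreshed.
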(event `self.ReceiveBeginPlay`
  (bind _as_bp_mechanewt (`self.As BP Mechanewt`))
  (bind _asbp_mechanewt (cast `/Game/Blueprints/Enemies/BP_Mechanewt` (`self.GetParentActor`)))
  (set `self.As BP Mechanewt` _asbp_mechanewt)
  (bind _outactors (`GameplayStatics.GetAllActorsOfClass` "BP_Pylon_C"))
  (set `self.All Pylons Array` _outactors)
  (set `/Game/Blueprints/Enemies/BP_Mechanewt.HealthGate1` true _as_bp_mechanewt)
  (set `/Game/Blueprints/Enemies/BP_Mechanewt.HealthGate2` true _as_bp_mechanewt)
  (set `/Game/Blueprints/Enemies/BP_Mechanewt.HealthGate3` true _as_bp_mechanewt)
  (`KismetSystemLibrary.PrintString` (`KismetStringLibrary.Conv_IntToString` (`KismetArrayLibrary.Array_Length` (`self.All Pylons Array`))))
  (`KismetSystemLibrary.LogString` "Pylons"))

(event `RemoveHealthGate`
  (bind _as_bp_mechanewt (`self.As BP Mechanewt`))
  (bind _as_bp_mechanewt_2 (`self.As BP Mechanewt`))
  (bind _as_bp_mechanewt_3 (`self.As BP Mechanewt`))
  (bind _returnvalue (`KismetArrayLibrary.Array_Length` (`self.All Pylons Array`)))
  (bind _returnvalue_2 (`KismetArrayLibrary.Array_Length` (`self.All Pylons Array`)))
  (bind _returnvalue_3 (`KismetArrayLibrary.Array_Length` (`self.All Pylons Array`)))
  ;[1 1 1] Removing Health Gate when Pylon is destroyed
  (if (>= _returnvalue_3 3)
    (set `/Game/Blueprints/Enemies/BP_Mechanewt.HealthGate1` false _as_bp_mechanewt_3)
    (set `/Game/Blueprints/Enemies/BP_Mechanewt.HealthGate2` true _as_bp_mechanewt_3)
    (set `/Game/Blueprints/Enemies/BP_Mechanewt.HealthGate3` true _as_bp_mechanewt_3)
    (set `Actor.bCanBeDamaged` true _as_bp_mechanewt_3)
    (`/Game/Blueprints/Enemies/BP_Mechanewt.HealthGates` _as_bp_mechanewt_3)
    (`KismetSystemLibrary.PrintString` (`KismetStringLibrary.Conv_IntToString` _returnvalue_3))
    (`KismetSystemLibrary.LogString` "Pylons")
    (`self.K2_DestroyActor`)
    (elif (== _returnvalue 2)
      (set `/Game/Blueprints/Enemies/BP_Mechanewt.HealthGate1` false _as_bp_mechanewt)
      (set `/Game/Blueprints/Enemies/BP_Mechanewt.HealthGate2` false _as_bp_mechanewt)
      (set `/Game/Blueprints/Enemies/BP_Mechanewt.HealthGate3` true _as_bp_mechanewt)
      (set `Actor.bCanBeDamaged` true _as_bp_mechanewt)
      (`/Game/Blueprints/Enemies/BP_Mechanewt.HealthGates` _as_bp_mechanewt)
      (`KismetSystemLibrary.PrintString` (`KismetStringLibrary.Conv_IntToString` _returnvalue))
      (`KismetSystemLibrary.LogString` "Pylons")
      (`self.K2_DestroyActor`)
      (elif (== _returnvalue_2 1)
        (set `/Game/Blueprints/Enemies/BP_Mechanewt.HealthGate1` false _as_bp_mechanewt_2)
        (set `/Game/Blueprints/Enemies/BP_Mechanewt.HealthGate2` false _as_bp_mechanewt_2)
        (set `Actor.bCanBeDamaged` true _as_bp_mechanewt_2)
        (set `/Game/Blueprints/Enemies/BP_Mechanewt.HealthGate3` false _as_bp_mechanewt_2)
        (`/Game/Blueprints/Enemies/BP_Mechanewt.HealthGates` _as_bp_mechanewt_2)
        (`KismetSystemLibrary.PrintString` (`KismetStringLibrary.Conv_IntToString` _returnvalue_2))
        (`KismetSystemLibrary.LogString` "Pylons")
        (`self.K2_DestroyActor`)
        (else
          (`self.K2_DestroyActor`))))))

(event `self.ReceiveAnyDamage`
  (params (Damage :type "Float (single-precision)") (DamageType :type "DamageType Object Reference") (InstigatedBy :type "Controller Object Reference") (DamageCauser :type "Actor Object Reference"))
  ;[1 1 1] Health Manager
  (set `self.Attacking Actor` DamageCauser)
  (bind _output_get (set `self.CurrentHealth` (- (`self.CurrentHealth`) Damage)))
  (if (<= _output_get 0.0)
    (`self.UpdatePylonCount`)
    (else
      (`KismetSystemLibrary.PrintString` (`KismetStringLibrary.Conv_DoubleToString` (`self.CurrentHealth`))))))

(event `UpdatePylonCount`
  ;[1 1 1] Remove Pylon from Array when one is destroyed
  (`self.RemoveHealthGate`))

(fn `UserConstructionScript`)