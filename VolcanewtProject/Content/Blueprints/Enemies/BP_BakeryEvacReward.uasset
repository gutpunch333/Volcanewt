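; BP_BakeryEvacReward is an enemy-folder actor that restores health to the player's Volcanewt when the tongue eats it.
; On BeginPlay it casts the player pawn to BP_Volcanewt and sets the reward as a fraction of the Volcanewt's total health.
; When destroyed, it grants that health only if its Cube component is the Volcanewt's current tongue target.
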(event `self.ReceiveBeginPlay`
  (bind _asbp_volcanewt (cast `/Game/Player/BP_Volcanewt` (`GameplayStatics.GetPlayerPawn` 0)))
  (bind _output_get (set `self.As BP Volcanewt` _asbp_volcanewt))
  ;[1 1 1] Turns health given into a precentage of total health
  (set `self.HealthGiven` (* (`/Game/Player/BP_Volcanewt.TotalHealth` _output_get) 0.05)))

(event `self.ReceiveDestroyed`
  ;[1 1 1] Check's if the target currently being destroyed is also being eaten
  (if (== (`self.Cube`) (`/Game/Player/BP_Volcanewt.Tongue's Target` (stale `self.ReceiveBeginPlay` _output_get)))
    (`/Game/Player/BP_Volcanewt.Restore Volcanewt Health` (stale `self.ReceiveBeginPlay` _output_get) (`self.HealthGiven`))))

(fn `UserConstructionScript`)