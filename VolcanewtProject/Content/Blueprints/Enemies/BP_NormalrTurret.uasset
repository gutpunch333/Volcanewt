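; Enemy turret that tracks the nearest visible BP_Volcanewt pawn in range and shoots projectiles at it.
; A looping timer runs target search by sphere overlap and line of sight, turns the neck in yaw and pitch-clamped cannon head, then fires when cooled down and facing the target.
; Nested FlipFlops cycle shots through four muzzles.
; Any damage destroys it, reporting its monetary value and turret count to BPGM_Volcanewt.
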(event `self.ReceiveBeginPlay`
  ;[1 1 1 1 30] Rotates towards player and fires when facing them
  (`KismetSystemLibrary.K2_SetTimerDelegate` (delegate `CustomUpdate`) (`self.CustomSeconds`) true))

(event `CustomUpdate`
  ;[1 1 1 1 30] Rotates towards player and fires when facing them
  (`self.FindTarget`)
  (`self.Target`
    (:`then`
      (`self.UpdateRotation` (`self.CustomSeconds`))
      (`self.UpdateFire`))
    (:`else`)))

(event `Fire`
  (bind _currentgun (`self.CurrentGun`))
  (bind (_returnvalue_location _returnvalue_rotation _returnvalue_scale) (`KismetMathLibrary.BreakTransform` (`SceneComponent.K2_GetComponentToWorld` _currentgun)))
  (set `self.TimeOfLastFire` (`KismetSystemLibrary.GetGameTimeInSeconds`))
  (`/Engine/EditorBlueprintResources/StandardMacros.FlipFlop`
    (:`A`
      (`/Engine/EditorBlueprintResources/StandardMacros.FlipFlop`
        (:`A`
          ;[1 1 1] A bit spaghetti, but fires each cannon one after the other (adjust delays as needed)
          (set `self.CurrentGun` (`self.FireTransform`)))
        (:`B`
          (set `self.CurrentGun` (`self.FireTransform2`)))))
    (:`B`
      (`/Engine/EditorBlueprintResources/StandardMacros.FlipFlop`
        (:`A`
          (set `self.CurrentGun` (`self.FireTransform1`)))
        (:`B`
          (set `self.CurrentGun` (`self.FireTransform3`))))))
  (`GameplayStatics.PlaySoundAtLocation` "/Game/Audio/SoundEffects/StockandDeprectatedSFX/shootFree.shootFree" (`self.K2_GetActorLocation`) (struct) 0.02 1.0 0.0 null null null null)
  (`NiagaraFunctionLibrary.SpawnSystemAtLocation` null (`SceneComponent.K2_GetComponentLocation` _currentgun) (struct :`Roll` 180.0) (0.001 0.001 0.001))
  (`|SpawnActorFromClass` "/Game/Blueprints/Projectiles/BP_Projectile_Base.BP_Projectile_Base_C" (`KismetMathLibrary.MakeTransform` _returnvalue_location _returnvalue_rotation (* _returnvalue_scale (`self.ProjectileScale`))) "AlwaysSpawn" "MultiplyWithRoot" self 7000.0 7000.0 0.0 null null false null null false 0.0 false 0.0 false self))

(event `self.ReceiveAnyDamage`
  (params (Damage :type "Float (single-precision)") (DamageType :type "DamageType Object Reference") (InstigatedBy :type "Controller Object Reference") (DamageCauser :type "Actor Object Reference"))
  ;[1 1 1 1 100] Destroys Enemy
  (`GameplayStatics.PlaySoundAtLocation` "/Game/Audio/SoundEffects/Player/stompBoom.stompBoom" (`self.K2_GetActorLocation`) (struct) 0.4 1.1 0.15 null null null null)
  (bind _asbpgm_volcanewt (cast `/Game/Blueprints/Systems/BPGM_Volcanewt` (`GameplayStatics.GetGameMode`)))
  (`/Game/Blueprints/Systems/BPGM_Volcanewt.EnemyDestroyed` _asbpgm_volcanewt (`self.EnemyMonetaryValue`))
  (`/Game/Blueprints/Systems/BPGM_Volcanewt.TurretsCount` _asbpgm_volcanewt)
  (`self.K2_DestroyActor`))

(fn `FindTarget`
  (set `self.BestDistance` (+ (`self.SensingRange`) 1.0))
  (bind _outactors (`KismetSystemLibrary.SphereOverlapActors` (`self.K2_GetActorLocation`) (`self.SensingRange`) (`|MakeArray` "ObjectTypeQuery3" :!type "EObjectTypeQuery Enum") "/Game/Player/Blueprints/BP_Volcanewt.BP_Volcanewt_C"))
  (for _array_element _outactors
    (bind _output_get (set `self.CurrentTarget` _array_element))
    (bind _output_get_2 (set `self.CurrentDistance` (`self.GetDistanceTo` _output_get self)))
    (if (or (< _output_get_2 (`self.BestDistance`)) (not (`KismetSystemLibrary.IsValid` (`self.BestTarget`))))
      (bind _result (`/Game/Blueprints/Libraries_and_Interfaces/BPFL_MuhFunctionLibrary.HasLineOfSight` (`SceneComponent.K2_GetComponentLocation` (`self.sm_turretCannonHead_v2`)) (`self.K2_GetActorLocation` (`self.CurrentTarget`)) (`|MakeArray` self null :!type "Actor Object Reference")))
      (if _result
        (set `self.BestTarget` (`self.CurrentTarget`))
        (set `self.BestDistance` (`self.CurrentDistance`)))))
  (set `self.Target` (`self.BestTarget`)))

(fn `UpdateFire`
  (bind _sm_turretcannonhead_v2 (`self.sm_turretCannonHead_v2`))
  (if (> (- (`KismetSystemLibrary.GetGameTimeInSeconds`) (`self.TimeOfLastFire`)) (`self.RateOfFire`))
    (if (> (`KismetMathLibrary.Dot_VectorVector` (`KismetMathLibrary.GetDirectionUnitVector` (`SceneComponent.K2_GetComponentLocation` _sm_turretcannonhead_v2) (`self.K2_GetActorLocation` (`self.Target`))) (`SceneComponent.GetForwardVector` _sm_turretcannonhead_v2)) 0.99)
      (`self.Fire`)
      (`KismetSystemLibrary.PrintString` "Firing ground turret"))))

(fn `UpdateRotation`
  (params (Seconds :type "Float (double-precision)"))
  (locals (NewRotation :type "Rotator Structure") (NewCannonRotation :type "Rotator Structure"))
  (bind _sm_turretneck_v2 (`self.sm_turretNeck_v2`))
  (bind _sm_turretcannonhead_v2 (`self.sm_turretCannonHead_v2`))
  ;[1 1 1] Turret base movement
  (bind _output_get (set `local.NewRotation` (`KismetMathLibrary.RInterpTo_Constant` (`SceneComponent.K2_GetComponentRotation` _sm_turretneck_v2) (`KismetMathLibrary.FindLookAtRotation` (`SceneComponent.K2_GetComponentLocation` _sm_turretneck_v2) (`self.K2_GetActorLocation` (`self.Target`))) (`local.Seconds`) (`self.RotationSpeed`))))
  (`SceneComponent.K2_SetWorldRotation` (`self.sm_turretNeck_v2`) (`KismetMathLibrary.MakeRotator` (.roll _output_get) (`KismetMathLibrary.ClampAngle` (.pitch _output_get)) (.yaw _output_get)) false false)
  ;[1 1 1] Turret cannon movement
  (bind _output_get_2 (set `local.NewCannonRotation` (`KismetMathLibrary.RInterpTo_Constant` (`SceneComponent.K2_GetComponentRotation` _sm_turretcannonhead_v2) (`KismetMathLibrary.FindLookAtRotation` (`SceneComponent.K2_GetComponentLocation` _sm_turretcannonhead_v2) (`self.K2_GetActorLocation` (`self.Target`))) (`self.CustomSeconds`) (`self.RotationSpeed`))))
  (`SceneComponent.K2_SetWorldRotation` (`self.sm_turretCannonHead_v2`) (`KismetMathLibrary.MakeRotator` (.roll _output_get) (`KismetMathLibrary.ClampAngle` (.pitch _output_get_2) -45.0 45.0) (.yaw _output_get)) false false))

(fn `UserConstructionScript`)