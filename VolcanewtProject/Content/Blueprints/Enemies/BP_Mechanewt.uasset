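; BP_Mechanewt is an enemy character that spots the player's Volcanewt through PawnSensing and turns to face it.
; Sighting starts a looping yaw interpolation toward the player and writes seen and distance blackboard keys, though the distance derives from summed locations.
; Helper functions, uncalled by its event graph, cover leg/tail overlap damage, escalating-odds fire and explosion rolls, lava spawning, slope/climb traces and charge cooldowns.
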(event `self.ReceiveBeginPlay`
  (bind _asbp_volcanewt (cast `/Game/Player/Blueprints/BP_Volcanewt` (`GameplayStatics.GetPlayerCharacter` 0)))
  (set `self.As BP Volcanewt` _asbp_volcanewt)
  (cast `/Game/Blueprints/Systems/BPGM_Volcanewt` (`GameplayStatics.GetGameMode`)))

(event `self.PawnSensing.OnSeePawn`
  (params (Pawn :type "Pawn Object Reference"))
  (`self.FacePlayer` :!label _label)
  (cast `/Game/Player/Blueprints/BP_Volcanewt` Pawn)
  (`BlackboardComponent.SetValueAsBool` (`AIBlueprintHelperLibrary.GetBlackboard` (`AIBlueprintHelperLibrary.GetAIController` self)) "hasSeenPlayer?" true)
  (`BlackboardComponent.SetValueAsFloat` (`AIBlueprintHelperLibrary.GetBlackboard` (`AIBlueprintHelperLibrary.GetAIController` self)) "DistanceToPlayer" (`KismetStringLibrary.Conv_StringToDouble` (`KismetStringLibrary.Conv_Vector3fToString` (+ (`self.K2_GetActorLocation` self) (`self.K2_GetActorLocation` self)))))
  (`KismetSystemLibrary.RetriggerableDelay` 0.6)
  (goto _label))

(event `FacePlayer`
  (bind (_returnvalue_roll _returnvalue_pitch _returnvalue_yaw) (`KismetMathLibrary.BreakRotator` (`KismetMathLibrary.RInterpTo` (`self.K2_GetActorRotation`) (`KismetMathLibrary.FindLookAtRotation` (`self.K2_GetActorLocation`) (`self.K2_GetActorLocation` (`self.As BP Volcanewt`))) (`GameplayStatics.GetWorldDeltaSeconds`) 1.0)))
  (`self.K2_SetActorRotation` (`KismetMathLibrary.MakeRotator` 0.0 0.0 _returnvalue_yaw) :!label _label_2)
  (`KismetSystemLibrary.Delay` 0.001)
  (goto _label_2))

(fn `AbilityUnlock`
  (params (NewParam :type Boolean))
  (returns (AbilityToBeUnlock :type Boolean))
  (return false))

(fn `AccelerationCheckPoint`
  (params (`Char.MovementComp.BeingChecked` :type "CharacterMovementComponent Object Reference") (AccelerationIsAbove :type "Float (double-precision)"))
  (returns (`AccelerationIsAbove?` :type Boolean))
  (return (> (`CharacterMovementComponent.GetMaxAcceleration` `Char.MovementComp.BeingChecked`) (- AccelerationIsAbove 1.0))))

(fn `AverageTwoVectors`
  (params (FirstVector :type "Vector Structure") (SecondVector :type "Vector Structure"))
  (returns (AveragedVector :type "Vector Structure"))
  (return (/ (+ FirstVector SecondVector) 2.0)))

(fn `ClimbLineTrace`
  (returns (`Out Hit` :type "HitResult Structure") (`Has Hit` :type Boolean))
  (bind _sphere (`self.Sphere`))
  (bind _returnvalue (`SceneComponent.K2_GetComponentLocation` _sphere))
  (if (not (`NavMovementComponent.IsFalling` (`self.CharacterMovement`)))
    (bind (_outhit _returnvalue_2) (`KismetSystemLibrary.LineTraceSingle` :`Start` _returnvalue :`End` (+ _returnvalue (* (`SceneComponent.GetForwardVector` _sphere) 1200.0)) :`TraceChannel` "TraceTypeQuery1" :`DrawDebugType` "ForDuration"))
    (return _outhit _returnvalue_2)))

(fn `DecreaseChargeCooldown`
  (params (NewParam :type "Float (double-precision)") (NewParam1 :type "Actor Object Reference"))
  (set `self.CooldownBlock` true)
  (if (not (== NewParam 2.0))
    (bind _output_get (set `self.ChargeCooldown` (- NewParam 1.0)))
    (if (`self.IsDebugEnabled`)
      (`KismetSystemLibrary.PrintString` (`KismetStringLibrary.Conv_DoubleToString` _output_get))
      (`KismetSystemLibrary.PrintString` "Charge cooldown"))))

(fn `DecreaseFootHitBox`
  (params (`Leg to Shrink` :type "BoxComponent Object Reference") (`X scalar` :type "Float (double-precision)") (`Y scalar` :type "Float (double-precision)") (`Z scalar` :type "Float (double-precision)"))
  (`BoxComponent.SetBoxExtent` `Leg to Shrink` (/ (`SceneComponent.K2_GetComponentScale` `Leg to Shrink`) (`KismetMathLibrary.MakeVector` `X scalar` `Y scalar` `Z scalar`)) true))

(fn `GetNearestEnemy`
  (returns (ClosestEnemy :type "Actor Object Reference"))
  (locals (NearestEnemy :type "Actor Object Reference"))
  (bind _returnvalue (`self.K2_GetActorLocation`))
  (bind _outhits (`KismetSystemLibrary.SphereTraceMultiForObjects` _returnvalue _returnvalue 1000.0 (`|MakeArray` "ObjectTypeQuery3" :!type "EObjectTypeQuery Enum")))
  (for _array_element _outhits
    (if (`self.ActorHasTag` (`.HitActor` (`GameplayStatics.BreakHitResult` _array_element)) "Edible")
      (`/Engine/EditorBlueprintResources/StandardMacros.IsValid` (`local.NearestEnemy`)
        (:`Is Valid`
          (if (not (< (`self.GetDistanceTo` (`local.NearestEnemy`) self) (`self.GetDistanceTo` (`.HitActor` (`GameplayStatics.BreakHitResult` _array_element)) self)))
            (set `local.NearestEnemy` (`.HitActor` (`GameplayStatics.BreakHitResult` _array_element)) :!label _label)))
        (:`Is Not Valid`
          (goto _label)))))
  (return null))

(fn `IgnoreBuildings`
  (params (Array :type "Array of Actor Object Reference")))

(fn `IncreaseFootHitBox`
  (params (`Leg to Grow` :type "BoxComponent Object Reference") (`X scalar` :type "Float (double-precision)") (`Y scalar` :type "Float (double-precision)") (`Z scalar` :type "Float (double-precision)"))
  (`BoxComponent.SetBoxExtent` `Leg to Grow` (* (`SceneComponent.K2_GetComponentScale` `Leg to Grow`) (`KismetMathLibrary.MakeVector` `X scalar` `Y scalar` `Z scalar`)) true))

(fn `LavaFireSpawn`
  (`|SpawnActorFromClass` "/Game/Player/Blueprints/BP_Lava.BP_Lava_C" (`SceneComponent.K2_GetComponentToWorld` (`self.LavaSpawn`)) "Undefined" "MultiplyWithRoot" null null))

(fn `ResetChargeCooldown`
  (if (!= (`self.ChargeCooldown`) 5.0)
    (bind _output_get (set `self.ChargeCooldown` 5.0))
    (if (`self.IsDebugEnabled`)
      (`KismetSystemLibrary.PrintString` (`KismetStringLibrary.Conv_DoubleToString` _output_get))
      (`KismetSystemLibrary.PrintString` "Charge cooldown"))))

(fn `RollForCreateExplosion`
  (params (ShouldRollForExplosion :type Boolean) (DamageOfExplosion :type "Float (double-precision)") (ExplosionChanceToSpawn :type Integer) (ExplosionSpawnLocation :type "Vector Structure") (ExplosionHasRandomOffset :type Boolean) (RandomLocationOffsetAmount :type "Float (double-precision)") (DoesExplosionHaveChanceToCreateFlame :type Boolean) (ExplosionChanceToCreateFlame :type Integer) (FailsEscalateOdds :type Boolean))
  (if ShouldRollForExplosion
    (if (> ExplosionChanceToSpawn (`self.RandomExplosionStoredChance`))
      (set `self.RandomExplosionStoredChance` ExplosionChanceToSpawn))
    (if (<= (`KismetMathLibrary.RandomIntegerInRange` 1 100) (`self.RandomExplosionStoredChance`))
      (`|SpawnActorFromClass` "/Game/Blueprints/SpawnedActors/RandomExplosion.RandomExplosion_C" (`KismetMathLibrary.MakeTransform` ExplosionSpawnLocation) "Undefined" "MultiplyWithRoot" null DamageOfExplosion ExplosionHasRandomOffset RandomLocationOffsetAmount RandomLocationOffsetAmount "/Game/VFX/Effects/FXS_Explosion.FXS_Explosion" "/Game/Audio/SoundEffects/Player/jumpBoom.jumpBoom" null)
      (set `self.RandomExplosionStoredChance` ExplosionChanceToSpawn)
      (if DoesExplosionHaveChanceToCreateFlame
        (if (<= (`KismetMathLibrary.RandomIntegerInRange` 1 100) ExplosionChanceToCreateFlame)
          (`self.RollForCreateFlame` false 5.0 4.0 false 10 10 ExplosionSpawnLocation)))
      (elif FailsEscalateOdds
        (set `self.RandomExplosionStoredChance` (+ (`self.RandomExplosionStoredChance`) ExplosionChanceToSpawn))))))

(fn `RollForCreateFlame`
  (params (ShouldRollForFire :type Boolean) (DamageOfFireTick :type "Float (double-precision)" :default 5.0) (SecondsBetweenTicks :type "Float (double-precision)" :default 4.0) (DoesThisFireSpread :type Boolean) (FireChanceToSpread :type Integer :default 10) (FireChanceToSpawn :type Integer :default 10) (FireSpawnLocation :type "Vector Structure") (ScaleToSpawnAt :type "Float (double-precision)" :default 1.0) (FailsEscalateOdds :type Boolean))
  (if ShouldRollForFire
    (if (> FireChanceToSpawn (`self.RandomFireStoredChance`))
      (set `self.RandomFireStoredChance` FireChanceToSpawn))
    (if (<= (`KismetMathLibrary.RandomIntegerInRange` 1 100) (`self.RandomFireStoredChance`))
      (`|SpawnActorFromClass` "/Game/Blueprints/SpawnedActors/RandomExplosion.RandomExplosion_C" (`KismetMathLibrary.MakeTransform` FireSpawnLocation (struct) (`KismetMathLibrary.MakeVector` ScaleToSpawnAt ScaleToSpawnAt ScaleToSpawnAt)) "Undefined" "MultiplyWithRoot" null DamageOfFireTick false 20.0 20.0 "/Game/VFX/Effects/FXS_Explosion.FXS_Explosion" null null)
      (set `self.RandomFireStoredChance` FireChanceToSpawn)
      (elif FailsEscalateOdds
        (set `self.RandomFireStoredChance` (+ (`self.RandomFireStoredChance`) FireChanceToSpawn))))))

(fn `RollForCreateLava`
  (params (ShouldRollForFire :type Boolean) (DamageOfFireTick :type "Float (double-precision)" :default 5.0) (SecondsBetweenTicks :type "Float (double-precision)" :default 4.0) (DoesThisFireSpread :type Boolean) (FireChanceToSpread :type Integer :default 10) (FireChanceToSpawn :type Integer :default 10) (FireSpawnLocation :type "Vector Structure") (ScaleToSpawnAt :type "Float (double-precision)" :default 1.0) (LavaRotation :type "Rotator Structure"))
  (if ShouldRollForFire
    (if (<= (`KismetMathLibrary.RandomIntegerInRange` 1 100) FireChanceToSpawn)
      (`|SpawnActorFromClass` "/Game/Blueprints/Enemies/ProjectilesEtc/BP_LaserProjectile.BP_LaserProjectile_C" (`KismetMathLibrary.MakeTransform` FireSpawnLocation LavaRotation (`KismetMathLibrary.MakeVector` ScaleToSpawnAt ScaleToSpawnAt ScaleToSpawnAt)) "Undefined" "MultiplyWithRoot" null null) ; Might have to mess with this, maybe another variant of laser? -Sean
    )))

(fn `SlopeLineTrace`
  (returns (`Out Hit` :type "HitResult Structure") (`Has Hit` :type Boolean))
  (bind _returnvalue (`SceneComponent.K2_GetComponentLocation` (`self.Sphere`)))
  (bind (_outhit _returnvalue_2) (`KismetSystemLibrary.LineTraceSingle` :`Start` _returnvalue :`End` (- _returnvalue (0.0 0.0 1500.0)) :`TraceChannel` "TraceTypeQuery1" :`DrawDebugType` "ForDuration"))
  (return _outhit _returnvalue_2))

(fn `SpeedCheckPoint`
  (params (VelocityIsAbove :type "Float (double-precision)"))
  (returns (WasVelocityReached :type Boolean))
  (return (> (`KismetMathLibrary.VSize` (`self.GetVelocity`)) (- VelocityIsAbove 1.0))))

(fn `SpeedReverseCheckPoint`
  (params (VelocityIsBelow :type "Float (double-precision)"))
  (returns (WasVelocityReached :type Boolean))
  (return (< (`KismetMathLibrary.VSize` (`self.GetVelocity`)) VelocityIsBelow)))

(fn `UserConstructionScript`)

(fn `WalkingDamage`
  (if (not (`self.Cooldown`))
    (`|ExecutionSequence`
      (:`then_0`
        (for _array_element (`PrimitiveComponent.GetOverlappingActors` (`self.RightRearLeg`) null)
          ;[1 1 1] To avoid helicopters from damage by walking
          (if (`self.ActorHasTag` _array_element "FlyingUnit")
            _
            (elif (not (`self.ActorHasTag` _array_element "Newt"))
              (`GameplayStatics.ApplyDamage` _array_element (`self.WalkAOEDamage`))))))
      (:`then_1`
        (for _array_element_2 (`PrimitiveComponent.GetOverlappingActors` (`self.LeftRearLeg`) null)
          (if (`self.ActorHasTag` _array_element_2 "FlyingUnit")
            _
            (elif (not (`self.ActorHasTag` _array_element_2 "Newt"))
              (`GameplayStatics.ApplyDamage` _array_element_2 (`self.WalkAOEDamage`))))))
      (:`then_2`
        (for _array_element_3 (`PrimitiveComponent.GetOverlappingActors` (`self.RightFrontLeg`) null)
          (if (`self.ActorHasTag` _array_element_3 "FlyingUnit")
            _
            (elif (not (`self.ActorHasTag` _array_element_3 "Newt"))
              (`GameplayStatics.ApplyDamage` _array_element_3 (`self.WalkAOEDamage`))))))
      (:`then_3`
        (for _array_element_4 (`PrimitiveComponent.GetOverlappingActors` (`self.LeftFrontLeg`) null)
          (if (`self.ActorHasTag` _array_element_4 "FlyingUnit")
            _
            (elif (not (`self.ActorHasTag` _array_element_4 "Newt"))
              (`GameplayStatics.ApplyDamage` _array_element_4 (`self.WalkAOEDamage`))))))
      (:`then_4`
        (for _array_element_5 (`PrimitiveComponent.GetOverlappingActors` (`self.TailRear`) null)
          (if (`self.ActorHasTag` _array_element_5 "FlyingUnit")
            _
            (elif (not (`self.ActorHasTag` _array_element_5 "Newt"))
              (`GameplayStatics.ApplyDamage` _array_element_5 (`self.TailAOEDamage`))))))
      (:`then_5`
        (for _array_element_6 (`PrimitiveComponent.GetOverlappingActors` (`self.TailTip`) null)
          (if (`self.ActorHasTag` _array_element_6 "FlyingUnit")
            _
            (elif (not (`self.ActorHasTag` _array_element_6 "Newt"))
              (`GameplayStatics.ApplyDamage` _array_element_6 (`self.TailAOEDamage`)))))))))