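; BP_Rocket is a homing projectile that seeks Newt-tagged actors and explodes on contact with a Volcanewt.
; Every half second it searches by distance for the nearest target, updating projectile homing and a Niagara target parameter.
; Overlapping a player-controlled Volcanewt deals damage before a briefly delayed explosion; other Volcanewts trigger an immediate explosion without damage.
; A delay in LockOn also makes it self-destruct after seven seconds.
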(event `self.Sphere.OnComponentHit`
  (params (HitComponent :type "PrimitiveComponent Object Reference") (OtherActor :type "Actor Object Reference") (OtherComp :type "PrimitiveComponent Object Reference") (NormalImpulse :type "Vector Structure") (Hit :type "HitResult Structure (by ref)"))
  (`KismetSystemLibrary.PrintString` "Ouchie"))

(event `Lock On`
  (bind _homingtarget (`self.Find Homing Target`))
  (set `ProjectileMovementComponent.HomingTargetComponent` _homingtarget (`self.ProjectileMovement`))
  (`GameplayStatics.GetAllActorsOfClass` "/Game/Player/BP_Volcanewt.BP_Volcanewt_C")
  (`NiagaraComponent.SetVariableVec3` (`self.Niagara`) "Target" (`SceneComponent.K2_GetComponentLocation` _homingtarget))
  (`KismetSystemLibrary.Delay` 7.0)
  (`NiagaraFunctionLibrary.SpawnSystemAtLocation` "/Game/VFX/P_Explosion.P_Explosion" (`self.K2_GetActorLocation`))
  (`self.K2_DestroyActor`))

(event `self.ReceiveBeginPlay`
  (`self.Lock On` :!label _label)
  (`KismetSystemLibrary.Delay` 0.5)
  (goto _label))

(event `self.Sphere.OnComponentBeginOverlap`
  (params (OverlappedComponent :type "PrimitiveComponent Object Reference") (OtherActor :type "Actor Object Reference") (OtherComp :type "PrimitiveComponent Object Reference") (OtherBodyIndex :type Integer) (bFromSweep :type Boolean) (SweepResult :type "HitResult Structure (by ref)"))
  (bind _returnvalue (`GameplayStatics.GetPlayerCharacter` 0))
  (cast `/Game/Player/BP_Volcanewt` OtherActor)
  (if (== OtherActor _returnvalue)
    (`|ExecutionSequence`
      (:`then_0`
        (`GameplayStatics.ApplyDamage` _returnvalue 25.0))
      (:`then_1`
        (`KismetSystemLibrary.Delay` 0.2)
        (`NiagaraFunctionLibrary.SpawnSystemAtLocation` "/Game/VFX/P_Explosion.P_Explosion" (`self.K2_GetActorLocation`))
        (`self.K2_DestroyActor`)))
    (else
      (`NiagaraFunctionLibrary.SpawnSystemAtLocation` "/Game/VFX/P_Explosion.P_Explosion" (`self.K2_GetActorLocation`))
      (`self.K2_DestroyActor`))))

(fn `Find Homing Target`
  (returns (HomingTarget :type "SceneComponent Object Reference"))
  (bind _outactors (`GameplayStatics.GetAllActorsOfClassWithTag` "/Script/Engine.Actor" "Newt"))
  (for _array_element _outactors
    (bind _returnvalue (`KismetMathLibrary.VSize` (- (`self.K2_GetActorLocation` _array_element) (`self.K2_GetActorLocation`))))
    (if (< _returnvalue (`self.NewtDistance`))
      (set `self.NewtDistance` _returnvalue)
      (set `self.HomingTarget` _array_element)))
  (return (`self.GetComponentByClass` (`self.HomingTarget`) "/Script/Engine.SceneComponent")))

(fn `UserConstructionScript`)