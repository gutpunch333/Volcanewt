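; Basic helicopter-sounding enemy that chases and shoots the player's Volcanewt, driven by AI through a blackboard.
; Pawn sensing sets a seen-player flag, cleared by a retriggerable delay shortly after sightings stop.
; AttackPlayer sphere-traces forward and spawns a test projectile on hitting the player; any damage destroys the enemy and reports its monetary value to the game mode.
; Older roam and follow logic remains as disconnected leftovers, noted as superseded by an AI tree.
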(event `self.ReceiveBeginPlay`
  ;[1 1 1 1 100] Event BeginPlay
  (`GameplayStatics.PlaySoundAtLocation` "/Game/Audio/SoundEffects/HelicopterBlades.HelicopterBlades" (`self.K2_GetActorLocation`) (struct) 0.8 1.0 0.0 null null null null))

(event `self.ReceiveAnyDamage`
  (params (Damage :type "Float (single-precision)") (DamageType :type "DamageType Object Reference") (InstigatedBy :type "Controller Object Reference") (DamageCauser :type "Actor Object Reference"))
  ;[1 1 1 1 100] Destroys Enemy
  (`GameplayStatics.PlaySoundAtLocation` "/Game/Audio/SoundEffects/Player/stompBoom.stompBoom" (`self.K2_GetActorLocation`) (struct) 0.4 1.1 0.15 null null null null)
  (bind _asbpgm_volcanewt (cast `/Game/Blueprints/Systems/BPGM_Volcanewt` (`GameplayStatics.GetGameMode`)))
  (`/Game/Blueprints/Systems/BPGM_Volcanewt.EnemyDestroyed` _asbpgm_volcanewt (`self.EnemyMonetaryValue`))
  (`self.K2_DestroyActor`))

(event `self.PawnSensing.OnSeePawn`
  (params (Pawn :type "Pawn Object Reference"))
  (bind _returnvalue (`AIBlueprintHelperLibrary.GetBlackboard` (`AIBlueprintHelperLibrary.GetAIController` self)))
  ;[1 1 1 1 30] On seeing the player, follow them
  (cast `/Game/Player/BP_Volcanewt` Pawn)
  (`BlackboardComponent.SetValueAsBool` _returnvalue "hasSeenPlayer?" true)
  (`KismetSystemLibrary.RetriggerableDelay` 0.6)
  (`BlackboardComponent.SetValueAsBool` _returnvalue "hasSeenPlayer?" false))

(event `Roam Around`
  ;[1 1 1 1 70] This should all be redundant because it uses an AI tree now, but im scared to delet in case i need it -griffin
)

(event `AttackPlayer`
  (bind _returnvalue (`self.K2_GetActorLocation`))
  ;[1 1 1] Attack Player
  (bind (_outhit _returnvalue_2) (`KismetSystemLibrary.SphereTraceSingleForObjects` _returnvalue (+ _returnvalue (* (`KismetMathLibrary.GetForwardVector` (`self.K2_GetActorRotation`)) 1500.0)) 250.0 (`|MakeArray` "ObjectTypeQuery3" :!type "EObjectTypeQuery Enum")))
  (if _returnvalue_2
    (cast `/Game/Player/BP_Volcanewt` (`.HitActor` (`GameplayStatics.BreakHitResult` _outhit)))
    (`GameplayStatics.PlaySoundAtLocation` "/Game/Audio/SoundEffects/EnemySFX/machine_gun.machine_gun" (`self.K2_GetActorLocation`) (struct) 1.0 1.0 0.0 null null null null)
    (`|SpawnActorFromClass` "/Game/Blueprints/Enemies/ProjectilesEtc/TestProjectile.TestProjectile_C" (`SceneComponent.K2_GetComponentToWorld` (`self.spawn proj loc`)) "AlwaysSpawn" "MultiplyWithRoot" null null)))

(event `self.ReceiveTick`
  (params (DeltaSeconds :type "Float (single-precision)"))
  ;[1 1 1 1 70] This should all be redundant because it uses an AI tree now, but im scared to delet in case i need it -griffin
)

(event `Follow Player`
  ;[1 1 1 1 70] This should all be redundant because it uses an AI tree now, but im scared to delet in case i need it -griffin
)

(fn `UserConstructionScript`)