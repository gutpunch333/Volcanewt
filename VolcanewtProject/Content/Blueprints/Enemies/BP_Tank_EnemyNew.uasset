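; Tank enemy that registers with the Volcanewt game mode, tracks the player with a turret and shoots projectiles.
; Each tick it finds the nearest visible Volcanewt in range, yaws the turret toward it and fires once aligned (dot-product check) and off cooldown.
; Pawn sensing sets the AI blackboard's seen-player flag and starts a self-repeating delay loop that turns the body toward the player.
; Any damage destroys it and reports its monetary value.
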(event `self.ReceiveBeginPlay`
  (bind _asbp_volcanewt (cast `/Game/Player/Blueprints/BP_Volcanewt` (`GameplayStatics.GetPlayerCharacter` 0)))
  (set `self.As BP Volcanewt` _asbp_volcanewt)
  (bind _asbpgm_volcanewt (cast `/Game/Blueprints/Systems/BPGM_Volcanewt` (`GameplayStatics.GetGameMode`)))
  (bind _output_get (set `self.As BPGM Volcanewt` _asbpgm_volcanewt))
  (`/Game/Blueprints/Systems/BPGM_Volcanewt.Increase Enemies` _output_get))

(event `self.ReceiveTick`
  (params (DeltaSeconds :type "Float (single-precision)"))
  (`self.FindTarget`)
  (`self.Target`
    (:`then`
      (`self.UpdateRotation` DeltaSeconds)
      (`self.UpdateFire`))
    (:`else`)))

(event `self.PawnSensing.OnSeePawn`
  (params (Pawn :type "Pawn Object Reference"))
  (bind _returnvalue (`AIBlueprintHelperLibrary.GetBlackboard` (`AIBlueprintHelperLibrary.GetAIController` self)))
  ;[1 1 1 1 30] On seeing the player, follow them (copied from basic/helicopter enemy script)
  (`self.FacePlayer` :!label _label)
  (if (`self.ActorHasTag` Pawn "Newt") :!label _label_2
    (cast `/Game/Player/Blueprints/BP_Volcanewt` Pawn)
    (`BlackboardComponent.SetValueAsBool` _returnvalue "hasSeenPlayer?" true)
    (`KismetSystemLibrary.RetriggerableDelay` 0.6)
    (goto _label)
    (else
      (`BlackboardComponent.SetValueAsBool` _returnvalue "hasSeenPlayer?" false)
      (`KismetSystemLibrary.RetriggerableDelay` 0.6)
      (goto _label_2))))

(event `self.ReceiveAnyDamage`
  (params (Damage :type "Float (single-precision)") (DamageType :type "DamageType Object Reference") (InstigatedBy :type "Controller Object Reference") (DamageCauser :type "Actor Object Reference"))
  ;[1 1 1 1 100] Destroys Enemy
  (`GameplayStatics.PlaySoundAtLocation` "/Game/Audio/SoundEffects/Player/stompBoom.stompBoom" (`self.K2_GetActorLocation`) (struct) 0.4 1.1 0.15 null null null null)
  (bind _asbpgm_volcanewt (cast `/Game/Blueprints/Systems/BPGM_Volcanewt` (`GameplayStatics.GetGameMode`)))
  (`/Game/Blueprints/Systems/BPGM_Volcanewt.EnemyDestroyed` _asbpgm_volcanewt (`self.EnemyMonetaryValue`))
  (`self.K2_DestroyActor`))

(event `Fire`
  (bind _spawn_proj_loc (`self.spawn proj loc`))
  ;[1 1 1] Updated fire
  (set `self.TimeOfLastFire` (`KismetSystemLibrary.GetGameTimeInSeconds`))
  (`GameplayStatics.PlaySoundAtLocation` "/Game/Audio/SoundEffects/shootFree.shootFree" (`self.K2_GetActorLocation`) (struct) 1.0 1.0 0.0 null null null null)
  (`NiagaraFunctionLibrary.SpawnSystemAtLocation` "/Game/VFX/Effects/FXS_Explosion.FXS_Explosion" (`SceneComponent.K2_GetComponentLocation` _spawn_proj_loc) (struct) (0.001 0.001 0.001))
  (`|SpawnActorFromClass` "/Game/Blueprints/Enemies/ProjectilesEtc/BP_TestProjectile.BP_TestProjectile_C" (`SceneComponent.K2_GetComponentToWorld` _spawn_proj_loc) "AlwaysSpawn" "MultiplyWithRoot" null null))

(event `FacePlayer`
  (bind (_returnvalue_roll _returnvalue_pitch _returnvalue_yaw) (`KismetMathLibrary.BreakRotator` (`KismetMathLibrary.RInterpTo` (`self.K2_GetActorRotation`) (`KismetMathLibrary.FindLookAtRotation` (`self.K2_GetActorLocation`) (`self.K2_GetActorLocation` (`self.As BP Volcanewt`))) (`GameplayStatics.GetWorldDeltaSeconds`) 20.0)))
  ;[1 1 1] Rotate to face player (same as basic enemy BP)
  (`self.K2_SetActorRotation` (`KismetMathLibrary.MakeRotator` 0.0 0.0 _returnvalue_yaw))
  (`KismetSystemLibrary.Delay` 0.001)
  (`self.FacePlayer`))

(fn `FindTarget`
  ;[1 1 1] Determines best target and ensures it can be seen (same as birthday cake boss)
  (set `self.BestDistance` (+ (`self.SensingRange`) 1.0))
  (bind _outactors (`KismetSystemLibrary.SphereOverlapActors` (`self.K2_GetActorLocation`) (`self.SensingRange`) (`|MakeArray` "ObjectTypeQuery3" :!type "EObjectTypeQuery Enum") "/Game/Player/Blueprints/BP_Volcanewt.BP_Volcanewt_C"))
  (for _array_element _outactors
    (bind _output_get (set `self.CurrentTarget` _array_element))
    (bind _output_get_2 (set `self.CurrentDistance` (`self.GetDistanceTo` _output_get self)))
    (if (or (< _output_get_2 (`self.BestDistance`)) (not (`KismetSystemLibrary.IsValid` (`self.BestTarget`))))
      (bind _result (`/Game/Blueprints/Libraries_and_Interfaces/BPFL_MuhFunctionLibrary.HasLineOfSight` (`SceneComponent.K2_GetComponentLocation` (`self.Top`)) (`self.K2_GetActorLocation` (`self.CurrentTarget`)) (`|MakeArray` self (`self.CurrentTarget`) :!type "Actor Object Reference")))
      (if _result
        (set `self.BestTarget` (`self.CurrentTarget`))
        (set `self.BestDistance` (`self.CurrentDistance`)))))
  (set `self.Target` (`self.BestTarget`)))

(fn `UpdateFire`
  (bind _top (`self.Top`))
  (if (> (- (`KismetSystemLibrary.GetGameTimeInSeconds`) (`self.TimeOfLastFire`)) (`self.RateOfFire`))
    (if (> (`KismetMathLibrary.Dot_VectorVector` (`KismetMathLibrary.GetDirectionUnitVector` (`SceneComponent.K2_GetComponentLocation` _top) (`self.K2_GetActorLocation` (`self.Target`))) (`SceneComponent.GetForwardVector` _top)) 0.99)
      (`self.Fire`)
      (`KismetSystemLibrary.PrintString` "Firing Turret"))))

(fn `UpdateRotation`
  (params (DeltaSeconds :type "Float (double-precision)"))
  (locals (NewRotation :type "Rotator Structure"))
  (bind _top (`self.Top`))
  (bind _output_get (set `local.NewRotation` (`KismetMathLibrary.RInterpTo_Constant` (`SceneComponent.K2_GetComponentRotation` _top) (`KismetMathLibrary.FindLookAtRotation` (`SceneComponent.K2_GetComponentLocation` _top) (`self.K2_GetActorLocation` (`self.Target`))) (`local.DeltaSeconds`) (`self.RotationSpeed`))))
  (`SceneComponent.K2_SetWorldRotation` (`self.Top`) (`KismetMathLibrary.MakeRotator` (.roll _output_get) (`KismetMathLibrary.ClampAngle` (.pitch _output_get)) (.yaw _output_get)) false false))

(fn `UserConstructionScript`)