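; Tank enemy projectile that explodes and damages the player on hit.
; The Hit event only proceeds when the other actor casts to BP_Volcanewt, so other impacts are ignored here.
; If that actor is the player character, it waits briefly, spawns a scaled-down explosion effect, applies fixed damage and destroys itself.
; A non-player Volcanewt gets the explosion and bullet destruction immediately, without damage.
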(event `self.Bullet.OnComponentHit`
  (params (HitComponent :type "PrimitiveComponent Object Reference") (OtherActor :type "Actor Object Reference") (OtherComp :type "PrimitiveComponent Object Reference") (NormalImpulse :type "Vector Structure") (Hit :type "HitResult Structure (by ref)")))

(event `self.ReceiveHit`
  (params (MyComp :type "PrimitiveComponent Object Reference") (Other :type "Actor Object Reference") (OtherComp :type "PrimitiveComponent Object Reference") (bSelfMoved :type Boolean) (HitLocation :type "Vector Structure") (HitNormal :type "Vector Structure") (NormalImpulse :type "Vector Structure") (Hit :type "HitResult Structure (by ref)"))
  (bind _returnvalue (`GameplayStatics.GetPlayerCharacter` 0))
  ;[1 0.07292 0.07292] Dealing Damage
  (cast `/Game/Player/Blueprints/BP_Volcanewt` Other)
  (if (== Other _returnvalue)
    (`KismetSystemLibrary.Delay` 0.2)
    (`NiagaraFunctionLibrary.SpawnSystemAtLocation` "/Game/VFX/Effects/FXS_Explosion.FXS_Explosion" (`self.K2_GetActorLocation`) (struct) (0.5 0.5 0.5))
    (`GameplayStatics.ApplyDamage` _returnvalue 25.0)
    (`self.K2_DestroyActor`)
    (else
      (`NiagaraFunctionLibrary.SpawnSystemAtLocation` "/Game/VFX/Effects/FXS_Explosion.FXS_Explosion" (`self.K2_GetActorLocation`) (struct) (0.5 0.5 0.5))
      (`self.K2_DestroyActor`))))

(fn `UserConstructionScript`)