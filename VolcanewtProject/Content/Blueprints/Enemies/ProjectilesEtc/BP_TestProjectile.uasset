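; BP_TestProjectile is a test enemy projectile, built as an AI-moved pawn, that damages the player on hit.
; On BeginPlay it uses AIMoveTo toward the player's starting location with a large acceptance radius.
; On Hit it destroys itself, first applying damage after a brief delay if it struck the player.
; Roaming, following and attack logic is disconnected or empty; PawnSensing only sets a flag.
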(event `Roam Around`)

(event `self.ReceiveAnyDamage`
  (params (Damage :type "Float (single-precision)") (DamageType :type "DamageType Object Reference") (InstigatedBy :type "Controller Object Reference") (DamageCauser :type "Actor Object Reference")))

(event `self.ReceiveHit`
  (params (MyComp :type "PrimitiveComponent Object Reference") (Other :type "Actor Object Reference") (OtherComp :type "PrimitiveComponent Object Reference") (bSelfMoved :type Boolean) (HitLocation :type "Vector Structure") (HitNormal :type "Vector Structure") (NormalImpulse :type "Vector Structure") (Hit :type "HitResult Structure (by ref)"))
  (bind _returnvalue (`GameplayStatics.GetPlayerPawn` 0))
  ;[1 0.07292 0.07292] Dealing Damage
  (if (== Other _returnvalue)
    (`KismetSystemLibrary.Delay` 0.1)
    (`GameplayStatics.ApplyDamage` _returnvalue 25.0)
    (`self.K2_DestroyActor`)
    (else
      (`self.K2_DestroyActor`))))

(event `self.ReceiveTick`
  (params (DeltaSeconds :type "Float (single-precision)"))
  ;[1 1 1] If seeing player, or roaming has not ended, stop moving and end roaming
)

(event `self.ReceiveBeginPlay`
  ;[0.5067 1 0.1729] Moving to target location
  (`KismetSystemLibrary.Delay` 0.001)
  (`|AIMoveTo` self (`self.K2_GetActorLocation` (`GameplayStatics.GetPlayerCharacter` 0)) null 2000.0))

(event `Follow Player`)

(event `self.PawnSensing.OnSeePawn`
  (params (Pawn :type "Pawn Object Reference"))
  ;[1 1 1] On seeing the player, follow them
  (set `self.isSeeingPlayer` true))

(fn `UserConstructionScript`)