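; Laser turret enemy owned by an Albatross boss (Albatross_Proto) that tracks and shoots at the player's Volcanewt.
; A looping timer picks the nearest visible target in range, rotates neck and pitch-clamped cannon, then fires projectiles when aligned and off cooldown.
; First damage flags which turret is engaged on the Albatross.
; Every hit calls the game mode's EnemyDestroyed and TurretsCount; death stops the Albatross's death-laser charge and destroys the turret.
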(event `self.ReceiveBeginPlay`
  ;[1 1 1 1 30] Rotates towards player and fires when facing them
  (`KismetSystemLibrary.K2_SetTimerDelegate` (delegate `CustomUpdate`) (`self.CustomSecondsRotationUpdate`) true)
  (set `self.CurrentHealth` (`self.MaxHealth`)))

(event `CustomUpdate`
  ;[1 1 1 1 30] Rotates towards player and fires when facing them
  (`self.FindTarget`)
  (`self.Target`
    (:`then`
      (`self.UpdateRotation` (`self.CustomSecondsRotationUpdate`))
      (`self.UpdateFire`))
    (:`else`)))

(event `self.ReceiveAnyDamage`
  (params (Damage :type "Float (single-precision)") (DamageType :type "DamageType Object Reference") (InstigatedBy :type "Controller Object Reference") (DamageCauser :type "Actor Object Reference"))
  (`|ExecutionSequence`
    (:`then_0`
      (`/Engine/EditorBlueprintResources/StandardMacros.DoOnce` false
        (:`Completed`
          (bind _asalbatross_proto (cast `/Game/Blueprints/Enemies/Albatross/Albatross_Proto` (`self.AlbatrossOwner`))
            (:`then`
              (`|ExecutionSequence`
                (:`then_0`
                  (if (`self.IsTurret1`)
                    (set `/Game/Blueprints/Enemies/Albatross/Albatross_Proto.PlayerFightingTurret1` true _asalbatross_proto)
                    (`/Game/Blueprints/Enemies/Albatross/Albatross_Proto.TurretWasDamaged` _asalbatross_proto :!label _label)))
                (:`then_1`
                  (if (`self.IsTurret2`)
                    (set `/Game/Blueprints/Enemies/Albatross/Albatross_Proto.PlayerFightingTurret2` true _asalbatross_proto)
                    (goto _label)))
                (:`then_2`
                  (if (`self.IsTurret3`)
                    (set `/Game/Blueprints/Enemies/Albatross/Albatross_Proto.PlayerFightingTurret3` true _asalbatross_proto)
                    (goto _label)))))
            (:`CastFailed`
              (`KismetSystemLibrary.PrintString` "albatross cast failed"))))))
    (:`then_1`
      (`KismetSystemLibrary.PrintString` (`KismetStringLibrary.Conv_DoubleToString` Damage))
      ;[1 1 1 1 100] Destroys Enemy
      (set `self.CurrentHealth` (- (`self.CurrentHealth`) Damage))
      (`GameplayStatics.PlaySoundAtLocation` "/Game/Audio/SoundEffects/Player/stompBoom.stompBoom" (`self.K2_GetActorLocation`) (struct) 0.4 1.1 0.15 null null null null)
      (bind _asbpgm_volcanewt (cast `/Game/Blueprints/Systems/BPGM_Volcanewt` (`GameplayStatics.GetGameMode`)))
      (`/Game/Blueprints/Systems/BPGM_Volcanewt.EnemyDestroyed` _asbpgm_volcanewt (`self.EnemyMonetaryValue`))
      (`/Game/Blueprints/Systems/BPGM_Volcanewt.TurretsCount` _asbpgm_volcanewt)
      (if (<= (`self.CurrentHealth`) 0.0)
        (bind _asalbatross_proto_2 (cast `/Game/Blueprints/Enemies/Albatross/Albatross_Proto` (`self.AlbatrossOwner`)))
        (`/Game/Blueprints/Enemies/Albatross/Albatross_Proto.StopChargeDeathLaser` _asalbatross_proto_2)
        (`self.K2_DestroyActor`)))))

(event `Fire`
  (bind _firetransform (`self.FireTransform`))
  (bind (_returnvalue_location _returnvalue_rotation _returnvalue_scale) (`KismetMathLibrary.BreakTransform` (`SceneComponent.K2_GetComponentToWorld` _firetransform)))
  ;[1 1 1 1 30] Fires laser
  (set `self.TimeOfLastFire` (`KismetSystemLibrary.GetGameTimeInSeconds`))
  (`GameplayStatics.PlaySoundAtLocation` null (`self.K2_GetActorLocation`) (struct) 1.0 1.0 0.0 null null null null)
  (`NiagaraFunctionLibrary.SpawnSystemAtLocation` null (`SceneComponent.K2_GetComponentLocation` _firetransform) (struct) (0.001 0.001 0.001))
  (`|SpawnActorFromClass` "/Game/Blueprints/Projectiles/BP_Projectile_Alba.BP_Projectile_Alba_C" (`KismetMathLibrary.MakeTransform` _returnvalue_location _returnvalue_rotation (* _returnvalue_scale (`self.ProjectileScale`))) "AlwaysSpawn" "MultiplyWithRoot" null 300.0 0.0 0.0 null null false null null false 0.0 false 0.0 false null))

(fn `FindTarget`
  (set `self.BestDistance` (+ (`self.SensingRange`) 1.0))
  (bind _outactors (`KismetSystemLibrary.SphereOverlapActors` (`self.K2_GetActorLocation`) (`self.SensingRange`) (`|MakeArray` "ObjectTypeQuery3" :!type "EObjectTypeQuery Enum") "/Game/Player/Blueprints/BP_Volcanewt.BP_Volcanewt_C"))
  (for _array_element _outactors
    (bind _output_get (set `self.CurrentTarget` _array_element))
    (bind _output_get_2 (set `self.CurrentDistance` (`self.GetDistanceTo` _output_get self)))
    (if (or (< _output_get_2 (`self.BestDistance`)) (not (`KismetSystemLibrary.IsValid` (`self.BestTarget`))))
      (bind _result (`/Game/Blueprints/Libraries_and_Interfaces/BPFL_MuhFunctionLibrary.HasLineOfSight` (`SceneComponent.K2_GetComponentLocation` (`self.sm_turretCannonHead_v2`)) (`self.K2_GetActorLocation` (`self.CurrentTarget`)) (`|MakeArray` self null :!type "Actor Object Reference")))
      (if _result
        (set `self.BestTarget` (`self.CurrentTarget`))
        (set `self.BestDistance` (`self.CurrentDistance`)))))
  (set `self.Target` (`self.BestTarget`)))

(fn `UpdateFire`
  (bind _sm_turretcannonhead_v2 (`self.sm_turretCannonHead_v2`))
  (if (> (- (`KismetSystemLibrary.GetGameTimeInSeconds`) (`self.TimeOfLastFire`)) (`self.RateOfFire`))
    (if (> (`KismetMathLibrary.Dot_VectorVector` (`KismetMathLibrary.GetDirectionUnitVector` (`SceneComponent.K2_GetComponentLocation` _sm_turretcannonhead_v2) (`self.K2_GetActorLocation` (`self.Target`))) (`SceneComponent.GetForwardVector` _sm_turretcannonhead_v2)) 0.99)
      (`self.Fire`)
      (`KismetSystemLibrary.PrintString` "Firing ground turret"))))

(fn `UpdateRotation`
  (params (Seconds :type "Float (double-precision)"))
  (locals (NewRotation :type "Rotator Structure") (NewCannonRotation :type "Rotator Structure"))
  (bind _sm_turretneck_v2 (`self.sm_turretNeck_v2`))
  (bind _sm_turretcannonhead_v2 (`self.sm_turretCannonHead_v2`))
  ;[1 1 1] Turret base movement
  (bind _output_get (set `local.NewRotation` (`KismetMathLibrary.RInterpTo_Constant` (`SceneComponent.K2_GetComponentRotation` _sm_turretneck_v2) (`KismetMathLibrary.FindLookAtRotation` (`SceneComponent.K2_GetComponentLocation` _sm_turretneck_v2) (`self.K2_GetActorLocation` (`self.Target`))) (`local.Seconds`) (`self.RotationSpeed`))))
  (`SceneComponent.K2_SetWorldRotation` (`self.sm_turretNeck_v2`) (`KismetMathLibrary.MakeRotator` (.roll _output_get) (`KismetMathLibrary.ClampAngle` (.pitch _output_get)) (.yaw _output_get)) false false)
  ;[1 1 1] Turret cannon movement
  (bind _output_get_2 (set `local.NewCannonRotation` (`KismetMathLibrary.RInterpTo_Constant` (`SceneComponent.K2_GetComponentRotation` _sm_turretcannonhead_v2) (`KismetMathLibrary.FindLookAtRotation` (`SceneComponent.K2_GetComponentLocation` _sm_turretcannonhead_v2) (`self.K2_GetActorLocation` (`self.Target`))) (`self.CustomSecondsRotationUpdate`) (`self.RotationSpeed`))))
  (`SceneComponent.K2_SetWorldRotation` (`self.sm_turretCannonHead_v2`) (`KismetMathLibrary.MakeRotator` (.roll _output_get) (`KismetMathLibrary.ClampAngle` (.pitch _output_get_2) -45.0 45.0) (.yaw _output_get)) false false))

(fn `UserConstructionScript`
  (`self.SetOwner` (`self.AlbatrossOwner`)))