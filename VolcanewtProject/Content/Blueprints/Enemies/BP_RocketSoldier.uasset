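; Rocket soldier enemy that registers with the Volcanewt game mode on spawn and, on any damage, reports its monetary value and destroys itself.
; Pawn sensing writes AI blackboard keys, clearing player sight after a retriggerable delay, and starts a self-repeating delay loop that turns toward the player.
; AttackPlayer fires BP_Rocket when a forward sphere trace hits the player.
; Older roam and follow logic remains disconnected, noted as superseded by an AI tree.
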(event `self.ReceiveBeginPlay`
  ;[1 1 1 1 100] Event BeginPlay
  (bind _asbp_volcanewt (cast `/Game/Player/Blueprints/BP_Volcanewt` (`GameplayStatics.GetPlayerCharacter` 0)))
  (set `self.Char Ref` _asbp_volcanewt)
  (bind _asbpgm_volcanewt (cast `/Game/Blueprints/Systems/BPGM_Volcanewt` (`GameplayStatics.GetGameMode`)))
  (bind _output_get (set `self.As BPGM Volcanewt` _asbpgm_volcanewt))
  (`/Game/Blueprints/Systems/BPGM_Volcanewt.Increase Enemies` _output_get))

(event `self.ReceiveAnyDamage`
  (params (Damage :type "Float (single-precision)") (DamageType :type "DamageType Object Reference") (InstigatedBy :type "Controller Object Reference") (DamageCauser :type "Actor Object Reference"))
  ;[1 1 1 1 100] Destroys Enemy
  (`GameplayStatics.PlaySoundAtLocation` "/Game/Audio/SoundEffects/Player/stompBoom.stompBoom" (`self.K2_GetActorLocation`) (struct) 0.4 1.1 0.15 null null null null)
  (`/Game/Blueprints/Systems/BPGM_Volcanewt.EnemyDestroyed` (`/Game/Player/Blueprints/BP_Volcanewt.As BPGM Volcanewt` (`self.Char Ref`)) (`self.EnemyMonetaryValue`))
  (`self.K2_DestroyActor`))

(event `self.PawnSensing.OnSeePawn`
  (params (Pawn :type "Pawn Object Reference"))
  (bind _returnvalue (`AIBlueprintHelperLibrary.GetBlackboard` (`AIBlueprintHelperLibrary.GetAIController` self)))
  ;[1 1 1 1 30] On seeing the player, follow and attack them
  (bind _asbp_volcanewt (cast `/Game/Player/Blueprints/BP_Volcanewt` Pawn))
  (`self.FacePlayer`)
  (`BlackboardComponent.SetValueAsBool` _returnvalue "hasSeenPlayer?" true)
  (`BlackboardComponent.SetValueAsFloat` (`AIBlueprintHelperLibrary.GetBlackboard` (`AIBlueprintHelperLibrary.GetAIController` self)) "DistanceToPlayer" (`KismetStringLibrary.Conv_StringToDouble` (`KismetStringLibrary.Conv_Vector3fToString` (+ (`self.K2_GetActorLocation` self) (`self.K2_GetActorLocation` _asbp_volcanewt)))))
  (`KismetSystemLibrary.RetriggerableDelay` 0.6)
  (`BlackboardComponent.SetValueAsBool` _returnvalue "hasSeenPlayer?" false)
  (`|ExecutionSequence`
    (:`then_0`
      (if (`self.ActorHasTag` "Soldier")
        (`BlackboardComponent.SetValueAsBool` (`AIBlueprintHelperLibrary.GetBlackboard` (`AIBlueprintHelperLibrary.GetAIController` self)) "hasSeenOtherSoldier?" true)
        (else
          (`BlackboardComponent.SetValueAsBool` (`AIBlueprintHelperLibrary.GetBlackboard` (`AIBlueprintHelperLibrary.GetAIController` self)) "hasSeenOtherSoldier?" false))))))

(event `Roam Around`
  ;[1 1 1 1 70] This should all be redundant because it uses an AI tree now, but im scared to delet in case i need it -griffin
)

(event `AttackPlayer`
  (bind _returnvalue (`self.K2_GetActorLocation`))
  ;[1 1 1] Attack Player
  (bind (_outhit _returnvalue_2) (`KismetSystemLibrary.SphereTraceSingleForObjects` _returnvalue (+ _returnvalue (* (`KismetMathLibrary.GetForwardVector` (`self.K2_GetActorRotation`)) 1500.0)) 250.0 (`|MakeArray` "ObjectTypeQuery3" :!type "EObjectTypeQuery Enum")))
  (if _returnvalue_2
    (cast `/Game/Player/Blueprints/BP_Volcanewt` (`.HitActor` (`GameplayStatics.BreakHitResult` _outhit)))
    (`GameplayStatics.PlaySoundAtLocation` "/Game/Audio/SoundEffects/shootFree.shootFree" (`self.K2_GetActorLocation`) (struct) 1.0 1.0 0.0 null null null null)
    (`|SpawnActorFromClass` "/Game/Blueprints/Enemies/BP_Rocket.BP_Rocket_C" (`SceneComponent.K2_GetComponentToWorld` (`self.spawn proj loc`)) "AlwaysSpawn" "MultiplyWithRoot" null null)))

(event `self.ReceiveTick`
  (params (DeltaSeconds :type "Float (single-precision)"))
  ;[1 1 1 1 70] This should all be redundant because it uses an AI tree now, but im scared to delet in case i need it -griffin
)

(event `FacePlayer`
  (bind (_returnvalue_roll _returnvalue_pitch _returnvalue_yaw) (`KismetMathLibrary.BreakRotator` (`KismetMathLibrary.RInterpTo` (`self.K2_GetActorRotation`) (`KismetMathLibrary.FindLookAtRotation` (`self.K2_GetActorLocation`) (`self.K2_GetActorLocation` (`self.Char Ref`))) (`GameplayStatics.GetWorldDeltaSeconds`) 20.0)))
  ;[1 1 1] Rotate to face player
  (`self.K2_SetActorRotation` (`KismetMathLibrary.MakeRotator` 0.0 0.0 _returnvalue_yaw))
  (`KismetSystemLibrary.Delay` 0.001)
  (`self.FacePlayer`))

(event `Follow Player`
  ;[1 1 1 1 70] This should all be redundant because it uses an AI tree now, but im scared to delet in case i need it -griffin
)

(fn `UserConstructionScript`)