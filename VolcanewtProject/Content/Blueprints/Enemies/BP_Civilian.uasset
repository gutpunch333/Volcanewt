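; BP_Civilian is a civilian enemy character that reacts to the Volcanewt player and dies from any damage.
; Overlap with its Collision component by BP_Volcanewt sets "hasSeenPlayer" on the AI Blackboard for BT_Civilian.
; Damage stops movement, spawns a blood decal with a gulp sound, notifies BPGM_Volcanewt via EnemyDestroyed, then hides the actor and destroys it after a delay.
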(event `self.Collision.OnComponentBeginOverlap`
  (params (OverlappedComponent :type "PrimitiveComponent Object Reference") (OtherActor :type "Actor Object Reference") (OtherComp :type "PrimitiveComponent Object Reference") (OtherBodyIndex :type Integer) (bFromSweep :type Boolean) (SweepResult :type "HitResult Structure (by ref)"))
  ;[1 1 1] When sensing player
  (cast `/Game/Player/Blueprints/BP_Volcanewt` OtherActor)
  ;[1 1 1] Change the bool "hasSeenPlayer" to true in BT_Civilian
  (`BlackboardComponent.SetValueAsBool` (`AIBlueprintHelperLibrary.GetBlackboard` (`AIBlueprintHelperLibrary.GetAIController` self)) "hasSeenPlayer" true))

(event `self.ReceiveAnyDamage`
  (params (Damage :type "Float (single-precision)") (DamageType :type "DamageType Object Reference") (InstigatedBy :type "Controller Object Reference") (DamageCauser :type "Actor Object Reference"))
  (`MovementComponent.StopMovementImmediately` (`self.CharacterMovement`))
  (`GameplayStatics.SpawnDecalAtLocation` "/Game/PrototypingAssets/M_BloodCircle.M_BloodCircle" (50.0 50.0 50.0) (`self.K2_GetActorLocation`) (struct :`Pitch` -90.0) 10.0) ; Spawn blood pool when killed
  (`GameplayStatics.PlaySoundAtLocation` "/Game/Audio/SoundEffects/Player/gulp.gulp" (`self.K2_GetActorLocation`) (struct) 1.0 1.0 0.0 null null null null)
  (bind _asbpgm_volcanewt (cast `/Game/Blueprints/Systems/BPGM_Volcanewt` (`GameplayStatics.GetGameMode`)))
  (`/Game/Blueprints/Systems/BPGM_Volcanewt.EnemyDestroyed` _asbpgm_volcanewt 0.0)
  (`self.SetActorHiddenInGame` true)
  (`KismetSystemLibrary.Delay` 10.0)
  (`self.K2_DestroyActor`))

(fn `UserConstructionScript`)