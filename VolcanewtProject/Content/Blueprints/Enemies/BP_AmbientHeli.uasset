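; Ambient helicopter enemy that flies in a loop along a randomly chosen BP_HeliPath spline in the level.
; A looping timer advances its distance by the path's speed and sets its transform from the spline, wrapping to zero at the end.
; A gate holds movement until a random startup delay ends and the mesh is made visible.
; Any damage plays a boom, calls EnemyDestroyed with its monetary value and destroys it.
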(event `DestroyHeli`
  (`self.K2_DestroyActor`))

(event `Attach to Heli Path`
  (bind _allhelipathsarray (`self.AllHeliPathsArray`))
  (bind _asbp_heli_path (cast `/Game/Blueprints/BP_HeliPath` (`|GetArrayItem` _allhelipathsarray (`KismetMathLibrary.RandomInteger` (`KismetArrayLibrary.Array_Length` _allhelipathsarray)))))
  (set `self.HeliPathRef` _asbp_heli_path))

(event `self.ReceiveBeginPlay`
  ;[1 1 1 1 100] Event BeginPlay
  (`KismetSystemLibrary.K2_SetTimerDelegate` (delegate `UpdateRate`) (`self.CustomSeconds`) true)
  (`GameplayStatics.PlaySoundAtLocation` "/Game/Audio/SoundEffects/SoundCues/HelicopterBlades.HelicopterBlades" (`self.K2_GetActorLocation`) (struct) 1.0 1.0 0.0 null "/Game/Audio/SoundConcurrency/HelicopterBlades_SCC.HelicopterBlades_SCC" null null)
  (bind _outactors (`GameplayStatics.GetAllActorsOfClass` "/Game/Blueprints/BP_HeliPath.BP_HeliPath_C"))
  (set `self.AllHeliPathsArray` _outactors)
  (`self.Attach to Heli Path`)
  (set `self.StartingHeliDistance` 0.0)
  (`KismetSystemLibrary.Delay` (`KismetMathLibrary.RandomFloatInRange` 0.0 5.0))
  (`self.UnlockMovement`))

(event `UpdateRate`
  (bind _helipathref (`self.HeliPathRef`))
  (bind (_returnvalue_location _returnvalue_rotation) (`KismetMathLibrary.BreakTransform` (`SplineComponent.GetTransformAtDistanceAlongSpline` (`/Game/Blueprints/BP_HeliPath.Spline` _helipathref) (`self.HeliDistance`) "World" false)))
  (`/Engine/EditorBlueprintResources/StandardMacros.Gate` true :!label _label
    (:`Exit`
      (set `self.HeliDistance` (+ (* (`self.CustomSeconds`) (`/Game/Blueprints/BP_HeliPath.PathSpeed` _helipathref)) (`self.HeliDistance`)))
      (`self.K2_SetActorTransform` (`KismetMathLibrary.MakeTransform` (+ _returnvalue_location (0.0 0.0 0.0)) _returnvalue_rotation))
      (if (> (`self.HeliDistance`) (`SplineComponent.GetSplineLength` (`/Game/Blueprints/BP_HeliPath.Spline` (`self.HeliPathRef`))))
        (set `self.HeliDistance` 0.0)))))

(event `self.ReceiveAnyDamage`
  (params (Damage :type "Float (single-precision)") (DamageType :type "DamageType Object Reference") (InstigatedBy :type "Controller Object Reference") (DamageCauser :type "Actor Object Reference"))
  ;[1 1 1 1 100] Destroys Enemy
  (`GameplayStatics.PlaySoundAtLocation` "/Game/Audio/SoundEffects/Player/stompBoom.stompBoom" (`self.K2_GetActorLocation`) (struct) 0.4 1.1 0.15 null null null null)
  (bind _output_get (set `self.As BPGM Volcanewt` null))
  (`/Game/Blueprints/Systems/BPGM_Volcanewt.EnemyDestroyed` _output_get (`self.EnemyMonetaryValue`))
  (`self.K2_DestroyActor`))

(event `UnlockMovement`
  (`SceneComponent.SetVisibility` (`self.Mesh`) true false)
  (goto _label :!via `Open`))

(fn `UserConstructionScript`)