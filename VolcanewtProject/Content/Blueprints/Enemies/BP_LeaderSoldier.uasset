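; Leader soldier enemy for Volcanewt that registers with the game mode, finds its team's NPC manager and dies to any damage, reporting its value.
; Pawn sensing starts a self-repeating turn toward the player and sets a blackboard flag for the behavior tree.
; AttackPlayer sphere-traces for the player, then fires a projectile after a random delay to stagger volleys.
; Older roam and follow logic remains disconnected.
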(event `self.ReceiveBeginPlay`
  ;[1 1 1 1 100] Event BeginPlay
  (bind _asbp_volcanewt (cast `/Game/Player/Blueprints/BP_Volcanewt` (`GameplayStatics.GetPlayerCharacter` 0)))
  (set `self.Char Ref` _asbp_volcanewt)
  (bind _asbpgm_volcanewt (cast `/Game/Blueprints/Systems/BPGM_Volcanewt` (`GameplayStatics.GetGameMode`)))
  (bind _output_get (set `self.As BPGM Volcanewt` _asbpgm_volcanewt))
  (`/Game/Blueprints/Systems/BPGM_Volcanewt.Increase Enemies` _output_get)
  (`self.FindNPCManager`))

(event `self.ReceiveAnyDamage`
  (params (Damage :type "Float (single-precision)") (DamageType :type "DamageType Object Reference") (InstigatedBy :type "Controller Object Reference") (DamageCauser :type "Actor Object Reference"))
  (bind _as_bpgm_volcanewt (`/Game/Player/Blueprints/BP_Volcanewt.As BPGM Volcanewt` (`self.Char Ref`)))
  ;[1 1 1 1 100] Destroys Enemy
  (`MovementComponent.StopMovementImmediately` (`self.CharacterMovement`))
  (`self.SetActorEnableCollision` false)
  (`self.SetActorHiddenInGame` true)
  (`GameplayStatics.SpawnDecalAtLocation` "/Game/PrototypingAssets/M_BloodCircle.M_BloodCircle" (50.0 50.0 50.0) (`self.K2_GetActorLocation`))
  (`GameplayStatics.PlaySoundAtLocation` "/Game/Audio/SoundEffects/Player/stompBoom.stompBoom" (`self.K2_GetActorLocation`) (struct) 0.4 1.1 0.15 null null null null)
  (`/Game/Blueprints/Systems/BPGM_Volcanewt.EnemyDestroyed` _as_bpgm_volcanewt (`self.EnemyMonetaryValue`))
  (`/Game/Blueprints/Systems/BPGM_Volcanewt.SoldierCount` _as_bpgm_volcanewt)
  (`KismetSystemLibrary.Delay` 5.0)
  (`self.K2_DestroyActor`))

(event `self.PawnSensing.OnSeePawn`
  (params (Pawn :type "Pawn Object Reference"))
  (bind _returnvalue (`AIBlueprintHelperLibrary.GetBlackboard` (`AIBlueprintHelperLibrary.GetAIController` self)))
  ;[1 1 1 1 30] On seeing the player, follow and attack them
  (`/Engine/EditorBlueprintResources/StandardMacros.FlipFlop`
    (:`A`
      (`self.FacePlayer`)
      (if (`self.ActorHasTag` Pawn "Newt") :!label _label
        (cast `/Game/Player/Blueprints/BP_Volcanewt` Pawn)
        (`BlackboardComponent.SetValueAsBool` _returnvalue "hasSeenPlayer?" true)
        (`KismetSystemLibrary.RetriggerableDelay` 0.6)
        (goto _label)
        (else
          (`BlackboardComponent.SetValueAsBool` _returnvalue "hasSeenPlayer?" false)
          (`KismetSystemLibrary.RetriggerableDelay` 0.6)
          (goto _label))))))

(event `Roam Around`
  ;[1 1 1 1 70] This should all be redundant because it uses an AI tree now, but im scared to delet in case i need it -griffin
)

(event `AttackPlayer`
  (bind _returnvalue (`self.K2_GetActorLocation`))
  ;[1 1 1] Attack Player
  (bind (_outhit _returnvalue_2) (`KismetSystemLibrary.SphereTraceSingleForObjects` _returnvalue (+ _returnvalue (* (`KismetMathLibrary.GetForwardVector` (`self.K2_GetActorRotation`)) 1500.0)) 2000.0 (`|MakeArray` "ObjectTypeQuery3" :!type "EObjectTypeQuery Enum")))
  (if _returnvalue_2
    (cast `/Game/Player/Blueprints/BP_Volcanewt` (`.HitActor` (`GameplayStatics.BreakHitResult` _outhit)))
    (`KismetSystemLibrary.Delay` (`KismetMathLibrary.RandomFloatInRange` (`self.RandomFireMin`) (`self.RandomFireMax`))) ; Random delay so troops don't fire a same time
    (`GameplayStatics.PlaySoundAtLocation` "/Game/Audio/SoundEffects/shootFree.shootFree" (`self.K2_GetActorLocation`) (struct) 1.0 1.0 0.0 null null null null)
    (`|SpawnActorFromClass` "/Game/Blueprints/Enemies/ProjectilesEtc/BP_TestProjectile.BP_TestProjectile_C" (`SceneComponent.K2_GetComponentToWorld` (`self.spawn proj loc`)) "AlwaysSpawn" "MultiplyWithRoot" null null)
    (`KismetSystemLibrary.Delay` 1.5)))

(event `FacePlayer`
  (bind (_returnvalue_roll _returnvalue_pitch _returnvalue_yaw) (`KismetMathLibrary.BreakRotator` (`KismetMathLibrary.RInterpTo` (`self.K2_GetActorRotation`) (`KismetMathLibrary.FindLookAtRotation` (`self.K2_GetActorLocation`) (`self.K2_GetActorLocation` (`self.Char Ref`))) (`GameplayStatics.GetWorldDeltaSeconds`) 10.0)))
  ;[1 1 1] Rotate to face player (not used atm for basic soldier because they tend to hitch at a certain interval, plus they chase the player constantly anyway. But it's here in case we need it)
  (`self.K2_SetActorRotation` (`KismetMathLibrary.MakeRotator` 0.0 0.0 _returnvalue_yaw))
  (`KismetSystemLibrary.Delay` 0.001)
  (`self.FacePlayer`))

(event `SetAlerted`
  (params (NewState :type "/Game/Blueprints/Enemies/AlertState Enum" :default "NewEnumerator0"))
  (set `self.AlertState` "NewEnumerator1"))

(event `Follow Player`
  ;[1 1 1 1 70] This should all be redundant because it uses an AI tree now, but im scared to delet in case i need it -griffin
)

(fn `UserConstructionScript`)