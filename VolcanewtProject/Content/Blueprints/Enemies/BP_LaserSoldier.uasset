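; Laser soldier enemy that spots the player, fires laser projectiles, and on any damage dies and reports its monetary value to the game mode.
; Pawn sensing starts a self-repeating delay loop to face the player and writes sighting keys to the Blackboard.
; AttackPlayer widens a Niagara aiming laser per call until LaserDelay, then sphere-traces, fires and flashes the big laser.
; An AI tree supersedes the disconnected roam and follow logic.
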(event `self.ReceiveBeginPlay`
  ;[1 1 1 1 100] Event BeginPlay
  (`SceneComponent.SetVisibility` (`self.SmallLaser`) false false)
  (bind _asbp_volcanewt (cast `/Game/Player/Blueprints/BP_Volcanewt` (`GameplayStatics.GetPlayerCharacter` 0)))
  (set `self.Char Ref` _asbp_volcanewt))

(event `self.ReceiveAnyDamage`
  (params (Damage :type "Float (single-precision)") (DamageType :type "DamageType Object Reference") (InstigatedBy :type "Controller Object Reference") (DamageCauser :type "Actor Object Reference"))
  ;[1 1 1 1 100] Destroys Enemy
  (`GameplayStatics.PlaySoundAtLocation` "/Game/Audio/SoundEffects/Player/stompBoom.stompBoom" (`self.K2_GetActorLocation`) (struct) 0.4 1.1 0.15 null null null null)
  (`/Game/Blueprints/Systems/BPGM_Volcanewt.EnemyDestroyed` (`/Game/Player/Blueprints/BP_Volcanewt.As BPGM Volcanewt` (`self.Char Ref`)) (`self.EnemyMonetaryValue`))
  (`self.K2_DestroyActor`))

(event `self.PawnSensing.OnSeePawn`
  (params (Pawn :type "Pawn Object Reference"))
  (bind _returnvalue (`AIBlueprintHelperLibrary.GetBlackboard` (`AIBlueprintHelperLibrary.GetAIController` self)))
  ;[1 1 1 1 30] On seeing the player, follow and attack them
  (bind _asbp_volcanewt (cast `/Game/Player/Blueprints/BP_Volcanewt` Pawn))
  (`self.FacePlayer`)
  (`BlackboardComponent.SetValueAsBool` (`AIBlueprintHelperLibrary.GetBlackboard` (`AIBlueprintHelperLibrary.GetAIController` self)) "hasSeenPlayer?" true)
  (`BlackboardComponent.SetValueAsFloat` _returnvalue "DistanceToPlayer" (`KismetStringLibrary.Conv_StringToDouble` (`KismetStringLibrary.Conv_Vector3fToString` (+ (`self.K2_GetActorLocation` self) (`self.K2_GetActorLocation` _asbp_volcanewt)))))
  (`KismetSystemLibrary.RetriggerableDelay` 0.6)
  (`BlackboardComponent.SetValueAsBool` _returnvalue "hasSeenPlayer?" false)
  (`|ExecutionSequence`
    (:`then_0`
      (if (`self.ActorHasTag` "Soldier")
        (`BlackboardComponent.SetValueAsBool` (`AIBlueprintHelperLibrary.GetBlackboard` (`AIBlueprintHelperLibrary.GetAIController` self)) "hasSeenOtherSoldier?" true)
        (else
          (`BlackboardComponent.SetValueAsBool` (`AIBlueprintHelperLibrary.GetBlackboard` (`AIBlueprintHelperLibrary.GetAIController` self)) "hasSeenOtherSoldier?" false))))))

(event `Roam Around`
  ;[1 1 1 1 70] This should all be redundant because it uses an AI tree now, but im scared to delet in case i need it -griffin
)

(event `AttackPlayer`
  (bind _returnvalue (`self.K2_GetActorLocation`))
  ;[1 1 1] Attack Player
  (if (== (`self.DelayCount`) (`self.LaserDelay`))
    (`KismetSystemLibrary.Delay` (`self.LaserDelay`))
    (bind (_outhit _returnvalue_2) (`KismetSystemLibrary.SphereTraceSingleForObjects` _returnvalue (+ _returnvalue (* (`KismetMathLibrary.GetForwardVector` (`self.K2_GetActorRotation`)) 1500.0)) 2500.0 (`|MakeArray` "ObjectTypeQuery3" :!type "EObjectTypeQuery Enum")))
    (if _returnvalue_2
      (cast `/Game/Player/Blueprints/BP_Volcanewt` (`.HitActor` (`GameplayStatics.BreakHitResult` _outhit)))
      (`GameplayStatics.PlaySoundAtLocation` "/Game/Audio/SoundEffects/shootFree.shootFree" (`self.K2_GetActorLocation`) (struct) 1.0 1.0 0.0 null null null null)
      (`|SpawnActorFromClass` "/Game/Blueprints/Enemies/ProjectilesEtc/BP_LaserProjectile.BP_LaserProjectile_C" (`SceneComponent.K2_GetComponentToWorld` (`self.spawn proj loc`)) "AlwaysSpawn" "MultiplyWithRoot" null null)
      (`SceneComponent.SetVisibility` (`self.BigLaser`) true false)
      (`|ExecutionSequence`
        (:`then_0`
          (`KismetSystemLibrary.Delay` 0.5)
          (`SceneComponent.SetVisibility` (`self.BigLaser`) false false))
        (:`then_1`
          (`KismetSystemLibrary.Delay` 1.5)
          (`SceneComponent.SetVisibility` (`self.SmallLaser`) false false))))
    (else
      (bind _newradius (`self.SmallLaserIncreaseWidth` (`self.DelayCount`)))
      (set `self.SmallLaserRadius` _newradius)
      (`/Engine/EditorBlueprintResources/StandardMacros.IncrementFloat` (`self.DelayCount`)))))

(event `self.ReceiveTick`
  (params (DeltaSeconds :type "Float (single-precision)"))
  ;[1 1 1 1 70] This should all be redundant because it uses an AI tree now, but im scared to delet in case i need it -griffin
)

(event `FacePlayer`
  (bind (_returnvalue_roll _returnvalue_pitch _returnvalue_yaw) (`KismetMathLibrary.BreakRotator` (`KismetMathLibrary.RInterpTo` (`self.K2_GetActorRotation`) (`KismetMathLibrary.FindLookAtRotation` (`self.K2_GetActorLocation`) (`self.K2_GetActorLocation` (`self.Char Ref`))) (`GameplayStatics.GetWorldDeltaSeconds`) 20.0)))
  ;[1 1 1] Rotate to face player
  (`self.K2_SetActorRotation` (`KismetMathLibrary.MakeRotator` 0.0 0.0 _returnvalue_yaw))
  (`SceneComponent.SetVisibility` (`self.SmallLaser`) true false)
  (`KismetSystemLibrary.Delay` 0.001)
  (`self.FacePlayer`))

(event `Follow Player`
  ;[1 1 1 1 70] This should all be redundant because it uses an AI tree now, but im scared to delet in case i need it -griffin
)

(fn `SmallLaserIncreaseWidth`
  (params (LaserFuncCount :type "Float (double-precision)"))
  (returns (NewRadius :type "Float (double-precision)"))
  (bind _returnvalue (* LaserFuncCount (`self.SmallLaserRadius`)))
  (`|ExecutionSequence`
    (:`then_0`
      (`NiagaraComponent.SetVariableFloat` (`self.SmallLaser`) "User LaserWidth" _returnvalue)
      (return _returnvalue))))

(fn `UserConstructionScript`)