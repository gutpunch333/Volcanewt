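; Birthday cake boss (B.I.R.T.H.D.A.Y) with three stacked turret tiers and an on-screen boss health bar.
; Tick targets the nearest visible Volcanewt, rotates each living turret toward it, and fires projectiles when cooled down and aligned.
; Non-enemy damage lowers health, exploding and hiding tiers top to bottom at fixed thresholds until death removes the bar.
; Pawn sensing separately sets a blackboard flag for seeing the player.
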(event `self.ReceiveBeginPlay`
  (bind _bosshealthbarwbp (`self.BossHealthBarWBP`))
  (`|ExecutionSequence`
    (:`then_0`
      ;[1 1 1] Sets boss health and disables it at start
      (set `self.CurrentHealth` (`self.MaxHealth`)))
    (:`then_1`
      (bind _returnvalue (`|CreateWidget` "/Game/UI/Widgets/WBP_BossHealthBar.WBP_BossHealthBar_C" (`GameplayStatics.GetPlayerController` 0)))
      (bind _output_get (set `self.BossHealthBarWBP` _returnvalue))
      (`UserWidget.AddToViewport` _output_get 0)
      (`/Game/UI/Widgets/WBP_BossHealthBar.SetBossBarName` _bosshealthbarwbp "B.I.R.T.H.D.A.Y")
      (`/Game/UI/Widgets/WBP_BossHealthBar.SetBossOwner` _bosshealthbarwbp self))))

(event `Enable Boss`
  ;[1 1 1] Enables boss
  (set `self.CurrentHealth` (`self.MaxHealth`))
  (`SceneComponent.SetVisibility` (`self.Mesh`) true true))

(event `self.ReceiveTick`
  (params (DeltaSeconds :type "Float (single-precision)"))
  (if (not (`self.IsDead`))
    ;[1 1 1] Rotates to player and fires turrets
    (`self.FindTarget`)
    (`self.Target`
      (:`then`
        (`self.UpdateBottomTurretRotation` DeltaSeconds)
        (`self.UpdateFireBottom`)
        (if (`self.IsMidAlive`)
          (`self.UpdateMiddleTurretRotation` DeltaSeconds)
          (`self.UpdateFireMiddle`)
          (if (`self.IsTopAlive`)
            (`self.UpdateTopTurretRotation` DeltaSeconds)
            (`self.UpdateFireTop`))))
      (:`else`))))

(event `FireTop`
  ;[1 1 1] Fire each turret
  (set `self.TimeOfLastFireTop` (`KismetSystemLibrary.GetGameTimeInSeconds`))
  (`|SpawnActorFromClass` "/Game/Blueprints/Enemies/ProjectilesEtc/BP_BdayCakeTop.BP_BdayCakeTop_C" (`SceneComponent.K2_GetComponentToWorld` (`self.TopFireLocationR`)) "AlwaysSpawn" "MultiplyWithRoot" null null)
  (`|SpawnActorFromClass` "/Game/Blueprints/Enemies/ProjectilesEtc/BP_BdayCakeTop.BP_BdayCakeTop_C" (`SceneComponent.K2_GetComponentToWorld` (`self.TopFireLocationL`)) "AlwaysSpawn" "MultiplyWithRoot" null null))

(event `self.ReceiveAnyDamage`
  (params (Damage :type "Float (single-precision)") (DamageType :type "DamageType Object Reference") (InstigatedBy :type "Controller Object Reference") (DamageCauser :type "Actor Object Reference"))
  (bind _bottomturretrotation (`self.BottomTurretRotation`))
  (bind _middleturretrotation (`self.MiddleTurretRotation`))
  (bind _topturretrotation (`self.TopTurretRotation`))
  ;[1 1 1] Boss health manager
  (if (`self.IsDead`)
    _
    (elif (not (`self.ActorHasTag` DamageCauser "EnemyUnit"))
      (bind _output_get (set `self.CurrentHealth` (- (`self.CurrentHealth`) Damage)))
      (`/Game/UI/Widgets/WBP_BossHealthBar.UpdateBossBarHealth` (`self.BossHealthBarWBP`) _output_get (`self.MaxHealth`))
      (if (<= (`self.CurrentHealth`) 1250.0)
        (set `self.IsTopAlive` false)
        (`NiagaraFunctionLibrary.SpawnSystemAtLocation` "/Game/VFX/Effects/FXS_Explosion.FXS_Explosion" (`SceneComponent.K2_GetComponentLocation` _topturretrotation)) ; Seems to be too much to have on the top turret, as they fire more rapidly
        (`SceneComponent.SetHiddenInGame` _topturretrotation true false)
        (`SceneComponent.SetHiddenInGame` (`self.TopTurretRight`) true false)
        (`SceneComponent.SetHiddenInGame` (`self.TopTurretLeft`) true false)
        (if (<= (`self.CurrentHealth`) 500.0)
          (set `self.IsMidAlive` false)
          (`NiagaraFunctionLibrary.SpawnSystemAtLocation` "/Game/VFX/Effects/FXS_Explosion.FXS_Explosion" (`SceneComponent.K2_GetComponentLocation` _middleturretrotation)) ; Seems to be too much to have on the top turret, as they fire more rapidly
          (`SceneComponent.SetHiddenInGame` _middleturretrotation true false)
          (`SceneComponent.SetHiddenInGame` (`self.MiddleTurret`) true false)
          (if (<= (`self.CurrentHealth`) 0.0)
            (`NiagaraFunctionLibrary.SpawnSystemAtLocation` "/Game/VFX/Effects/FXS_Explosion.FXS_Explosion" (`SceneComponent.K2_GetComponentLocation` _bottomturretrotation)) ; Seems to be too much to have on the top turret, as they fire more rapidly
            (set `self.IsDead` true)
            (`SceneComponent.SetHiddenInGame` _bottomturretrotation true false)
            (`SceneComponent.SetHiddenInGame` (`self.BottomTurret`) true false)
            (`/Game/UI/Widgets/WBP_BossHealthBar.RemoveBossBarFromHUD` (`self.BossHealthBarWBP`))))))))

(event `FireMiddle`
  (bind _middlefirelocation (`self.MiddleFireLocation`))
  ;[1 1 1] Fire each turret
  (set `self.TimeOfLastFireMid` (`KismetSystemLibrary.GetGameTimeInSeconds`))
  (`GameplayStatics.PlaySoundAtLocation` "/Game/Audio/SoundEffects/shootFree.shootFree" (`self.K2_GetActorLocation`) (struct) 1.0 1.0 0.0 null null null null)
  (`NiagaraFunctionLibrary.SpawnSystemAtLocation` "/Game/VFX/Effects/FXS_Explosion.FXS_Explosion" (`SceneComponent.K2_GetComponentLocation` _middlefirelocation) (struct) (0.003 0.003 0.003))
  (`|SpawnActorFromClass` "/Game/Blueprints/Enemies/ProjectilesEtc/BP_BdayCakeMid.BP_BdayCakeMid_C" (`SceneComponent.K2_GetComponentToWorld` _middlefirelocation) "AlwaysSpawn" "MultiplyWithRoot" null null))

(event `FireBottom`
  (bind _bottomfirelocation (`self.BottomFireLocation`))
  ;[1 1 1] Fire each turret
  (set `self.TimeOfLastFireBottom` (`KismetSystemLibrary.GetGameTimeInSeconds`))
  (`GameplayStatics.PlaySoundAtLocation` "/Game/Audio/SoundEffects/shootFree.shootFree" (`self.K2_GetActorLocation`) (struct) 1.0 1.0 0.0 null null null null)
  (`NiagaraFunctionLibrary.SpawnSystemAtLocation` "/Game/VFX/Effects/FXS_Explosion.FXS_Explosion" (`SceneComponent.K2_GetComponentLocation` _bottomfirelocation) (struct) (0.003 0.003 0.003))
  (`|SpawnActorFromClass` "/Game/Blueprints/Enemies/ProjectilesEtc/BP_BdayCakeBottom.BP_BdayCakeBottom_C" (`SceneComponent.K2_GetComponentToWorld` _bottomfirelocation) "AlwaysSpawn" "MultiplyWithRoot" null null))

(event `self.PawnSensing.OnSeePawn`
  (params (Pawn :type "Pawn Object Reference"))
  (bind _returnvalue (`AIBlueprintHelperLibrary.GetBlackboard` (`AIBlueprintHelperLibrary.GetAIController` self)))
  ;[1 1 1 1 30] On seeing the player, follow them (copied from basic/helicopter enemy script)
  (if (`self.ActorHasTag` Pawn "Newt") :!label _label
    (cast `/Game/Player/Blueprints/BP_Volcanewt` Pawn)
    (`BlackboardComponent.SetValueAsBool` _returnvalue "hasSeenPlayer?" true)
    (else
      (`BlackboardComponent.SetValueAsBool` _returnvalue "hasSeenPlayer?" false)
      (`KismetSystemLibrary.RetriggerableDelay` 0.6)
      (goto _label))))

(fn `FindTarget`
  (locals (BestDistance :type "Float (double-precision)") (CurrentDistance :type "Float (double-precision)") (BestTarget :type "Actor Object Reference") (CurrentTarget :type "Actor Object Reference"))
  ;[1 1 1] Determines best target and ensures it can be seen
  (set `local.BestDistance` (+ (`self.SensingRange`) 1.0))
  (bind _outactors (`KismetSystemLibrary.SphereOverlapActors` (`self.K2_GetActorLocation`) (`self.SensingRange`) (`|MakeArray` "ObjectTypeQuery3" :!type "EObjectTypeQuery Enum") "/Game/Player/Blueprints/BP_Volcanewt.BP_Volcanewt_C"))
  (for _array_element _outactors
    (bind _output_get (set `local.CurrentTarget` _array_element))
    (bind _output_get_2 (set `local.CurrentDistance` (`self.GetDistanceTo` _output_get self)))
    (if (or (< _output_get_2 (`local.BestDistance`)) (not (`KismetSystemLibrary.IsValid` (`local.BestTarget`))))
      (bind _result (`/Game/Blueprints/Libraries_and_Interfaces/BPFL_MuhFunctionLibrary.HasLineOfSight` (`SceneComponent.K2_GetComponentLocation` (`self.Mesh`)) (`self.K2_GetActorLocation` (`local.CurrentTarget`)) (`|MakeArray` self (`local.CurrentTarget`) :!type "Actor Object Reference")))
      (if _result
        (set `local.BestTarget` (`local.CurrentTarget`))
        (set `local.BestDistance` (`local.CurrentDistance`)))))
  (set `self.Target` (`local.BestTarget`)))

(fn `UpdateBottomTurretRotation`
  (params (DeltaSeconds :type "Float (double-precision)"))
  (locals (NewRotation :type "Rotator Structure" :default (struct)) (NewRotationBarrelBot :type "Rotator Structure" :default (struct)))
  (bind _bottomturretrotation (`self.BottomTurretRotation`))
  (bind _bottomturret (`self.BottomTurret`))
  ;[1 1 1] Turret rotation (left and right only)
  (bind _output_get (set `local.NewRotation` (`KismetMathLibrary.RInterpTo_Constant` (`SceneComponent.K2_GetComponentRotation` _bottomturretrotation) (`KismetMathLibrary.FindLookAtRotation` (`SceneComponent.K2_GetComponentLocation` _bottomturretrotation) (`self.K2_GetActorLocation` (`self.Target`))) (`local.DeltaSeconds`) (`self.BottomRotationSpeed`))))
  (`SceneComponent.K2_SetWorldRotation` (`self.BottomTurretRotation`) (`KismetMathLibrary.MakeRotator` (.roll _output_get) (`KismetMathLibrary.ClampAngle` (.pitch _output_get)) (.yaw _output_get)) false false)
  ;[1 1 1] Barrel rotation (up and down only)
  (bind _output_get_2 (set `local.NewRotationBarrelBot` (`KismetMathLibrary.RInterpTo_Constant` (`SceneComponent.K2_GetComponentRotation` _bottomturret) (`KismetMathLibrary.FindLookAtRotation` (`SceneComponent.K2_GetComponentLocation` _bottomturret) (`self.K2_GetActorLocation` (`self.Target`))) (`local.DeltaSeconds`) (`self.BottomRotationSpeed`))))
  (`SceneComponent.K2_SetWorldRotation` (`self.BottomTurret`) (`KismetMathLibrary.MakeRotator` (.pitch _output_get) (`KismetMathLibrary.ClampAngle` (.pitch _output_get_2) -45.0 45.0) (.yaw _output_get)) false false))

(fn `UpdateFireBottom`
  (bind _bottomturretrotation (`self.BottomTurretRotation`))
  ;[1 1 1 1 24] Checks if turret has cooldown and is facing target, fires if both are true
  (if (> (- (`KismetSystemLibrary.GetGameTimeInSeconds`) (`self.TimeOfLastFireBottom`)) (`self.RateOfFireBottom`))
    (if (> (`KismetMathLibrary.Dot_VectorVector` (`KismetMathLibrary.GetDirectionUnitVector` (`SceneComponent.K2_GetComponentLocation` _bottomturretrotation) (`self.K2_GetActorLocation` (`self.Target`))) (`SceneComponent.GetForwardVector` _bottomturretrotation)) 0.99)
      (`self.FireBottom`)
      (`KismetSystemLibrary.PrintString` "Firing bottom"))))

(fn `UpdateFireMiddle`
  ;[1 1 1 1 24] Checks if turret has cooldown and is facing target, fires if both are true
  (if (> (- (`KismetSystemLibrary.GetGameTimeInSeconds`) (`self.TimeOfLastFireMid`)) (`self.RateOfFireMid`))
    (if (> (`KismetMathLibrary.Dot_VectorVector` (`KismetMathLibrary.GetDirectionUnitVector` (`SceneComponent.K2_GetComponentLocation` (`self.MiddleTurretRotation`)) (`self.K2_GetActorLocation` (`self.Target`))) (`SceneComponent.GetForwardVector` (`self.MiddleTurretRotation`))) 0.99)
      (`self.FireMiddle`)
      (`KismetSystemLibrary.PrintString` "Firing mid"))))

(fn `UpdateFireTop`
  (bind _topturretrotation (`self.TopTurretRotation`))
  ;[1 1 1 1 24] Checks if turret has cooldown and is facing target, fires if both are true
  (if (> (- (`KismetSystemLibrary.GetGameTimeInSeconds`) (`self.TimeOfLastFireTop`)) (`self.RateOfFireTop`))
    (if (> (`KismetMathLibrary.Dot_VectorVector` (`KismetMathLibrary.GetDirectionUnitVector` (`SceneComponent.K2_GetComponentLocation` _topturretrotation) (`self.K2_GetActorLocation` (`self.Target`))) (`SceneComponent.GetForwardVector` _topturretrotation)) 0.99)
      (`self.FireTop`)
      (`KismetSystemLibrary.PrintString` "Firing top "))))

(fn `UpdateMiddleTurretRotation`
  (params (DeltaSeconds :type "Float (double-precision)"))
  (locals (NewRotation :type "Rotator Structure" :default (struct)) (NewRotationBarrel :type "Rotator Structure" :default (struct)))
  (bind _middleturret (`self.MiddleTurret`))
  (bind _middleturretrotation (`self.MiddleTurretRotation`))
  ;[1 1 1] Comment
  (bind _output_get (set `local.NewRotation` (`KismetMathLibrary.RInterpTo_Constant` (`SceneComponent.K2_GetComponentRotation` _middleturretrotation) (`KismetMathLibrary.FindLookAtRotation` (`SceneComponent.K2_GetComponentLocation` _middleturretrotation) (`self.K2_GetActorLocation` (`self.Target`))) (`local.DeltaSeconds`) (`self.MiddleRotationSpeed`))))
  (`SceneComponent.K2_SetWorldRotation` (`self.MiddleTurretRotation`) (`KismetMathLibrary.MakeRotator` (.roll _output_get) (`KismetMathLibrary.ClampAngle` (.pitch _output_get)) (.yaw _output_get)) false false)
  ;[1 1 1] Barrel rotation (up and down only)
  (bind _output_get_2 (set `local.NewRotationBarrel` (`KismetMathLibrary.RInterpTo_Constant` (`SceneComponent.K2_GetComponentRotation` _middleturret) (`KismetMathLibrary.FindLookAtRotation` (`SceneComponent.K2_GetComponentLocation` _middleturret) (`self.K2_GetActorLocation` (`self.Target`))) (`local.DeltaSeconds`) (`self.MiddleRotationSpeed`))))
  (`SceneComponent.K2_SetWorldRotation` (`self.MiddleTurret`) (`KismetMathLibrary.MakeRotator` (.roll _output_get) (`KismetMathLibrary.ClampAngle` (.pitch _output_get_2) -45.0 45.0) (.yaw _output_get)) false false))

(fn `UpdateTopTurretRotation`
  (params (DeltaSeconds :type "Float (double-precision)"))
  (locals (NewRotation :type "Rotator Structure" :default (struct)) (NewRotationBarrels :type "Rotator Structure" :default (struct)))
  (bind _topturretrotation (`self.TopTurretRotation`))
  (bind _topturretrotation_2 (`self.TopTurretRotation`))
  ;[1 1 1] Turret rotation (left and right)
  (bind _output_get (set `local.NewRotation` (`KismetMathLibrary.RInterpTo_Constant` (`SceneComponent.K2_GetComponentRotation` _topturretrotation_2) (`KismetMathLibrary.FindLookAtRotation` (`SceneComponent.K2_GetComponentLocation` _topturretrotation_2) (`self.K2_GetActorLocation` (`self.Target`))) (`local.DeltaSeconds`) (`self.TopRotationSpeed`))))
  (`SceneComponent.K2_SetWorldRotation` (`self.TopTurretRotation`) (`KismetMathLibrary.MakeRotator` (.roll _output_get) (`KismetMathLibrary.ClampAngle` (.pitch _output_get)) (.yaw _output_get)) false false)
  ;[1 1 1] Barrel rotation (up and down only)
  (bind _output_get_2 (set `local.NewRotationBarrels` (`KismetMathLibrary.RInterpTo_Constant` (`SceneComponent.K2_GetComponentRotation` _topturretrotation) (`KismetMathLibrary.FindLookAtRotation` (`SceneComponent.K2_GetComponentLocation` _topturretrotation) (`self.K2_GetActorLocation` (`self.Target`))) (`local.DeltaSeconds`) (`self.TopRotationSpeed`))))
  (`SceneComponent.K2_SetWorldRotation` (`self.TopTurretRotation`) (`KismetMathLibrary.MakeRotator` (.roll _output_get) (`KismetMathLibrary.ClampAngle` (.pitch _output_get_2) -45.0 45.0) (.yaw _output_get)) false false))

(fn `UserConstructionScript`)