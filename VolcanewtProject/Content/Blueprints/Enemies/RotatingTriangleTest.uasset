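; Test enemy indicator actor with a triangle sprite that turns to face the player on the yaw axis.
; A looping timer eases yaw toward the target, starting either at BeginPlay or, in sphere mode, while a character overlaps the sphere.
; The construction script sets the owner and scales sprite and sphere, dividing out the image scale for the sphere.
; The timed rotation also destroys the actor once its owning actor is invalid.
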(event `self.ReceiveBeginPlay`
  (if (not (`self.IsUsingSphere`))
    (set `self.CharacterReference` (`GameplayStatics.GetPlayerCharacter` 0))
    (bind _returnvalue (`KismetSystemLibrary.K2_SetTimerDelegate` (delegate `Rotate`) (`self.RotationSpeed`) true :!label _label))
    (set `self.TimerHandle` _returnvalue)))

(event `self.Sphere.OnComponentBeginOverlap`
  (params (OverlappedComponent :type "PrimitiveComponent Object Reference") (OtherActor :type "Actor Object Reference") (OtherComp :type "PrimitiveComponent Object Reference") (OtherBodyIndex :type Integer) (bFromSweep :type Boolean) (SweepResult :type "HitResult Structure (by ref)"))
  (if (`self.IsUsingSphere`)
    (bind _ascharacter (cast `Character` OtherActor))
    (set `self.CharacterReference` _ascharacter)
    (goto _label)))

(event `Rotate`
  (bind (_returnvalue_roll _returnvalue_pitch _returnvalue_yaw) (`KismetMathLibrary.BreakRotator` (`KismetMathLibrary.RInterpTo` (`self.K2_GetActorRotation`) (`KismetMathLibrary.FindLookAtRotation` (`self.K2_GetActorLocation`) (`self.K2_GetActorLocation` (`self.CharacterReference`))) (`GameplayStatics.GetWorldDeltaSeconds`) (`self.Interpolation Speed`))))
  (`self.K2_SetActorRotation` (`KismetMathLibrary.MakeRotator` 0.0 0.0 _returnvalue_yaw))
  (if (not (`KismetSystemLibrary.IsValid` (`self.ActorWhoOwnsRotatingImage`)))
    (`self.K2_DestroyActor`)))

(event `self.Sphere.OnComponentEndOverlap`
  (params (OverlappedComponent :type "PrimitiveComponent Object Reference") (OtherActor :type "Actor Object Reference") (OtherComp :type "PrimitiveComponent Object Reference") (OtherBodyIndex :type Integer))
  (if (`self.IsUsingSphere`)
    (`KismetSystemLibrary.K2_ClearAndInvalidateTimerHandle` (`self.TimerHandle`))))

(fn `UserConstructionScript`
  (bind _triangle5_sprite (`self.triangle5_Sprite`))
  (bind _sphere (`self.Sphere`))
  (bind _returnvalue (/ (* (`SphereComponent.GetShapeScale` _sphere) (`self.SphereScaleFactor`)) (`self.ImageScaleFactor`)))
  (`self.SetOwner` (`self.ActorWhoOwnsRotatingImage`))
  (`SceneComponent.SetRelativeScale3D` _triangle5_sprite (* (`SceneComponent.K2_GetComponentScale` _triangle5_sprite) (`self.ImageScaleFactor`)))
  (`SceneComponent.SetRelativeScale3D` _sphere (`KismetMathLibrary.MakeVector` _returnvalue _returnvalue _returnvalue)))