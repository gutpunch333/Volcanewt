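; Enemy helicopter spawner that flies a random BP_HeliTankPath spline and drops up to two NC3 squads.
; A looping timer moves it along the spline through a gate, wrapping at the end.
; Another timer spawns squads with random Y offset and yaw under the game mode's enemy cap, then removes the helicopter after a delay.
; Any damage destroys it, but the game mode reference is cleared before the kill is reported.
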(event `DestroyHeli`
  (`self.K2_DestroyActor`))

(event `Attach to Heli Path`
  (bind _allhelitankpathsarray (`self.AllHeliTankPathsArray`))
  (bind _asbp_heli_tank_path (cast `/Game/Blueprints/BP_HeliTankPath` (`|GetArrayItem` _allhelitankpathsarray (`KismetMathLibrary.RandomInteger` (`KismetArrayLibrary.Array_Length` _allhelitankpathsarray)))))
  (set `self.As BP Heli Tank Path` _asbp_heli_tank_path))

(event `self.ReceiveBeginPlay`
  ;[1 1 1 1 100] Event BeginPlay
  (`|ExecutionSequence`
    (:`then_0`
      (bind _output_get (set `self.Looping` true))
      (`KismetSystemLibrary.K2_SetTimerDelegate` (delegate `SpawnTank`) 1.0 _output_get)
      (`GameplayStatics.PlaySoundAtLocation` "/Game/Audio/SoundEffects/SoundCues/HelicopterBlades.HelicopterBlades" (`self.K2_GetActorLocation`) (struct) 1.0 1.0 0.0 null "/Game/Audio/SoundConcurrency/HelicopterBlades_SCC.HelicopterBlades_SCC" null null)
      (bind _outactors (`GameplayStatics.GetAllActorsOfClass` "/Game/Blueprints/BP_HeliTankPath.BP_HeliTankPath_C"))
      (set `self.AllHeliTankPathsArray` _outactors)
      (`self.Attach to Heli Path`)
      (set `self.StartingHeliDistance` 0.0)
      (`self.UnlockMovement`))
    (:`then_1`
      (`KismetSystemLibrary.K2_SetTimerDelegate` (delegate `CustomUpdate`) (`self.UpdateRate`) true))))

(event `CustomUpdate`
  (bind _as_bp_heli_tank_path (`self.As BP Heli Tank Path`))
  (bind (_returnvalue_location _returnvalue_rotation) (`KismetMathLibrary.BreakTransform` (`SplineComponent.GetTransformAtDistanceAlongSpline` (`/Game/Blueprints/BP_HeliTankPath.Spline` _as_bp_heli_tank_path) (`self.HeliDistance`) "World" false)))
  (`/Engine/EditorBlueprintResources/StandardMacros.Gate` true :!label _label
    (:`Exit`
      (set `self.HeliDistance` (+ (* (`self.UpdateRate`) (`/Game/Blueprints/BP_HeliTankPath.PathSpeed` _as_bp_heli_tank_path)) (`self.HeliDistance`)))
      (`self.K2_SetActorTransform` (`KismetMathLibrary.MakeTransform` (+ _returnvalue_location (0.0 0.0 0.0)) _returnvalue_rotation))
      (if (> (`self.HeliDistance`) (`SplineComponent.GetSplineLength` (`/Game/Blueprints/BP_HeliTankPath.Spline` (`self.As BP Heli Tank Path`))))
        (set `self.HeliDistance` 0.0)))))

(event `self.ReceiveAnyDamage`
  (params (Damage :type "Float (single-precision)") (DamageType :type "DamageType Object Reference") (InstigatedBy :type "Controller Object Reference") (DamageCauser :type "Actor Object Reference"))
  ;[1 1 1 1 100] Destroys Enemy
  (`GameplayStatics.PlaySoundAtLocation` "/Game/Audio/SoundEffects/Player/stompBoom.stompBoom" (`self.K2_GetActorLocation`) (struct) 0.4 1.1 0.15 null null null null)
  (bind _output_get (set `self.As BPGM Volcanewt` null))
  (`/Game/Blueprints/Systems/BPGM_Volcanewt.EnemyDestroyed` _output_get (`self.EnemyMonetaryValue`))
  (`self.K2_DestroyActor`))

(event `UnlockMovement`
  (`SceneComponent.SetVisibility` (`self.Mesh`) true false)
  (goto _label :!via `Open`))

(event `SpawnTank`
  (bind _returnvalue (`self.GetTransform`))
  ;[1 1 1] Spawn Tanks
  (if (< (`/Game/Blueprints/Systems/BPGM_Volcanewt.EnemiesAlive` (`self.As BPGM Volcanewt`)) 50)
    (if (>= (`self.NumSquads`) 2)
      (set `self.Looping` false)
      (`KismetSystemLibrary.Delay` 10.0)
      (`self.K2_DestroyActor`)
      (else
        (`KismetSystemLibrary.Delay` 1.5)
        (`|SpawnActorFromClass` "/Game/Blueprints/Enemies/EnemySpawners/BP_NC3_SquadSpawn.BP_NC3_SquadSpawn_C" (`KismetMathLibrary.MakeTransform` (`KismetMathLibrary.MakeVector` (.x (.location _returnvalue)) (`KismetMathLibrary.RandomFloatInRange` (- (.y (.location _returnvalue)) 2500.0) (+ (.y (.location _returnvalue)) 2500.0)) (.z (.location _returnvalue))) (`KismetMathLibrary.MakeRotator` (.roll (.rotation _returnvalue)) (.pitch (.rotation _returnvalue)) (`KismetMathLibrary.RandomFloatInRange` (.yaw (.rotation _returnvalue)) 359.0)) (.scale _returnvalue)) "Undefined" "MultiplyWithRoot" null null)
        (`/Engine/EditorBlueprintResources/StandardMacros.IncrementInt` (`self.NumSquads`)
          (:`  `
            (`/Game/Blueprints/Systems/BPGM_Volcanewt.Increase Enemies` (`self.As BPGM Volcanewt`))))))))

(fn `UserConstructionScript`)