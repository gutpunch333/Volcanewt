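; BP_CivilianSpawner is a one-shot spawner that places civilians or buses in a ring around the player.
; On BeginPlay it asks BPGM_Volcanewt whether to spawn, destroying itself if not.
; It loops up to SpawnLimit, giving each spawn a 20% chance to be a bus and incrementing the game mode's enemy count.
; Random yaw and distance form the donut-shaped spawn area, and the spawner destroys itself afterward.
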(event `self.ReceiveBeginPlay`
  (`|ExecutionSequence`
    (:`then_0`
      (bind _asbpgm_volcanewt (cast `/Game/Blueprints/Systems/BPGM_Volcanewt` (`GameplayStatics.GetGameMode`)))
      (bind _output_get (set `self.As BPGM Volcanewt` _asbpgm_volcanewt))
      (`/Game/Blueprints/Systems/BPGM_Volcanewt.ShouldSpawn?` _output_get)
      (if (`/Game/Blueprints/Systems/BPGM_Volcanewt.ShouldSpawn` _output_get)
        (set `self.IsActive` true)
        (else
          (`self.K2_DestroyActor`))))
    (:`then_1`
      (if (`self.IsActive`)
        (`self.Spawn Civillians`)))))

(event `Spawn Civillians`
  (bind _returnvalue (`GameplayStatics.GetPlayerPawn` 0))
  (bind (_returnvalue_roll _returnvalue_pitch) (`KismetMathLibrary.BreakRotator` (`self.K2_GetActorRotation` _returnvalue)))
  (bind _returnvalue_2 (+ (`self.K2_GetActorLocation` _returnvalue) (* (`KismetMathLibrary.Conv_RotatorToVector` (`KismetMathLibrary.MakeRotator` _returnvalue_roll _returnvalue_pitch (`KismetMathLibrary.RandomFloatInRange` 0.0 360.0))) (`KismetMathLibrary.RandomFloatInRange` 4500.0 5000.0))))
  ;[1 1 1] Spawns civillians, 20% chance to spawn bus instead of civillians
  (for _index (range (+ (`self.SpawnLimit`) 1))
    (bind _output_get (set `self.SpawnBus?` (`KismetMathLibrary.RandomBoolWithWeight` 0.2)))
    (if _output_get
      (`/Game/Blueprints/Systems/BPGM_Volcanewt.Increase Enemies` (`self.As BPGM Volcanewt`))
      (`|SpawnActorFromClass` "/Game/Blueprints/Enemies/BP_Bus.BP_Bus_C" (`KismetMathLibrary.MakeTransform` _returnvalue_2) "Undefined" "MultiplyWithRoot" null null)
      (set `self.SpawnBus?` false)
      (if (== 0 (`self.SpawnLimit`))
        (break))
      (else
        (`/Game/Blueprints/Systems/BPGM_Volcanewt.Increase Enemies` (`self.As BPGM Volcanewt`))
        (`|SpawnActorFromClass` "/Game/Blueprints/Enemies/BP_Civilian.BP_Civilian_C" (`KismetMathLibrary.MakeTransform` _returnvalue_2) "Undefined" "MultiplyWithRoot" null null)
        (if (== _index (`self.SpawnLimit`))
          (break)))))
  (`self.K2_DestroyActor`))

(fn `UserConstructionScript`)