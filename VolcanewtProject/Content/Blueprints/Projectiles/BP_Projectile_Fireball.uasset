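; Fireball projectile Blueprint that activates its charge/trail effect on spawn and can deal area damage on impact.
; When soft homing is enabled, the first "EnemyUnit" actor entering the tracking radius becomes its target, enabling homing, playing a sound and calling RotateToTarget.
; A collision capsule hit applies explosion damage to every actor overlapping the explosion hitbox, except those tagged "Newt".
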(event `self.ReceiveBeginPlay`
  (`parent.ReceiveBeginPlay`)
  (`ActorComponent.SetActive` (`self.ChargeFX`) true true) ; FIRE TRAIL VFX
)

(event `self.Tracking Radius.OnComponentBeginOverlap`
  (params (OverlappedComponent :type "PrimitiveComponent Object Reference") (OtherActor :type "Actor Object Reference") (OtherComp :type "PrimitiveComponent Object Reference") (OtherBodyIndex :type Integer) (bFromSweep :type Boolean) (SweepResult :type "HitResult Structure (by ref)"))
  (if (and (`self.IsSoftHoming`) (not (`self.HasATargetChosen`)))
    (if (`self.ActorHasTag` OtherActor "EnemyUnit")
      (set `self.Target` OtherActor)
      (set `self.HasATargetChosen` true)
      (set `ProjectileMovementComponent.bIsHomingProjectile` true (`self.ProjectileMovement`))
      (`GameplayStatics.PlaySound2D` "/Game/Audio/gecko.gecko" 1.0 1.0 3.0 null null)
      (`self.RotateToTarget`))))

(event `self.Projectile'sSphereCollisionCapsule.OnComponentHit`
  (params (HitComponent :type "PrimitiveComponent Object Reference") (OtherActor :type "Actor Object Reference") (OtherComp :type "PrimitiveComponent Object Reference") (NormalImpulse :type "Vector Structure") (Hit :type "HitResult Structure (by ref)"))
  (for _array_element (`PrimitiveComponent.GetOverlappingActors` (`self.ExplosionHitbox`) null)
    (if (not (`self.ActorHasTag` _array_element "Newt"))
      (`GameplayStatics.ApplyDamage` _array_element (`self.ExplosionDamage`) null self))))

(fn `UserConstructionScript`
  (`parent.UserConstructionScript`))