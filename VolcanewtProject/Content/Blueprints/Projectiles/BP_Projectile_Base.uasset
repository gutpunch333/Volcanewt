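; Base projectile Blueprint that flies at a configurable speed and gravity, optionally aimed at or homing on a Target actor.
; The construction script configures ProjectileMovement, and BeginPlay ignores the owner for collision and points velocity at the Target.
; On hit it calls OnProjectileImpact with the actor and hit, spawns a Niagara or Cascade effect with sound, then destroys itself, optionally after a delay.
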(event `self.ReceiveBeginPlay`
  (`PrimitiveComponent.IgnoreActorWhenMoving` (`self.Projectile'sSphereCollisionCapsule`) (`self.GetOwner`) true)
  (`self.Target`
    (:`then`
      (`self.RotateToTarget`))
    (:`else`)))

(event `RotateToTarget`
  (set `MovementComponent.Velocity` (* (`KismetMathLibrary.GetDirectionUnitVector` (`self.K2_GetActorLocation`) (`self.K2_GetActorLocation` (`self.Target`))) (`self.Speed`)) (`self.ProjectileMovement`)))

(event `self.Projectile'sSphereCollisionCapsule.OnComponentHit`
  (params (HitComponent :type "PrimitiveComponent Object Reference") (OtherActor :type "Actor Object Reference") (OtherComp :type "PrimitiveComponent Object Reference") (NormalImpulse :type "Vector Structure") (Hit :type "HitResult Structure (by ref)"))
  (bind (_bblockinghit _binitialoverlap _time _distance _location) (`GameplayStatics.BreakHitResult` Hit))
  (`self.OnProjectileImpact` OtherActor Hit)
  (if (`self.UsesNiaga`)
    (`NiagaraFunctionLibrary.SpawnSystemAtLocation` (`self.Impact Niagara`) _location)
    (else
      (`GameplayStatics.SpawnEmitterAtLocation` (`self.Impact Particle Effect`) _location)))
  (`GameplayStatics.PlaySoundAtLocation` (`self.Impact Sound`) _location (struct) 1.0 0.8 0.0 null null null null)
  (if (`self.HasExplosionDelay`)
    (`KismetSystemLibrary.Delay` (`self.ExplosionDelay`)))
  (`self.K2_DestroyActor`))

(fn `UserConstructionScript`
  (bind _projectilemovement (`self.ProjectileMovement`))
  (bind _projectilemovement_2 (`self.ProjectileMovement`))
  (set `ProjectileMovementComponent.InitialSpeed` (`self.Speed`) _projectilemovement_2)
  (set `ProjectileMovementComponent.MaxSpeed` (`self.MaximumSpeed`) _projectilemovement_2)
  (set `ProjectileMovementComponent.ProjectileGravityScale` (`self.Gravity`) _projectilemovement_2)
  (`self.Target`
    (:`then`
      (if (`self.IsHoming`)
        (set `ProjectileMovementComponent.bIsHomingProjectile` true _projectilemovement)
        (set `ProjectileMovementComponent.HomingTargetComponent` (`Actor.RootComponent` (`self.Target`)) _projectilemovement)))
    (:`else`)))