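; Player controller for Volcanewt that owns the root UI_Base widget and acts as the entry point for menus and prompts.
; On BeginPlay it creates UI_Base, adds it to the viewport, hides the cursor and sets game-only input.
; Push events add pause, controls display, level complete and settings menus, plus parameterized prompts, to the UI_Base stack.
; Breaking news bar play and finish events are relayed through event dispatchers.
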(event `PushPauseMenu`
  ;[1 1 1] Pushing menus onto UI Base stack
  (`/Game/UI/Widgets/CommonUI/CommonWidgets/UI_Base.PushMenu` (`self.UI_BaseRef`) "/Game/UI/Widgets/CommonUI/CommonWidgets/UI_CommonPauseMenu.UI_CommonPauseMenu_C"))

(event `PushControlsDisplayMenu`
  ;[1 1 1] Pushing menus onto UI Base stack
  (`/Game/UI/Widgets/CommonUI/CommonWidgets/UI_Base.PushMenu` (`self.UI_BaseRef`) "/Game/UI/Widgets/CommonUI/CommonWidgets/UI_CommonControlsDisplayMenu.UI_CommonControlsDisplayMenu_C"))

(event `PushLevelCompleteMenu`
  ;[1 1 1] Pushing menus onto UI Base stack
  (`/Game/UI/Widgets/CommonUI/CommonWidgets/UI_Base.PushMenu` (`self.UI_BaseRef`) "/Game/UI/Widgets/CommonUI/CommonWidgets/UI_CommonLevelCompleteMenu.UI_CommonLevelCompleteMenu_C"))

(event `PushPrompt`
  (params (InPromptText :type Text) (InPromptEnum :type "/Game/UI/Widgets/CommonUI/Enum_PromptConfirm Enum" :default "NewEnumerator0"))
  ;[1 1 1] Pushing menus onto UI Base stack
  (`/Game/UI/Widgets/CommonUI/CommonWidgets/UI_Base.PushPrompt` (`self.UI_BaseRef`) InPromptText InPromptEnum))

(event `PushSettingsMenu`
  ;[1 1 1] Pushing menus onto UI Base stack
  (`/Game/UI/Widgets/CommonUI/CommonWidgets/UI_Base.PushMenu` (`self.UI_BaseRef`) "/Game/UI/Widgets/CommonUI/CommonWidgets/UI_CommonSettingsMenu.UI_CommonSettingsMenu_C"))

(event `self.ReceiveBeginPlay`
  ;[1 1 1] Establishing UI Menu Base
  (bind _returnvalue (`|CreateWidget` "/Game/UI/Widgets/CommonUI/CommonWidgets/UI_Base.UI_Base_C" self))
  (bind _output_get (set `self.UI_BaseRef` _returnvalue))
  (`UserWidget.AddToViewport` _output_get 0)
  (set `self.bShowMouseCursor` false)
  (`WidgetBlueprintLibrary.SetInputMode_GameOnly` self))

(event `/Game/Blueprints/Libraries_and_Interfaces/BPI_BreakingNewsBar.BreakingNewsBarPlay`
  (`self.BreakingNewsBarPlayDispatcher`))

(event `/Game/Blueprints/Libraries_and_Interfaces/BPI_BreakingNewsBar.BreakingNewsBarFinish`
  (`self.BreakingNewsBarFinishDispatcher`))

(fn `UserConstructionScript`)