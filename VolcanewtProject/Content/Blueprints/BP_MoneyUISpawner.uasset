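; BP_MoneyUISpawner is a short-lived actor that shows a floating money and building damage popup.
; On BeginPlay it passes its input money cost, damage, total health and current building health into the BPW_MoneycostUI widget on its MoneyWidget component.
; A timeline then lerps the actor from its start location to a raised diagonal offset and destroys it when finished.
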(event `self.ReceiveBeginPlay`
  ;[1 1 1] Setting variables in widget UI
  (bind _asbpw_moneycost_ui (cast `/Game/UI/Widgets/BPW_MoneycostUI` (`WidgetComponent.GetWidget` (`self.MoneyWidget`))))
  (set `/Game/UI/Widgets/BPW_MoneycostUI.MoneyCost` (`self.InputMoneyCost`) _asbpw_moneycost_ui)
  (set `/Game/UI/Widgets/BPW_MoneycostUI.DamageDone` (`self.InputDamage`) _asbpw_moneycost_ui)
  (set `/Game/UI/Widgets/BPW_MoneycostUI.TotalBuildingHealth` (`self.InputTotalHealth`) _asbpw_moneycost_ui)
  (set `/Game/UI/Widgets/BPW_MoneycostUI.BuildingCurrentHealth` (`self.InputCurrentBuildingHealth`) _asbpw_moneycost_ui)
  ;[1 1 1] Setting location for the UI to travel between
  (bind _output_get (set `self.StartLocation` (`self.K2_GetActorLocation`)))
  (set `self.EndLocation` (+ _output_get (-50.0 -50.0 100.0)))
  ;[1 1 1] Moving the actor across its path before destroying it
  (bind (_direction _move_track) (`Timeline|MoveT` :!via `PlayFromStart`)
    (:`Update`
      (`self.K2_SetActorLocation` (`KismetMathLibrary.VLerp` (`self.StartLocation`) (`self.EndLocation`) _move_track)))
    (:`Finished`
      (`self.K2_DestroyActor`))))

(fn `UserConstructionScript`)