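; BP_LargeBuilding is a destructible large building in Volcanewt that carries a monetary value, passed to its BP_BuildingParent child actor.
; Damage lowers its health with camera shake and Niagara effects.
; At zero health it reports to the game mode, crumbles its Chaos geometry collection, plays a sound and spawns a money UI.
; A timeline then fades dynamic materials created in the construction script before destroying the actor.
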(event `self.ReceiveBeginPlay`
  (set `self.bCanBeDamaged` true)
  (bind _asbpgm_volcanewt (cast `/Game/Blueprints/Systems/BPGM_Volcanewt` (`GameplayStatics.GetGameMode`)))
  (set `self.As BPGM Volcanewt` _asbpgm_volcanewt)
  (bind _asbp_building_parent (cast `/Game/Blueprints/Enviornment/BP_BuildingParent` (`ChildActorComponent.ChildActor` (`self.BP_BuildingParent`))))
  (set `/Game/Blueprints/Enviornment/BP_BuildingParent.MonetaryValue` (`self.LargeBuildingMV`) _asbp_building_parent))

(event `self.ReceiveAnyDamage`
  (params (Damage :type "Float (single-precision)") (DamageType :type "DamageType Object Reference") (InstigatedBy :type "Controller Object Reference") (DamageCauser :type "Actor Object Reference"))
  (bind _returnvalue_location (`KismetMathLibrary.BreakTransform` (`self.GetTransform`)))
  (bind _type_b_1_5floors5_geometrycollection (`self.Type_B_1_5Floors5_GeometryCollection`))
  (bind _returnvalue (<= (`self.LargeBuildingHealth`) 0))
  (if (not _returnvalue)
    (`GameplayStatics.PlayWorldCameraShake` "/Game/Player/jumpShakeMatinee.jumpShakeMatinee_C" (`self.K2_GetActorLocation`) 0.0 33333.0)
    (set `self.LargeBuildingHealth` (- (`self.LargeBuildingHealth`) Damage))
    (`/Game/Blueprints/Libraries_and_Interfaces/MuhFunctionLibrary.SpawnNiagaraAtActor` self "/Game/Textures/NPS_BuildingDamage.NPS_BuildingDamage")
    (if _returnvalue
      (bind _asbpgm_volcanewt (cast `/Game/Blueprints/Systems/BPGM_Volcanewt` (`GameplayStatics.GetGameMode`)))
      (`/Game/Blueprints/Systems/BPGM_Volcanewt.BuildingDestroyed` _asbpgm_volcanewt (`self.LargeBuildingMV`) self)
      ;[1 1 1] Crumbling building with chaos system
      (`PrimitiveComponent.SetSimulatePhysics` _type_b_1_5floors5_geometrycollection true)
      (`GeometryCollectionComponent.CrumbleCluster` _type_b_1_5floors5_geometrycollection 0)
      (`GeometryCollectionComponent.CrumbleCluster` _type_b_1_5floors5_geometrycollection 1)
      (`GeometryCollectionComponent.CrumbleCluster` _type_b_1_5floors5_geometrycollection 2)
      (`GameplayStatics.PlaySoundAtLocation` "/Game/Audio/SoundCues/BuildingDestruction_SC.BuildingDestruction_SC" (`self.K2_GetActorLocation`) (struct) 1.0 1.0 0.0 null null null null)
      ;[1 1 1] Spawn Money UI
      (`|SpawnActorFromClass` "/Game/Blueprints/Systems/BP_MoneyUISpawner.BP_MoneyUISpawner_C" (`KismetMathLibrary.MakeTransform` (+ _returnvalue_location (0.0 0.0 10.0))) "AlwaysSpawn" "MultiplyWithRoot" null (`self.LargeBuildingMV`) 0 0 0 null)
      (`KismetSystemLibrary.Delay` 1.0)
      ;[1 1 1] Lerping the dynamic materials' parameter values to fade the building out
      (bind (_direction _fadealpha) (`Timeline|FadeOutBuilding` :!via `PlayFromStart`)
        (:`Update`
          (bind _returnvalue_2 (`KismetMathLibrary.Lerp` 1.0 0.0 _fadealpha))
          (`MaterialInstanceDynamic.SetScalarParameterValue` (`self.DynamicMaterialInstanceIndex0`) "fadeOut" _returnvalue_2)
          (`MaterialInstanceDynamic.SetScalarParameterValue` (`self.DynamicMaterialInstanceIndex1`) "fadeOut" _returnvalue_2))
        (:`Finished`
          (`KismetSystemLibrary.Delay` 0.5)
          (`self.K2_DestroyActor`))))))

(fn `UserConstructionScript`
  (bind _type_b_1_5floors5_geometrycollection (`self.Type_B_1_5Floors5_GeometryCollection`))
  ;[1 1 1] Creating and setting references to Dynamic Material instances
  (bind _returnvalue (`PrimitiveComponent.CreateDynamicMaterialInstance` _type_b_1_5floors5_geometrycollection 1 "/Game/Models/Enviornment/Buildings/Textures/TypeB_Building1.TypeB_Building1" "None"))
  (set `self.DynamicMaterialInstanceIndex1` _returnvalue)
  (bind _returnvalue_2 (`PrimitiveComponent.CreateDynamicMaterialInstance` _type_b_1_5floors5_geometrycollection 0 "/Game/Models/Enviornment/Buildings/Textures/TypeB_Building1.TypeB_Building1" "None"))
  (set `self.DynamicMaterialInstanceIndex0` _returnvalue_2))