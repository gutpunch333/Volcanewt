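; Game mode for a Volcanewt city-destruction level, tracking building counts, monetary damage, level time and the NewtCon timer.
; BeginPlay totals small and large building values, creating the HUD and adding input mapping inside the small-building loop.
; BuildingDestroyed feeds damage to the HUD meter, triggering the meter-filled screen when its percent nears zero.
; A delayed Tick advances both timers, and LevelComplete pauses the game to show results.
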(event `Level Complete`
  (bind _returnvalue (`GameplayStatics.GetPlayerController` 0))
  (bind _bpw_levelcomplete (`self.BPW_LevelComplete`))
  ;[1 0.8775 0.114] Level Complete
  (bind _returnvalue_2 (`|CreateWidget` "/Game/UI/Widgets/BPW_LevelComplete.BPW_LevelComplete_C"))
  (bind _output_get (set `self.BPW_LevelComplete` _returnvalue_2))
  (`UserWidget.AddToViewport` _returnvalue_2 0)
  (`UserWidget.AddToViewport` _output_get 0)
  (`WidgetBlueprintLibrary.SetInputMode_UIOnlyEx` _returnvalue null)
  (set `PlayerController.bShowMouseCursor` true _returnvalue)
  (`GameplayStatics.SetGamePaused` true)
  (set `/Game/UI/Widgets/BPW_LevelComplete.TotalBuildingsDestroyed` (`self.TotalBuildingsDestroyed`) _bpw_levelcomplete)
  (set `/Game/UI/Widgets/BPW_LevelComplete.TotalMonetaryValueDestroyed` (`self.LevelMonetaryValueDestroyed`) _bpw_levelcomplete)
  (set `/Game/UI/Widgets/BPW_LevelComplete.WWDFForcesDefeated` 0 _bpw_levelcomplete)
  (set `/Game/UI/Widgets/BPW_LevelComplete.WWDFBudgetDestroyed` 0.0 _bpw_levelcomplete)
  (set `/Game/UI/Widgets/BPW_LevelComplete.Buildings Missed` (- (`self.TotalBuildings`) (`self.TotalBuildingsDestroyed`)) _bpw_levelcomplete)
  (set `/Game/UI/Widgets/BPW_LevelComplete.MinutesCompleted` (`self.World Minutes`) _bpw_levelcomplete)
  (set `/Game/UI/Widgets/BPW_LevelComplete.SecondsCompleted` (`self.World Seconds`) _bpw_levelcomplete))

(event `SmallBuildingDestroyed`
  ;[1 0.354 0.354] Counts Specific Destroyed Buildings
  (set `self.SmallBuildingsDestroyed` (+ (`self.LargeBuildingsDestroyed`) 1)))

(event `InputAction|EatTest`
  (params (Key :type "Key Structure"))
  ;[1 1 1] Test Function for Eating Civillians and Adding Time to NewtCon
  (:`Pressed`
    (set `/Game/UI/Widgets/BPW_HUD.NewtConTimer` (+ (`/Game/UI/Widgets/BPW_HUD.NewtConTimer` (`self.HUDWidget Ref`)) 15) (`self.HUDWidget Ref`))))

(event `DestructionMeterFilled`
  (bind _returnvalue (`GameplayStatics.GetPlayerController` 0))
  ;[1 0.4826 0.122] Destruction Meter Filled
  (bind _returnvalue_2 (`|CreateWidget` "/Game/UI/Widgets/BPW_DestructionMeterFilled.BPW_DestructionMeterFilled_C" (`GameplayStatics.GetPlayerController` 0)))
  (`UserWidget.AddToViewport` _returnvalue_2 0)
  (`WidgetBlueprintLibrary.SetInputMode_UIOnlyEx` _returnvalue null)
  (set `PlayerController.bShowMouseCursor` true _returnvalue)
  (set `self.CityDestroyed` true))

(event `LargeBuildingDestroyed`
  ;[1 0.354 0.354] Counts Specific Destroyed Buildings
  (set `self.LargeBuildingsDestroyed` (+ (`self.LargeBuildingsDestroyed`) 1)))

(event `self.ReceiveTick`
  (params (DeltaSeconds :type "Float (single-precision)"))
  (bind _hudwidget_ref (`self.HUDWidget Ref`))
  (bind _hudwidget_ref_2 (`self.HUDWidget Ref`))
  (bind _returnvalue (+ (`self.World Seconds`) 1))
  ;[1 1 1] Establishes World and NewtCon Timers
  (`KismetSystemLibrary.Delay` 1.0)
  (bind _output_get (set `self.World Seconds` _returnvalue))
  (set `/Game/UI/Widgets/BPW_HUD.WorldSecondsHUD` _output_get _hudwidget_ref)
  (set `/Game/UI/Widgets/BPW_HUD.NewtConTimer` (+ (`/Game/UI/Widgets/BPW_HUD.NewtConTimer` _hudwidget_ref) 1) _hudwidget_ref)
  (if (> _returnvalue 59)
    (bind _output_get_2 (set `self.World Minutes` (+ (`self.World Minutes`) 1)))
    (set `/Game/UI/Widgets/BPW_HUD.WorldMinutesHUD` _output_get_2 _hudwidget_ref_2)
    (bind _output_get_3 (set `self.World Seconds` 0))
    (set `/Game/UI/Widgets/BPW_HUD.WorldSecondsHUD` _output_get_3 _hudwidget_ref_2)))

(event `BuildingDestroyed`
  (params (Money :type "Float (double-precision)"))
  (bind _hudwidget_ref (`self.HUDWidget Ref`))
  ;[1 1 1] Tracks when buildings are destroyed and updates the destruction meter
  (bind _output_get (set `/Game/UI/Widgets/BPW_HUD.LevelDestroyedMonetaryValue` (+ (`/Game/UI/Widgets/BPW_HUD.LevelDestroyedMonetaryValue` _hudwidget_ref) Money) _hudwidget_ref))
  (set `self.LevelMonetaryValueDestroyed` _output_get)
  (set `self.TotalBuildingsDestroyed` (+ (`self.TotalBuildingsDestroyed`) 1))
  (if (<= (`/Game/UI/Widgets/BPW_HUD.Get_DestructionMeter_Percent` _hudwidget_ref) 0.001)
    (if (not (`self.CityDestroyed`))
      (`self.DestructionMeterFilled`))))

(event `self.ReceiveBeginPlay`
  ;[1 1 1] Finding all small buildings and recording their count and their total monitary value
  (bind _outactors (`GameplayStatics.GetAllActorsOfClass` "/Game/Blueprints/BP_SmallBuilding.BP_SmallBuilding_C"))
  (for _array_element _outactors
    (set `self.LevelMonetaryValue` (+ (`self.LevelMonetaryValue`) (`/Game/Blueprints/BP_SmallBuilding.SmallBuildingMV` _array_element)))
    (set `self.SmallBuildingTotal` (+ (`self.SmallBuildingTotal`) 1))
    (set `self.TotalBuildings` (+ (`self.TotalBuildings`) 1))
    (bind _returnvalue (`|CreateWidget` "/Game/UI/Widgets/BPW_HUD.BPW_HUD_C"))
    (bind _output_get (set `self.HUDWidget Ref` _returnvalue))
    (`UserWidget.AddToViewport` _output_get 0)
    ;[1 1 1] Adds Input System to Gamemode
    (`EnhancedInputSubsystemInterface.AddMappingContext` (pcsubsystem `EnhancedInputLocalPlayerSubsystem` (`GameplayStatics.GetPlayerController` 0)) "/Game/Player/IMC_ThirdPerson.IMC_ThirdPerson" 0 (struct)))
  ;[1 1 1] Debug print strings
  (`KismetSystemLibrary.PrintString` (`KismetStringLibrary.Conv_DoubleToString` (`self.LevelMonetaryValue`)) true true (struct :`G` 0.66 :`B` 1.0 :`A` 1.0) 5.0)
  ;[1 1 1] Finding all large buildings and recording their count and total monitary value
  (bind _outactors_2 (`GameplayStatics.GetAllActorsOfClass` "/Game/Blueprints/BP_LargeBuilding.BP_LargeBuilding_C"))
  (for _array_element_2 _outactors_2
    (bind _output_get_2 (set `self.LevelMonetaryValue` (+ (`self.LevelMonetaryValue`) (`/Game/Blueprints/BP_LargeBuilding.LargeBuildingMV` _array_element_2))))
    (set `self.LargeBuildingTotal` (+ (`self.LargeBuildingTotal`) 1))
    (set `self.TotalBuildings` (+ (`self.TotalBuildings`) 1))
    (set `/Game/UI/Widgets/BPW_HUD.LevelTotalMonetaryValue` _output_get_2 (`self.HUDWidget Ref`)))
  (`KismetSystemLibrary.PrintString` (`KismetStringLibrary.Conv_DoubleToString` (`self.LevelMonetaryValue`)) true true (struct :`G` 0.66 :`B` 1.0 :`A` 1.0) 5.0)
  (`KismetSystemLibrary.PrintString` (`KismetStringLibrary.Conv_IntToString` (`self.SmallBuildingTotal`)) true true (struct :`R` 0.808 :`A` 1.0) 20.0)
  (`KismetSystemLibrary.PrintString` (`KismetStringLibrary.Conv_IntToString` (`self.LargeBuildingTotal`)) true true (struct :`R` 0.966777 :`G` 0.048 :`B` 1.0 :`A` 1.0) 20.0))

(fn `UserConstructionScript`)