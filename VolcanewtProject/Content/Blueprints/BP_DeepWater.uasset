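; BP_DeepWater is a hazard volume that drains the player's health while BP_Volcanewt is in deep water.
; Box begin overlap starts a looping one-second timer that applies damage to player character 0 rather than the overlapping actor.
; End overlap clears that timer for BP_Volcanewt, though the IsDrowning flag changes for any overlapping actor because it is set before the cast.
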(event `self.ReceiveBeginPlay`)

(event `ClearTimer`
  ;[1 1 1] Decrease player health when in deep water
  (`KismetSystemLibrary.K2_ClearAndInvalidateTimerHandle` (stale `self.Box.OnComponentBeginOverlap` _returnvalue)))

(event `self.Box.OnComponentBeginOverlap`
  (params (OverlappedComponent :type "PrimitiveComponent Object Reference") (OtherActor :type "Actor Object Reference") (OtherComp :type "PrimitiveComponent Object Reference") (OtherBodyIndex :type Integer) (bFromSweep :type Boolean) (SweepResult :type "HitResult Structure (by ref)"))
  (bind _isdrowning (`self.IsDrowning`))
  ;[1 1 1] Decrease player health when in deep water
  (set `self.IsDrowning` true)
  (cast `/Game/Player/Blueprints/BP_Volcanewt` OtherActor)
  (if _isdrowning
    (bind _returnvalue (`KismetSystemLibrary.K2_SetTimerDelegate` (delegate `DecrementHealth`) 1.0 _isdrowning))))

(event `DecrementHealth`
  ;[1 1 1] Decrease player health when in deep water
  (`GameplayStatics.ApplyDamage` (`GameplayStatics.GetPlayerCharacter` 0) 50.0))

(event `self.Box.OnComponentEndOverlap`
  (params (OverlappedComponent :type "PrimitiveComponent Object Reference") (OtherActor :type "Actor Object Reference") (OtherComp :type "PrimitiveComponent Object Reference") (OtherBodyIndex :type Integer))
  ;[1 1 1] Stops damage from deep water
  (set `self.IsDrowning` false)
  (cast `/Game/Player/Blueprints/BP_Volcanewt` OtherActor)
  (`self.ClearTimer`))

(fn `UserConstructionScript`)