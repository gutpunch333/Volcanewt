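; BP_BonusObjManager hands level-configured bonus objective settings to the Volcanewt game mode.
; On BeginPlay it casts the game mode to BPGM_Volcanewt and copies in the active civilian and military objective arrays.
; Empty loops over both arrays supply their final index as each category's active value, rather than the element count.
; It also passes along timers for bakery evacuation, thermal energy and walker guys.
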(event `self.ReceiveBeginPlay`
  (bind _as_bpgm_volcanewt (`self.As BPGM Volcanewt`))
  (bind _as_bpgm_volcanewt_2 (`self.As BPGM Volcanewt`))
  (bind _asbpgm_volcanewt (cast `/Game/Blueprints/BPGM_Volcanewt` (`GameplayStatics.GetGameMode`)))
  (set `self.As BPGM Volcanewt` _asbpgm_volcanewt)
  (set `/Game/Blueprints/BPGM_Volcanewt.CivillianBonusObjectives` (`self.ActiveCivillianBonusObjectives`) _as_bpgm_volcanewt)
  (set `/Game/Blueprints/BPGM_Volcanewt.MilitaryBonusObjectives` (`self.ActiveMilitaryBonusObjectives`) _as_bpgm_volcanewt)
  (for (_ _array_index) (`self.ActiveCivillianBonusObjectives`)
    _)
  (set `/Game/Blueprints/BPGM_Volcanewt.CivillianBonusActive#` _array_index _as_bpgm_volcanewt_2)
  (for (_ _array_index_2) (`self.ActiveMilitaryBonusObjectives`)
    _)
  (set `/Game/Blueprints/BPGM_Volcanewt.MilitaryBonusActive#` _array_index_2 _as_bpgm_volcanewt_2)
  (set `/Game/Blueprints/BPGM_Volcanewt.BakeryEvacTimer` (`self.BakeryEvacTimer`) _as_bpgm_volcanewt_2)
  (set `/Game/Blueprints/BPGM_Volcanewt.ThermalEnergyTimer` (`self.ThermalEnergyTimer`) _as_bpgm_volcanewt_2)
  (set `/Game/Blueprints/BPGM_Volcanewt.WalkerGuysTimer` (`self.WalkerGuysTimer`) _as_bpgm_volcanewt_2))

(fn `UserConstructionScript`)