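; Destructible apartment building for the Volcanewt game mode that collapses when damaged.
; BeginPlay copies its monetary value to a child BP_BuildingParent actor.
; Damage taken while health is above 150 reduces health, reports destruction to the game mode, plays particles and sound, and crumbles the Geometry Collection with physics.
; Two dynamic material instances from the construction script then fade out on a timeline before the actor is destroyed.
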(event `self.ReceiveBeginPlay`
  (set `self.bCanBeDamaged` true)
  (bind _asbpgm_volcanewt (cast `/Game/Blueprints/BPGM_Volcanewt` (`GameplayStatics.GetGameMode`)))
  (set `self.As BPGM Volcanewt` _asbpgm_volcanewt)
  ;[1 1 1] A variable consistent across all building actors is established
  (bind _asbp_building_parent (cast `/Game/Blueprints/BP_BuildingParent` (`ChildActorComponent.ChildActor` (`self.BP_BuildingParent`))))
  (set `/Game/Blueprints/BP_BuildingParent.MonetaryValue` (`self.ApartmentBuildingMV`) _asbp_building_parent))

(event `self.ReceiveAnyDamage`
  (params (Damage :type "Float (single-precision)") (DamageType :type "DamageType Object Reference") (InstigatedBy :type "Controller Object Reference") (DamageCauser :type "Actor Object Reference"))
  (bind _smallbuildinghealth (`self.SmallBuildingHealth`))
  (bind _gc_apartmentbuilding4 (`self.GC_ApartmentBuilding4`))
  ;[1 1 1] Checks if the building has any health, if above 0 itlll do damage stuff
  (if (not (<= _smallbuildinghealth 150))
    (set `self.SmallBuildingHealth` (- _smallbuildinghealth (`KismetMathLibrary.FTrunc` Damage)))
    (`/Game/Blueprints/Libraries_and_Interfaces/MuhFunctionLibrary.SpawnNiagaraAtActor` self "/Game/Textures/NPS_BuildingDamage.NPS_BuildingDamage")
    (bind _asbpgm_volcanewt (cast `/Game/Blueprints/BPGM_Volcanewt` (`GameplayStatics.GetGameMode`)))
    (`/Game/Blueprints/BPGM_Volcanewt.BuildingDestroyed` _asbpgm_volcanewt (`self.ApartmentBuildingMV`) self)
    ;[1 1 1] Sets physics to mesh and breaks apart the separate geometry mesh
    (`PrimitiveComponent.SetSimulatePhysics` _gc_apartmentbuilding4 true)
    (`GeometryCollectionComponent.CrumbleCluster` _gc_apartmentbuilding4 0)
    (`GeometryCollectionComponent.CrumbleCluster` _gc_apartmentbuilding4 1)
    ;[1 1 1 1 1000] Sound :)
    (`GameplayStatics.PlaySoundAtLocation` "/Game/Audio/SoundEffects/rocks.rocks" (`self.K2_GetActorLocation`) (struct) 0.75 1.4 2.7 null null null null)
    ;;[1 1 1] Lerping the dynamic materials' parameter values to fade the building out
    (`KismetSystemLibrary.Delay` 1.0)
    (bind (_direction _fadealpha) (`Timeline|Timeline` :!via `PlayFromStart`)
      (:`Update`
        (bind _returnvalue (`KismetMathLibrary.Lerp` 1.0 0.0 _fadealpha))
        (`MaterialInstanceDynamic.SetScalarParameterValue` (`self.DynamicMaterialInstanceIndex1`) "fadeOut" _returnvalue)
        (`MaterialInstanceDynamic.SetScalarParameterValue` (`self.DynamicMaterialInstanceIndex0`) "fadeOut" _returnvalue))
      (:`Finished`
        (`KismetSystemLibrary.Delay` 7.0)
        (`self.K2_DestroyActor`)))))

(fn `UserConstructionScript`
  (bind _gc_apartmentbuilding4 (`self.GC_ApartmentBuilding4`))
  ;[1 1 1] Creating and setting references to Dynamic Material instances
  (bind _returnvalue (`PrimitiveComponent.CreateDynamicMaterialInstance` _gc_apartmentbuilding4 1 "/Game/Buildings/lambert1.lambert1" "None"))
  (set `self.DynamicMaterialInstanceIndex1` _returnvalue)
  (bind _returnvalue_2 (`PrimitiveComponent.CreateDynamicMaterialInstance` _gc_apartmentbuilding4 0 "/Game/Buildings/lambert1.lambert1" "None"))
  (set `self.DynamicMaterialInstanceIndex0` _returnvalue_2))