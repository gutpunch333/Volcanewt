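; A level-placed configuration actor that feeds per-level NewtCon settings to the BPGM_Volcanewt game mode.
; On BeginPlay it casts the game mode and copies in its arrays of infantry, ground and air vehicle types, wave limit boundaries and NewtCon dialogue.
; These values define which enemies spawn, how many per wave and which messages show at each NewtCon level.
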(event `self.ReceiveBeginPlay`
  (bind _as_bpgm_volcanewt (`self.As BPGM Volcanewt`))
  (bind _asbpgm_volcanewt (cast `/Game/Blueprints/BPGM_Volcanewt` (`GameplayStatics.GetGameMode`)))
  (set `self.As BPGM Volcanewt` _asbpgm_volcanewt)
  ;[1 1 1] Establishes what kinds of infantry spawn in the level at each NewtCon Level
  (set `/Game/Blueprints/BPGM_Volcanewt.ListOfInfantryTypes` (`self.LevelInfantryTypes`) _as_bpgm_volcanewt)
  ;[1 1 1] Establishes how many enemies can spawn in a wave for each NewtCon Level
  (set `/Game/Blueprints/BPGM_Volcanewt.LimitBoundaries` (`self.LevelLimitBoundaries`) _as_bpgm_volcanewt)
  ;[1 1 1] Establishes Level Specific NewtCon Messages
  (set `/Game/Blueprints/BPGM_Volcanewt.NewtConDialogueArray` (`self.LevelNewtConDialogue`) _as_bpgm_volcanewt)
  (set `/Game/Blueprints/BPGM_Volcanewt.ListOfGroundVehicles` (`self.LevelGroundVehicleTypes`) _as_bpgm_volcanewt)
  (set `/Game/Blueprints/BPGM_Volcanewt.ListOfAirVehicles` (`self.LevelAirVehicleTypes`) _as_bpgm_volcanewt))

(fn `UserConstructionScript`)