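; BP_MilitaryBase is a destructible military base building that reports its monetary value to the Volcanewt game mode when destroyed.
; BeginPlay caches the game mode and objective marker widget, and copies the value into its BP_BuildingParent child actor.
; Damage drains health, still stored in SmallStore-named variables, until the actor notifies the game mode and destroys itself.
; Tick updates the marker with the player's distance in metres.
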(event `self.ReceiveBeginPlay`
  ;[1 1 1] Adds to background information in game mode
  (bind _asbpgm_volcanewt (cast `/Game/Blueprints/Systems/BPGM_Volcanewt` (`GameplayStatics.GetGameMode`)))
  (set `self.As BPGM Volcanewt` _asbpgm_volcanewt)
  (bind _asbp_building_parent (cast `/Game/Blueprints/Enviornment/BP_BuildingParent` (`ChildActorComponent.ChildActor` (`self.BP_BuildingParent`))))
  (set `/Game/Blueprints/Enviornment/BP_BuildingParent.MonetaryValue` (`self.SmallStoreMV`) _asbp_building_parent)
  (bind _asbpw_objective_marker (cast `/Game/UI/Widgets/BPW_ObjectiveMarker` (`WidgetComponent.GetUserWidgetObject` (`self.Widget`))))
  (set `self.As BPW Objective Marker` _asbpw_objective_marker))

(event `self.ReceiveTick`
  (params (DeltaSeconds :type "Float (single-precision)"))
  ;[1 1 1] Activated by Bonus Objective in Gamemode. Calculates the distance between player and bonused building and updates the UI respectively in Meters
  (`/Game/UI/Widgets/BPW_ObjectiveMarker.Set DistanceText` (`self.As BPW Objective Marker`) (`KismetTextLibrary.Conv_DoubleToText` (/ (`KismetMathLibrary.Vector_Distance` (`self.K2_GetActorLocation`) (`self.K2_GetActorLocation` (`GameplayStatics.GetPlayerPawn` 0))) 100.0) "HalfToEven" false true 1 324 0 0)))

(event `self.ReceiveAnyDamage`
  (params (Damage :type "Float (single-precision)") (DamageType :type "DamageType Object Reference") (InstigatedBy :type "Controller Object Reference") (DamageCauser :type "Actor Object Reference"))
  (bind _smallstorehealth (`self.SmallStoreHealth`))
  (set `self.SmallStoreHealth` (- _smallstorehealth Damage))
  (if (<= _smallstorehealth 0.0)
    (`/Game/Blueprints/Systems/BPGM_Volcanewt.BuildingDestroyed` (`self.As BPGM Volcanewt`) (`self.SmallStoreMV`) self)
    (`self.K2_DestroyActor`)))

(fn `UserConstructionScript`)