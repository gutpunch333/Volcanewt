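; BP_LittleStatue is a damageable statue building that reports its destruction to the monument cluster.
; It relies on its parent for begin play and damage handling, then, if CurrentHealth is zero or below, calls LittleMonumentDestroyed on the BP_MonumentCluster found in the level and prints a debug message.
; Construction runs the parent script and enables FadeOut; the dynamic material setup is left unconnected.
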(event `self.ReceiveBeginPlay`
  (`parent.ReceiveBeginPlay`))

(event `self.ReceiveAnyDamage`
  (params (Damage :type "Float (single-precision)") (DamageType :type "DamageType Object Reference") (InstigatedBy :type "Controller Object Reference") (DamageCauser :type "Actor Object Reference"))
  (`parent.ReceiveAnyDamage` Damage null null null)
  (if (<= (`self.Current Health`) 0.0)
    (bind _returnvalue (`GameplayStatics.GetActorOfClass` "/Game/Blueprints/Systems/BP_MonumentCluster.BP_MonumentCluster_C"))
    (`/Game/Blueprints/Systems/BP_MonumentCluster.LittleMonumentDestroyed` _returnvalue self)
    (`KismetSystemLibrary.PrintString` "Hello")))

(fn `UserConstructionScript`
  (`parent.UserConstructionScript`)
  (set `self.Fade Out` true))