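; BP_Powerplant is a power plant building group made of silo and power building child actors, reporting its destruction to BPGM_Volcanewt.
; On BeginPlay it binds damage events on those buildings, caches its child actors and has the game mode count power plants.
; Damage or destruction callbacks recount invalid children, calling PowerPlantDestroyed on the game mode when the count equals TotalBuildings.
; TotalBuildings is taken from the loop's array index rather than the array length.
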(event `self.ReceiveBeginPlay`
  (add `self.OnTakeAnyDamage` (`ChildActorComponent.ChildActor` (`self.BP_PowerSilo1`)) (`|CreateDelegate` :!event `BP_Powerplant_AutoGenFunc2`))
  (add `self.OnTakeAnyDamage` (`ChildActorComponent.ChildActor` (`self.BP_PowerSilo`)) (`|CreateDelegate` :!event `BP_Powerplant_AutoGenFunc2`))
  (add `self.OnTakeAnyDamage` (`ChildActorComponent.ChildActor` (`self.BP_PowerBuilding`)) (`|CreateDelegate` :!event `BP_Powerplant_AutoGenFunc2`))
  (bind _asbpgm_volcanewt (cast `/Game/Blueprints/Systems/BPGM_Volcanewt` (`GameplayStatics.GetGameMode`)))
  (set `self.As BPGM Volcanewt` _asbpgm_volcanewt)
  (for (_array_element _array_index) (`self.GetAllChildActors` true)
    (`KismetArrayLibrary.Array_Add` (`self.Child Actors`) _array_element))
  (set `self.Total Buildings` _array_index)
  (`/Game/Blueprints/Systems/BPGM_Volcanewt.CountPowerPlants` (`self.As BPGM Volcanewt`)))

(event `CustomEvent`
  (for _array_element (`self.Child Actors`)
    (`/Engine/EditorBlueprintResources/StandardMacros.IsValid` _array_element
      (:`Is Not Valid`
        (set `self.Power Plant Buildings Destroyed` (+ (`self.Power Plant Buildings Destroyed`) 1))
        (`KismetSystemLibrary.PrintString` (`KismetStringLibrary.Conv_IntToString` 0)))))
  (if (== (`self.Power Plant Buildings Destroyed`) (`self.Total Buildings`))
    (`/Game/Blueprints/Systems/BPGM_Volcanewt.Power Plant Destroyed` (`self.As BPGM Volcanewt`))
    (else
      (set `self.Power Plant Buildings Destroyed` 0))))

(fn `BP_Powerplant_AutoGenFunc`
  (params (DestroyedActor :type "Actor Object Reference"))
  (`self.CustomEvent`))

(fn `BP_Powerplant_AutoGenFunc1`
  (params (DamagedActor :type "Actor Object Reference") (Damage :type "Float (single-precision)") (DamageType :type "DamageType Object Reference") (InstigatedBy :type "Controller Object Reference") (DamageCauser :type "Actor Object Reference"))
  (`self.CustomEvent`))

(fn `BP_Powerplant_AutoGenFunc2`
  (params (DamagedActor :type "Actor Object Reference") (Damage :type "Float (single-precision)") (DamageType :type "DamageType Object Reference") (InstigatedBy :type "Controller Object Reference") (DamageCauser :type "Actor Object Reference"))
  (`self.CustomEvent`))

(fn `UserConstructionScript`)