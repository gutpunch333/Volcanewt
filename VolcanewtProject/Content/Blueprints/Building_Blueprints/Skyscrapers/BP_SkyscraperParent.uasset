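; Parent skyscraper building Blueprint: a destructible building with a core and an array of weak points, worth money when destroyed.
; Core hits subtract health, shake the building and show money UI on larger hits, then report destruction to the game mode.
; At zero health, Geometry Collection clusters crumble with physics and sound, then weak points shrink and a timeline plays before the actor is destroyed.
; Weak point hits briefly toggle vulnerability off.
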(event `self.ShakeBuilding`
  ;[1 1 1] Shakes the whole building if the core is hit
  (`parent.ShakeBuilding`))

(event `Weak Point Hit`
  (params (`Weak Point Ref` :type "Actor Object Reference") (Damage :type "Float (double-precision)"))
  ;[1 1 1] Marks the weakpoint as no longer able to take damage
  (if (`self.Vulnerable`)
    (set `self.Vulnerable` false)
    ;[1 1 1] Makes the skyscraper vulnerable after a short delay
    (`KismetSystemLibrary.Delay` 0.3)
    (set `self.Vulnerable` true)))

(event `self.ReceiveBeginPlay`
  (`parent.ReceiveBeginPlay`))

(event `self.ReceiveAnyDamage`
  (params (Damage :type "Float (single-precision)") (DamageType :type "DamageType Object Reference") (InstigatedBy :type "Controller Object Reference") (DamageCauser :type "Actor Object Reference"))
  (bind _gc_component (`self.GC_Component`))
  (`self.Take Damage Base` Damage)
  (if (<= (`self.Current Health`) 0.0)
    (for _array_element (`self.Weak Points`)
      (if (`KismetSystemLibrary.IsValid` _array_element)
        (bind _gc_component_2 (`/Game/Blueprints/Building_Blueprints/BP_BuildingParentAverage.GC_Component` _array_element))
        (`GeometryCollectionComponent.CrumbleCluster` _gc_component_2 1)
        (`GeometryCollectionComponent.CrumbleCluster` _gc_component_2 2)
        (`PrimitiveComponent.SetSimulatePhysics` _gc_component_2 true)
        (`ActorComponent.K2_DestroyComponent` (`/Game/Blueprints/Building_Blueprints/Skyscrapers/BP_SkyscraperWeakpointParent.Box` _array_element))))
    (`GeometryCollectionComponent.CrumbleCluster` _gc_component 1)
    (`PrimitiveComponent.SetSimulatePhysics` _gc_component true)
    (`GameplayStatics.PlaySoundAtLocation` (`self.Destuction SFX`) (`self.K2_GetActorLocation`) (struct) 1.0 1.0 0.0 null null null null)
    (`KismetSystemLibrary.Delay` 5.0)
    (for _array_element_2 (`self.Weak Points`)
      (`/Game/Blueprints/Building_Blueprints/Skyscrapers/BP_SkyscraperWeakpointParent.Shrink` _array_element_2))
    (`Timeline|Timeline_1`
      (:`Finished`
        (`KismetSystemLibrary.Delay` 0.5)
        (`self.K2_DestroyActor`)))))

(fn `Core Hit`
  (params (Damage :type "Float (double-precision)"))
  (bind _current_health (`self.Current Health`))
  (bind _returnvalue (<= _current_health 0.0))
  (if (`self.bCanBeDamaged`)
    (set `self.damageTaken` Damage)
    (if (> (/ (`self.damageTaken`) (`self.TotalHealth`)) 0.05)
      (`self.ShakeBuilding`) ; skip if too low damage
      (`self.SpawnMoneyUI`) ; skip if too low damage
    )
    (if (not _returnvalue)
      (set `self.Current Health` (- _current_health (`self.damageTaken`)))
      (if _returnvalue
        (`/Game/Blueprints/Systems/BPGM_Volcanewt.BuildingDestroyed` (`self.As BPGM Volcanewt_0`) (`self.MonetaryValue`) self)))))

(fn `UserConstructionScript`
  (`parent.UserConstructionScript`)
  ;[1 1 1] Accumulates # of weakpoints based on the array assigned in-engine
  (for (_ _array_index) (`self.Weak Points`)
    (set `self.# of Weak Points` _array_index))
  (set `self.# of Weak Points` (+ (`self.# of Weak Points`) 1)))