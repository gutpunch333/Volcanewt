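; Parent Blueprint for skyscraper shielder buildings, which keep connected shields up until the whole group of adjacent shielders is destroyed.
; BeginPlay counts the adjacent shielders.
; When damage first leaves health at zero or below, it marks itself destroyed and tallies neighbors that are dead or invalid.
; If every neighbor is down, it calls DisableShield on each connected shield, so the last shielder to fall drops them.
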(event `self.ReceiveBeginPlay`
  (`parent.ReceiveBeginPlay`)
  (for _ (`self.Adjacent Shielders`)
    (`/Engine/EditorBlueprintResources/StandardMacros.IncrementInt` (`self.Adjacent Shielders Count`))))

(event `self.ReceiveAnyDamage`
  (params (Damage :type "Float (single-precision)") (DamageType :type "DamageType Object Reference") (InstigatedBy :type "Controller Object Reference") (DamageCauser :type "Actor Object Reference"))
  (bind _connected_shields (`self.Connected Shields`))
  (`parent.ReceiveAnyDamage` Damage DamageType InstigatedBy DamageCauser)
  (if (<= (`self.Current Health`) 0.0)
    (if (not (`self.Destroyed`))
      (set `self.Destroyed` true)
      ;[1 1 1] Determine if other skyscraper shielders are alive
      (if true
        (for _array_element (`self.Adjacent Shielders`)
          (if (`KismetSystemLibrary.IsValid` _array_element)
            (if (<= (`/Game/Blueprints/Building_Blueprints/BP_BuildingParentAverage.Current Health` _array_element) 0.0)
              (`/Engine/EditorBlueprintResources/StandardMacros.IncrementInt` (`self.Shielders Destroyed`) :!label _label))
            (else
              (goto _label))))
        (if (== (`self.Shielders Destroyed`) (`self.Adjacent Shielders Count`))
          ;[1 1 1] If false, destroy appropriate shields
          (for (_array_element_2 _array_index) _connected_shields
            (if (`KismetArrayLibrary.Array_IsValidIndex` _connected_shields _array_index)
              (`/Game/Blueprints/Building_Blueprints/Skyscrapers/BP_SkyscraperShieldParent.Disable Shield` _array_element_2))))))))

(fn `UserConstructionScript`
  (`parent.UserConstructionScript`))