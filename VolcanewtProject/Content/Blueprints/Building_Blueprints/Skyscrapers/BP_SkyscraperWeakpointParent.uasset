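; Parent Blueprint for destructible skyscraper weak points that take damage only while their skyscraper is vulnerable.
; Each hit notifies the skyscraper, shakes the building, spawns money UI and drains local health.
; At depletion the Geometry Collection crumbles with physics and sound, dealing the skyscraper an equal share of its max health per weak point.
; Hits below zero health pass reduced damage to the skyscraper; Shrink plays a timeline, then destroys the actor.
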(event `self.ReceiveBeginPlay`
  (set `self.Weak Point GC` null)
  (set `self.TotalHealth` (`self.Max Health`)))

(event `self.ReceiveAnyDamage`
  (params (Damage :type "Float (single-precision)") (DamageType :type "DamageType Object Reference") (InstigatedBy :type "Controller Object Reference") (DamageCauser :type "Actor Object Reference"))
  (bind _skyscraper_ref (`self.Skyscraper Ref`))
  (bind _skyscraper_ref_2 (`self.Skyscraper Ref`))
  (bind _gc_component (`self.GC_Component`))
  ;[1 1 1] Determines if point is damagable and where
  (if (`/Game/Blueprints/Building_Blueprints/Skyscrapers/BP_SkyscraperParent.Vulnerable` (`self.Skyscraper Ref`))
    (bind _output_get (set `self.damageTaken` Damage))
    (if (>= (`self.Current Health`) 0.0)
      ;[1 1 1] Hits either the weak point or skyscraper core if weakpoint is destroyed
      (`/Game/Blueprints/Building_Blueprints/Skyscrapers/BP_SkyscraperParent.Weak Point Hit` _skyscraper_ref self _output_get)
      (`self.ShakeBuilding`)
      (`self.SpawnMoneyUI`)
      (set `self.Current Health` (- (`self.Current Health`) (`self.damageTaken`)))
      ;[1 1 1] Crumbles the actor's geometry cluster
      (if (<= (`self.Current Health`) 0.0)
        (`GeometryCollectionComponent.CrumbleCluster` _gc_component 0)
        (`GeometryCollectionComponent.CrumbleCluster` _gc_component 1)
        (`GeometryCollectionComponent.CrumbleCluster` _gc_component 2)
        ;[1 1 1] Applies damage to the skyscraper's core based on the number of weak points
        (`PrimitiveComponent.SetSimulatePhysics` _gc_component true)
        (`GameplayStatics.PlaySoundAtLocation` (`self.Destuction SFX_0`) (`self.K2_GetActorLocation`) (struct) 1.0 1.0 0.0 null null null null)
        (`GameplayStatics.ApplyDamage` _skyscraper_ref_2 (/ (`/Game/Blueprints/Building_Blueprints/BP_BuildingParentAverage.Max Health` _skyscraper_ref_2) (`/Game/Blueprints/Building_Blueprints/Skyscrapers/BP_SkyscraperParent.# of Weak Points` _skyscraper_ref_2))))
      (else
        (`GameplayStatics.ApplyDamage` _skyscraper_ref (/ _output_get 3.0))))))

(event `Shrink`
  (`Timeline|Timeline_0`
    (:`Finished`
      (`KismetSystemLibrary.Delay` 0.5)
      (`self.K2_DestroyActor`))))

(fn `UserConstructionScript`
  (set `self.Current Health` (`self.Max Health`))
  (set `self.ActorStartingLocaton` (`self.K2_GetActorLocation`))
  (set `self.shakeTime` 1.0))