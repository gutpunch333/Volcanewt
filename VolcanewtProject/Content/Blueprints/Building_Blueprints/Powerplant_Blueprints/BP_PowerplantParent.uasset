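; Base Blueprint for powerplant buildings that reports each powerplant's creation and destruction to the Volcanewt game mode.
; On BeginPlay it runs the parent building logic, then calls PowerplantCount on the game mode reference.
; On AnyDamage it lets the parent handle the hit, then calls PowerplantDestroyed whenever CurrentHealth is at or below zero.
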(event `self.ReceiveBeginPlay`
  (`parent.ReceiveBeginPlay`)
  (`/Game/Blueprints/Systems/BPGM_Volcanewt.Powerplant Count` (`self.As BPGM Volcanewt_0`)))

(event `self.ReceiveAnyDamage`
  (params (Damage :type "Float (single-precision)") (DamageType :type "DamageType Object Reference") (InstigatedBy :type "Controller Object Reference") (DamageCauser :type "Actor Object Reference"))
  (`parent.ReceiveAnyDamage` Damage DamageType InstigatedBy DamageCauser)
  (if (<= (`self.Current Health`) 0.0)
    (`/Game/Blueprints/Systems/BPGM_Volcanewt.Powerplant Destroyed` (`self.As BPGM Volcanewt_0`))))

(fn `UserConstructionScript`
  (`parent.UserConstructionScript`))