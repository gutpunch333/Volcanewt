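; BP_PowerplantHub is a damageable powerplant hub building that owns an array of sub-plants and reports to the Volcanewt game mode.
; BeginPlay calls the game mode's powerplant count and stores the last sub index as TotalSubs.
; At zero health it reports its destruction and damages each sub by its max health at staggered intervals.
; SubDestroyed prunes the array; when empty, the hub destroys itself after a delay.
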(event `self.ReceiveBeginPlay`
  (`parent.ReceiveBeginPlay`)
  (`/Game/Blueprints/Systems/BPGM_Volcanewt.Powerplant Count` (`self.As BPGM Volcanewt_0`))
  (for (_ _array_index) (`self.Powerplant Subs`)
    (set `self.Total Subs` _array_index)))

(event `self.ReceiveAnyDamage`
  (params (Damage :type "Float (single-precision)") (DamageType :type "DamageType Object Reference") (InstigatedBy :type "Controller Object Reference") (DamageCauser :type "Actor Object Reference"))
  (bind _powerplant_subs (`self.Powerplant Subs`))
  (`parent.ReceiveAnyDamage` Damage DamageType InstigatedBy DamageCauser)
  (if (<= (`self.Current Health`) 0.0)
    (`/Game/Blueprints/Systems/BPGM_Volcanewt.Powerplant Destroyed` (`self.As BPGM Volcanewt_0`))
    (if (`KismetArrayLibrary.Array_IsValidIndex` _powerplant_subs)
      (bind _array_element (`/Game/Blueprints/Building_Blueprints/Powerplant_Blueprints/NewMacroLibrary.For Each Loop With Delay` _powerplant_subs)
        (:`Loop Body`
          (`GameplayStatics.ApplyDamage` _array_element (`/Game/Blueprints/Building_Blueprints/BP_BuildingParentAverage.Max Health` _array_element)))))))

(event `Sub Destroyed`
  (params (`Destroyed Sub` :type "/Game/Blueprints/Building_Blueprints/Powerplant_Blueprints/BP_PowerplantSub Object Reference"))
  (bind _powerplant_subs (`self.Powerplant Subs`))
  (bind _returnvalue (`KismetArrayLibrary.Array_IsValidIndex` _powerplant_subs))
  (set `self.Destroyed Sub` `Destroyed Sub`)
  ;[1 1 1] Checks if there are subplants to destroy
  (if _returnvalue
    (for (_array_element _array_index) _powerplant_subs
      ;[1 1 1] Removes index of subplant when it is destroyed
      (if (== _array_element (`self.Destroyed Sub`))
        (`KismetArrayLibrary.Array_Remove` (`self.Powerplant Subs`) _array_index)))
    ;[1 1 1] If no subplants remain, destroys the hub
    (if (not _returnvalue)
      (`KismetSystemLibrary.Delay` 1.0)
      (`GameplayStatics.ApplyDamage` self (`self.Max Health`))
      (`PrimitiveComponent.AddImpulse` (`self.GC_Component`) (0.0 0.0 0.0) "None" false))))

(fn `UserConstructionScript`
  (`parent.UserConstructionScript`))