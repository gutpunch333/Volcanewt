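; Ferris wheel building actor that spins while it has health and can be destroyed by damage.
; Tick rotates the merged wheel mesh by a fixed per-frame step, so speed depends on frame rate.
; BeginPlay and AnyDamage defer to the parent; at zero health, the wheel and car components are destroyed.
; Older standalone health, scoring, crumble and fade-out logic remains in the graphs but never runs.
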(event `self.ReceiveTick`
  (params (DeltaSeconds :type "Float (single-precision)"))
  (if (not (<= (`self.Current Health`) 0.0))
    (`SceneComponent.K2_AddLocalRotation` (`self.SM_MERGED_StaticMeshActor_13`) (struct :`Roll` 0.4) false false)))

(event `self.ReceiveBeginPlay`
  (`parent.ReceiveBeginPlay`))

(event `self.ReceiveAnyDamage`
  (params (Damage :type "Float (single-precision)") (DamageType :type "DamageType Object Reference") (InstigatedBy :type "Controller Object Reference") (DamageCauser :type "Actor Object Reference"))
  (`parent.ReceiveAnyDamage` Damage null null null)
  (if (<= (`self.Current Health`) 0.0)
    (`ActorComponent.K2_DestroyComponent` (`self.sm_ferrisCar_v6`))
    (`ActorComponent.K2_DestroyComponent` (`self.SM_MERGED_StaticMeshActor_13`))
    (`ActorComponent.K2_DestroyComponent` (`self.sm_ferrisCar_v5`))
    (`ActorComponent.K2_DestroyComponent` (`self.sm_ferrisCar_v4`))
    (`ActorComponent.K2_DestroyComponent` (`self.sm_ferrisCar_v7`))
    (`ActorComponent.K2_DestroyComponent` (`self.sm_ferrisCar_v3`))
    (`ActorComponent.K2_DestroyComponent` (`self.sm_ferrisCar_v2`))
    (`ActorComponent.K2_DestroyComponent` (`self.sm_ferrisCar_v8`))
    (`ActorComponent.K2_DestroyComponent` (`self.sm_ferrisCar_v11`))
    (`ActorComponent.K2_DestroyComponent` (`self.sm_ferrisCar_v10`))
    (`ActorComponent.K2_DestroyComponent` (`self.sm_ferrisCar_v9`))))

(fn `UserConstructionScript`
  (`parent.UserConstructionScript`)
  (set `self.Fade Out` false))