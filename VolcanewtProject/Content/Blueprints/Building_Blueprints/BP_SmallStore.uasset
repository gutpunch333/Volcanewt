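; BP_SmallStore is a destructible small store building with a monetary value, which it passes to its BP_BuildingParent child actor.
; AnyDamage drains its health; at zero it reports to BPGM_Volcanewt, crumbles its Geometry Collection with sound, fades out dynamic materials on a timeline, then destroys itself.
; Tick, noted as activated by the game mode's bonus objective, updates an objective marker widget with the player's distance in meters.
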(event `self.ReceiveBeginPlay`
  ;[1 1 1] Adds to background information in game mode
  (bind _asbpgm_volcanewt (cast `/Game/Blueprints/BPGM_Volcanewt` (`GameplayStatics.GetGameMode`)))
  (set `self.As BPGM Volcanewt` _asbpgm_volcanewt)
  (bind _asbp_building_parent (cast `/Game/Blueprints/BP_BuildingParent` (`ChildActorComponent.ChildActor` (`self.BP_BuildingParent`))))
  (set `/Game/Blueprints/BP_BuildingParent.MonetaryValue` (`self.SmallStoreMV`) _asbp_building_parent)
  (bind _asbpw_objective_marker (cast `/Game/UI/Widgets/BPW_ObjectiveMarker` (`WidgetComponent.GetUserWidgetObject` (`self.Widget`))))
  (set `self.As BPW Objective Marker` _asbpw_objective_marker))

(event `self.ReceiveTick`
  (params (DeltaSeconds :type "Float (single-precision)"))
  ;[1 1 1] Activated by Bonus Objective in Gamemode. Calculates the distance between player and bonused building and updates the UI respectively in Meters
  (`/Game/UI/Widgets/BPW_ObjectiveMarker.Set DistanceText` (`self.As BPW Objective Marker`) (`KismetTextLibrary.Conv_DoubleToText` (/ (`KismetMathLibrary.Vector_Distance` (`self.K2_GetActorLocation`) (`self.K2_GetActorLocation` (`GameplayStatics.GetPlayerPawn` 0))) 100.0) "HalfToEven" false true 1 324 0 0)))

(event `self.ReceiveAnyDamage`
  (params (Damage :type "Float (single-precision)") (DamageType :type "DamageType Object Reference") (InstigatedBy :type "Controller Object Reference") (DamageCauser :type "Actor Object Reference"))
  (bind _smallstorehealth (`self.SmallStoreHealth`))
  (bind _returnvalue (<= _smallstorehealth 0.0))
  (if (not _returnvalue)
    (set `self.SmallStoreHealth` (- _smallstorehealth Damage))
    (if _returnvalue
      (`/Game/Blueprints/BPGM_Volcanewt.BuildingDestroyed` (`self.As BPGM Volcanewt`) (`self.SmallStoreMV`) self)
      (`PrimitiveComponent.SetSimulatePhysics` (`self.type_a_building5_GeometryCollection`) true)
      (`GeometryCollectionComponent.CrumbleCluster` (`self.type_a_building5_GeometryCollection`) 0)
      (`GeometryCollectionComponent.CrumbleCluster` (`self.type_a_building5_GeometryCollection`) 1)
      (`GameplayStatics.PlaySoundAtLocation` "/Game/Audio/SoundEffects/rocks.rocks" (0.0 0.0 0.0) (struct) 0.75 1.4 2.7 null null null null)
      (`KismetSystemLibrary.Delay` 1.0)
      ;[1 1 1] Lerping the dynamic materials' parameter values to fade the building out
      (bind (_direction _fadealpha) (`Timeline|Timeline` :!via `PlayFromStart`)
        (:`Update`
          (bind _returnvalue_2 (`KismetMathLibrary.Lerp` 1.0 0.0 _fadealpha))
          (`MaterialInstanceDynamic.SetScalarParameterValue` (`self.Dynamic Material Instance Index 0`) "fadeOut" _returnvalue_2)
          (`MaterialInstanceDynamic.SetScalarParameterValue` (`self.Dynamic Material Instance Index 1`) "fadeOut" _returnvalue_2))
        (:`Finished`
          (`KismetSystemLibrary.Delay` 0.5)
          (`self.K2_DestroyActor`))))))

(fn `UserConstructionScript`
  (bind _returnvalue (`PrimitiveComponent.CreateDynamicMaterialInstance` (`self.type_a_building5_GeometryCollection`) 1 "/Game/Enemies/EnemyAssets/lambert1.lambert1" "None"))
  (set `self.Dynamic Material Instance Index 1` _returnvalue)
  (bind _returnvalue_2 (`PrimitiveComponent.CreateDynamicMaterialInstance` (`self.type_a_building5_GeometryCollection`) 0 "/Game/Enemies/EnemyAssets/lambert1.lambert1" "None"))
  (set `self.Dynamic Material Instance Index 0` _returnvalue_2))