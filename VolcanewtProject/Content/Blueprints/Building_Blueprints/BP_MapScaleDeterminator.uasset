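; Construction-script actor that lays out a grid of child actors, apparently as a scale reference for sizing maps, judging by its name.
; Nested loops over X and Y step 2000 units per cell from the root's world transform, adding manually attached child actor components.
; Each row also gets an extra child at its start, overlapping the first cell.
; The event graph is empty, and unconnected instanced static mesh nodes remain unused.
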(fn `UserConstructionScript`
  (set `self.current transform` (`SceneComponent.K2_GetComponentToWorld` (`self.DefaultSceneRoot`)))
  (for _ (range (+ (`self.Y`) 1))
    (`AddComponent|NODE_AddChildActorComponent-1` :`bManualAttachment` true :`RelativeTransform` (`self.current transform`))
    (for _index (range (+ (`self.X`) 1))
      (`AddComponent|NODE_AddChildActorComponent-2` :`bManualAttachment` true :`RelativeTransform` (`KismetMathLibrary.MakeTransform` (+ (.location (`self.current transform`)) (`KismetMathLibrary.MakeVector` (* 2000.0 _index) 0.0)) (.rotation (`self.current transform`)) (.scale (`self.current transform`)))))
    (set `self.current transform` (`KismetMathLibrary.MakeTransform` (+ (.location (`self.current transform`)) (0.0 2000.0 0.0)) (.rotation (`self.current transform`)) (.scale (`self.current transform`))))))