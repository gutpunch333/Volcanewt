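; BP_BSF is a destructible building that makes the buildings within its bounds invulnerable while it stands.
; Shortly after BeginPlay it disables damage on overlapping actors tagged Building.
; OutsideCheck then restores damage for anything touching four outer box colliders, gathered in the construction script, and destroys those boxes.
; When health runs out or BSFDeactivated fires, it makes all overlapping actors damageable again and destroys itself.
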(event `self.ReceiveBeginPlay`
  (`parent.ReceiveBeginPlay`)
  ;[1 1 1] Grabs all actors touching the BSF
  (`KismetSystemLibrary.Delay` 0.5)
  (for _array_element (`self.GetOverlappingActors` null)
    ;[1 1 1] Determines if the actor is a building
    (for _array_element_2 (`Actor.Tags` _array_element)
      (if (== _array_element_2 "Building")
        ;[1 1 1] Makes it invulnerable
        (set `Actor.bCanBeDamaged` false _array_element))))
  (`self.Outside Check`))

(event `self.ReceiveAnyDamage`
  (params (Damage :type "Float (single-precision)") (DamageType :type "DamageType Object Reference") (InstigatedBy :type "Controller Object Reference") (DamageCauser :type "Actor Object Reference"))
  ;[1 1 1] Reads when the BSF runs out of health
  (`parent.ReceiveAnyDamage` Damage null null null)
  (if (<= (`self.Current Health`) 0.0)
    ;[1 1 1] Grabs all actors inside the BSF and enables them to be damanged again
    (for _array_element (`self.GetOverlappingActors` null)
      (set `Actor.bCanBeDamaged` true _array_element))
    (`self.K2_DestroyActor`)))

(event `BSF Deactivated`
  (for _array_element (`self.GetOverlappingActors` null)
    (set `Actor.bCanBeDamaged` true _array_element))
  (`self.K2_DestroyActor`))

(fn `Outside Check`
  ;[1 1 1] Gets all actors inside box colliders outside BSF and allows them to be damaged
  (for _array_element (`self.Outside Colliders`)
    (for _array_element_2 (`PrimitiveComponent.GetOverlappingActors` _array_element null)
      (set `Actor.bCanBeDamaged` true _array_element_2)))
  (`ActorComponent.K2_DestroyComponent` (`self.Box`))
  (`ActorComponent.K2_DestroyComponent` (`self.Box2`))
  (`ActorComponent.K2_DestroyComponent` (`self.Box3`))
  (`ActorComponent.K2_DestroyComponent` (`self.Box1`)))

(fn `UserConstructionScript`
  (`parent.UserConstructionScript`)
  (`KismetArrayLibrary.Array_Add` (`self.Outside Colliders`) (`self.Box`))
  (`KismetArrayLibrary.Array_Add` (`self.Outside Colliders`) (`self.Box1`))
  (`KismetArrayLibrary.Array_Add` (`self.Outside Colliders`) (`self.Box2`))
  (`KismetArrayLibrary.Array_Add` (`self.Outside Colliders`) (`self.Box3`)))