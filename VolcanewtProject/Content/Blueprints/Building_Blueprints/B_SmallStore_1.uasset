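; Small store building actor that shows the player's distance to it on an objective marker when it is a bonus objective.
; BeginPlay runs the parent logic and caches the marker widget; Tick, noted as enabled by the game mode, writes the distance in whole meters.
; Its own health, crumble, money popup and material fade-out logic is disconnected and never runs, leaving only parent calls and the marker update live.
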(event `self.ReceiveBeginPlay`
  (`parent.ReceiveBeginPlay`)
  (bind _asbpw_objective_marker (cast `/Game/UI/Widgets/BPW_ObjectiveMarker` (`WidgetComponent.GetUserWidgetObject` (`self.Widget`))))
  (set `self.As BPW Objective Marker` _asbpw_objective_marker))

(event `self.ReceiveTick`
  (params (DeltaSeconds :type "Float (single-precision)"))
  ;[1 1 1] Activated by Bonus Objective in Gamemode. Calculates the distance between player and bonused building and updates the UI respectively in Meters
  (`/Game/UI/Widgets/BPW_ObjectiveMarker.Set DistanceText` (`self.As BPW Objective Marker`) (`KismetTextLibrary.Conv_DoubleToText` (/ (`KismetMathLibrary.Vector_Distance` (`self.K2_GetActorLocation`) (`self.K2_GetActorLocation` (`GameplayStatics.GetPlayerPawn` 0))) 100.0) "HalfToEven" false true 1 324 0 0)))

(fn `UserConstructionScript`
  (`parent.UserConstructionScript`))