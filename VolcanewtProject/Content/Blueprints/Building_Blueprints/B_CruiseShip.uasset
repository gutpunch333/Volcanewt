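; Cruise ship building actor for the Volcanewt game mode, with its live behavior left entirely to its parent class.
; BeginPlay, AnyDamage and the construction script only forward to the parent implementations.
; Disconnected leftover graphs hold an older standalone destruction sequence that never runs: game mode notification, mesh crumbling, sound, money UI spawn, timeline material fade and actor destruction.
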(event `self.ReceiveBeginPlay`
  (`parent.ReceiveBeginPlay`))

(event `self.ReceiveAnyDamage`
  (params (Damage :type "Float (single-precision)") (DamageType :type "DamageType Object Reference") (InstigatedBy :type "Controller Object Reference") (DamageCauser :type "Actor Object Reference"))
  (`parent.ReceiveAnyDamage` Damage null null null))

(fn `UserConstructionScript`
  ;[1 1 1] Creating and setting references to Dynamic Material instances
  (`parent.UserConstructionScript`))