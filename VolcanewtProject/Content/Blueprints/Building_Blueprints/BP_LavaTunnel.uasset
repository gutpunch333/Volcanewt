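; BP_LavaTunnel is the Volcanewt level exit, completing the level when an actor tagged Newt overlaps it with the destruction meter and powerplant objectives met.
; Its objective marker starts hidden; the first tick of a looping timer reveals it, without checking objectives.
; That same one-time event randomly plays or reverses a timeline that shakes and lerps the mesh toward the capsule's transform.
; A second shake-only event is never called.
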(event `Make Widget Hidden`
  (bind _aswbp_objective_marker (cast `/Game/UI/Widgets/WBP_ObjectiveMarker` (`WidgetComponent.GetWidget` (`self.LavaTunnelWidgetComponent`))))
  (bind _output_get (set `self.As WBP Objective Marker` _aswbp_objective_marker))
  (set `/Game/UI/Widgets/WBP_ObjectiveMarker.ObjectiveMarkerType` "NewEnumerator2" _output_get)
  (`Widget.SetVisibility` _output_get "Collapsed"))

(event `self.ReceiveBeginPlay`
  (bind (_returnvalue_location _returnvalue_rotation) (`KismetMathLibrary.BreakTransform` (`SceneComponent.GetRelativeTransform` (`self.StaticMesh`))))
  (`self.Make Widget Hidden`)
  (bind _asbpgm_volcanewt (cast `/Game/Blueprints/Systems/BPGM_Volcanewt` (`GameplayStatics.GetGameMode`)))
  (set `self.As BPGM Volcanewt` _asbpgm_volcanewt)
  (set `self.Initial Position` _returnvalue_location)
  (set `self.Initial Rotation` _returnvalue_rotation)
  (set `self.New Destination` (`SceneComponent.GetRelativeTransform` (`self.Capsule`)))
  (`KismetSystemLibrary.K2_SetTimerDelegate` (delegate `Check if objectives complete`) 18.0 true) ; how frequently the end level condition is checked from here. Would prefer if the game mode tracked completion itself somewhere
)

(event `self.Box.OnComponentBeginOverlap`
  (params (OverlappedComponent :type "PrimitiveComponent Object Reference") (OtherActor :type "Actor Object Reference") (OtherComp :type "PrimitiveComponent Object Reference") (OtherBodyIndex :type Integer) (bFromSweep :type Boolean) (SweepResult :type "HitResult Structure (by ref)"))
  (bind _as_bpgm_volcanewt (`self.As BPGM Volcanewt`))
  (for _array_element (`Actor.Tags` OtherActor)
    (if (== _array_element "Newt")
      (if (and (`/Game/Blueprints/Systems/BPGM_Volcanewt.Destruction Meter Filled` _as_bpgm_volcanewt) (`/Game/Blueprints/Systems/BPGM_Volcanewt.Required Powerplants Destroyed` _as_bpgm_volcanewt))
        (`/Game/Blueprints/Systems/BPGM_Volcanewt.Level Complete` _as_bpgm_volcanewt)))))

(event `Check if objectives complete`
  ;[1 1 1] Debug activates the timeline
  (`self.Objectives Complete`))

(event `Making widget visible`
  ;[1 1 1] Setting objective marker to correct type and making visible
  (`Widget.SetVisibility` (`self.As WBP Objective Marker`) "Visible"))

(event `self.Box1.OnComponentBeginOverlap`
  (params (OverlappedComponent :type "PrimitiveComponent Object Reference") (OtherActor :type "Actor Object Reference") (OtherComp :type "PrimitiveComponent Object Reference") (OtherBodyIndex :type Integer) (bFromSweep :type Boolean) (SweepResult :type "HitResult Structure (by ref)"))
  ;[1 1 1] Debug activates the timeline
)

(event `Objectives Complete`
  (bind _initial_position (`self.Initial Position`))
  (bind (_new_destination_location _new_destination_rotation) (`KismetMathLibrary.BreakTransform` (`self.New Destination`)))
  (`/Engine/EditorBlueprintResources/StandardMacros.DoOnce` false
    (:`Completed`
      (`self.Making widget visible`)
      (`TimelineComponent.SetLooping` (`self.Timeline`) true)
      (switch `int` (`KismetMathLibrary.RandomInteger` 1)
        (:`0`
          (bind (_direction _time _shake) (`Timeline|Timeline` :!via `PlayFromStart` :!label _label)
            (:`Update`
              (bind (_returnvalue_x _returnvalue_y) (`KismetMathLibrary.BreakVector` (+ _initial_position _shake)))
              (bind (_returnvalue_x_2 _returnvalue_y_2 _returnvalue_z) (`KismetMathLibrary.BreakVector` (`KismetMathLibrary.VLerp` _initial_position _new_destination_location _time)))
              (`SceneComponent.K2_SetRelativeTransform` (`self.StaticMesh`) (`KismetMathLibrary.MakeTransform` (`KismetMathLibrary.MakeVector` _returnvalue_x _returnvalue_y _returnvalue_z) (`KismetMathLibrary.RLerp` (`self.Initial Rotation`) _new_destination_rotation _time)) false true)
              (`KismetSystemLibrary.Delay` 3.0)
              (`TimelineComponent.SetLooping` (`self.Timeline`) false))))
        (:`1`
          (goto _label :!via `ReverseFromEnd`))))))

(event `CustomEvent`
  (`TimelineComponent.SetLooping` (`self.Timeline_0`) true)
  (switch `int` (`KismetMathLibrary.RandomInteger` 1)
    (:`0`
      (bind (_direction _shakevector) (`Timeline|Timeline_0` :!via `PlayFromStart` :!label _label_2)
        (:`Update`
          (bind (_returnvalue_x _returnvalue_y) (`KismetMathLibrary.BreakVector` (+ (`self.Initial Position`) _shakevector)))
          (`SceneComponent.K2_SetRelativeLocation` (`self.StaticMesh`) (`KismetMathLibrary.MakeVector` _returnvalue_x _returnvalue_y) false true)
          (`KismetSystemLibrary.Delay` 3.0)
          (`TimelineComponent.SetLooping` (`self.Timeline_0`) false))))
    (:`1`
      (goto _label_2 :!via `ReverseFromEnd`))))

(fn `UserConstructionScript`)