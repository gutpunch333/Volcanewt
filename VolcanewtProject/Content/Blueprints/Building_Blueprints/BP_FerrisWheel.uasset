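; Ferris wheel building Blueprint, a destructible-building child that adds a constantly spinning wheel.
; Tick rotates the merged static mesh by a fixed local step each frame, without delta-time scaling, so speed follows frame rate.
; BeginPlay, AnyDamage and the construction script only call the parent's versions.
; Local health, Geometry Collection-style crumble, money payout and material fade-out logic remains in the graphs but is disconnected and never runs.
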(event `self.ReceiveTick`
  (params (DeltaSeconds :type "Float (single-precision)"))
  (`SceneComponent.K2_AddLocalRotation` (`self.SM_MERGED_StaticMeshActor_13`) (struct :`Roll` 0.4) false false))

(event `self.ReceiveBeginPlay`
  (`parent.ReceiveBeginPlay`))

(event `self.ReceiveAnyDamage`
  (params (Damage :type "Float (single-precision)") (DamageType :type "DamageType Object Reference") (InstigatedBy :type "Controller Object Reference") (DamageCauser :type "Actor Object Reference"))
  (`parent.ReceiveAnyDamage` Damage null null null))

(fn `UserConstructionScript`
  ;[1 1 1] Creating and setting references to Dynamic Material instances
  (`parent.UserConstructionScript`))