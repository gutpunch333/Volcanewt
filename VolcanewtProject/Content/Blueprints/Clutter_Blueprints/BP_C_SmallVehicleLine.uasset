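; Clutter Blueprint that lays out a line of static child actors, small vehicles judging by its name, with randomized spacing.
; The construction script starts at the root's world transform and adds manually attached child actor components in a loop driven by Amount.
; Each step moves a random distance in the negative direction along world X when the Y flag is set, otherwise along world Y.
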(fn `UserConstructionScript`
  (set `self.CurrentTransform` (`SceneComponent.K2_GetComponentToWorld` (`self.DefaultSceneRoot`)))
  (if (`self.Y`)
    (for _ (range (+ (`self.Amount`) 1))
      (bind _returnvalue (`AddComponent|NODE_AddChildActorComponent-1` :`bManualAttachment` true :`RelativeTransform` (`self.CurrentTransform`)))
      (set `self.CurrentTransform` (`KismetMathLibrary.MakeTransform` (+ (.location (`self.CurrentTransform`)) (`KismetMathLibrary.MakeVector` (`KismetMathLibrary.RandomFloatInRange` -350.0 -750.0))) (.rotation (`self.CurrentTransform`)) (.scale (`self.CurrentTransform`))))
      (`SceneComponent.SetMobility` _returnvalue "Static"))
    (else
      (for _ (range (+ (`self.Amount`) 1))
        (bind _returnvalue_2 (`AddComponent|NODE_AddChildActorComponent-0` :`bManualAttachment` true :`RelativeTransform` (`self.CurrentTransform`)))
        (set `self.CurrentTransform` (`KismetMathLibrary.MakeTransform` (+ (.location (`self.CurrentTransform`)) (`KismetMathLibrary.MakeVector` 0.0 (`KismetMathLibrary.RandomFloatInRange` -350.0 -750.0))) (.rotation (`self.CurrentTransform`)) (.scale (`self.CurrentTransform`))))
        (`SceneComponent.SetMobility` _returnvalue_2 "Static")))))