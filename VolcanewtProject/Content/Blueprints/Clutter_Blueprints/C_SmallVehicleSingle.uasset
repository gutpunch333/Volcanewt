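; C_SmallVehicleSingle is a destructible small-vehicle clutter prop with a random monetary value.
; The construction script picks a random mesh, adds it as an instance, assigns the matching destroyed Geometry Collection and rolls the value.
; The first overlap marks it destroyed; if from the player pawn, it swaps the mesh for the flattened, physics-simulating Geometry Collection and calls the parent's RemoveValue.
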(event `self.InstancedStaticMesh.OnComponentBeginOverlap`
  (params (OverlappedComponent :type "PrimitiveComponent Object Reference") (OtherActor :type "Actor Object Reference") (OtherComp :type "PrimitiveComponent Object Reference") (OtherBodyIndex :type Integer) (bFromSweep :type Boolean) (SweepResult :type "HitResult Structure (by ref)"))
  (if (not (`self.Destroyed`))
    (set `self.Destroyed` true)
    (if (== OtherActor (`GameplayStatics.GetPlayerPawn` 0))
      (`SceneComponent.SetWorldScale3D` (`self.GC_Component`) (1.0 1.0 0.25))
      (`PrimitiveComponent.SetSimulatePhysics` (`self.GC_Component`) true)
      (`SceneComponent.SetVisibility` (`self.GC_Component`) true false)
      (`ActorComponent.K2_DestroyComponent` (`self.InstancedStaticMesh`))
      (`self.Remove Value`))))

(event `self.Remove Value`
  (`parent.Remove Value`))

(fn `UserConstructionScript`
  ;[1 1 1] Selects a random small vehicle static mesh and spawns it with the static mesh
  (bind _output_get (set `self.Static Mesh Ref` (`|GetArrayItem` (`self.Static Mesh`) (`KismetMathLibrary.RandomInteger` 3))))
  (`StaticMeshComponent.SetStaticMesh` (`self.InstancedStaticMesh`) _output_get)
  (`InstancedStaticMeshComponent.AddInstance` (`self.InstancedStaticMesh`) (`SceneComponent.GetRelativeTransform` (`self.DefaultSceneRoot`)) true)
  ;[1 1 1] Applies an appropriate destroyed car model
  (`GeometryCollectionComponent.SetRestCollection` (`self.GC_Component`) (`BlueprintMapLibrary.Map_Find` (`self.static`) (`self.Static Mesh Ref`)))
  ;[1 1 1] Sets a random value for the car
  (bind _output_get_2 (set `self.Monetary Value_0` (`KismetMathLibrary.RandomIntegerInRange` 5000 20000)))
  (set `self.Monetary Value` (`KismetMathLibrary.Conv_IntToDouble` _output_get_2)))