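; Clutter Blueprint for a single small vehicle that is destroyed when the player pawn overlaps it.
; The overlap flattens GCComponent on Z, turns on its physics and visibility, removes the InstancedStaticMesh, then fires RemoveValue, which forwards to the parent.
; A Destroyed flag makes this one-shot, but it is set before the player check, so any earlier overlap blocks later destruction.
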(event `self.InstancedStaticMesh.OnComponentBeginOverlap`
  (params (OverlappedComponent :type "PrimitiveComponent Object Reference") (OtherActor :type "Actor Object Reference") (OtherComp :type "PrimitiveComponent Object Reference") (OtherBodyIndex :type Integer) (bFromSweep :type Boolean) (SweepResult :type "HitResult Structure (by ref)"))
  (if (not (`self.Destroyed`))
    (set `self.Destroyed` true)
    (if (== OtherActor (`GameplayStatics.GetPlayerPawn` 0))
      (`SceneComponent.SetWorldScale3D` (`self.GC_Component`) (1.0 1.0 0.05))
      (`PrimitiveComponent.SetSimulatePhysics` (`self.GC_Component`) true)
      (`SceneComponent.SetVisibility` (`self.GC_Component`) true false)
      (`ActorComponent.K2_DestroyComponent` (`self.InstancedStaticMesh`))
      (`self.Remove Value`))))

(event `self.Remove Value`
  (`parent.Remove Value`))

(fn `UserConstructionScript`)