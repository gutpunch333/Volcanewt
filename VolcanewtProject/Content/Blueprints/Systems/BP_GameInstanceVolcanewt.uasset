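; Game Instance that owns the player's gamma and volume settings and persists them in a settings save game.
; On Init it loads or creates the save slot, copies the saved values into its variables and applies them.
; ApplySettings overrides and pushes Master, Music and SFX sound mixes and sends gamma as a console command.
; SaveSettings writes the current values back to the save object and saves it asynchronously.
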(event `self.ReceiveInit`
  (`self.Create Settings Save`)
  (`self.Load Settings`))

(event `Create Settings Save`
  ;[1 1 1] Checks if settings save exists, then loads it, or creates one if it doesn't exist
  (bind _returnvalue (`GameplayStatics.DoesSaveGameExist` (`self.SettingsSaveGameName`)))
  (if _returnvalue
    (bind _returnvalue_2 (`GameplayStatics.LoadGameFromSlot` (`self.SettingsSaveGameName`)))
    (bind _asbp_settings_save_game (cast `/Game/Blueprints/Systems/BP_SettingsSaveGame` _returnvalue_2))
    (set `self.SettingsSaveGameRef` _asbp_settings_save_game)
    (else
      (bind _returnvalue_3 (`GameplayStatics.CreateSaveGameObject` "/Game/Blueprints/Systems/BP_SettingsSaveGame.BP_SettingsSaveGame_C"))
      (`GameplayStatics.SaveGameToSlot` _returnvalue_3 (`self.SettingsSaveGameName`))
      (set `self.SettingsSaveGameRef` _returnvalue_3))))

(event `Async Save Settings`
  (bind _settingssavegameref (`self.SettingsSaveGameRef`))
  ;[1 1 1] Saves settings game to slot
  (`/Engine/EditorBlueprintResources/StandardMacros.IsValid` _settingssavegameref
    (:`Is Valid`
      (`AsyncActionHandleSaveGame.AsyncSaveGameToSlot` _settingssavegameref (`self.SettingsSaveGameName`)))
    (:`Is Not Valid`
      (`KismetSystemLibrary.PrintString` "save game ref not valid"))))

(fn `ApplySettings`
  (`GameplayStatics.SetSoundMixClassOverride` "/Game/Audio/MixClasses/Mix_Master.Mix_Master" "/Engine/EngineSounds/Master.Master" (`self.MasterVolumeVal`) 1.0 0.0)
  (`GameplayStatics.PushSoundMixModifier` "/Game/Audio/MixClasses/Mix_Master.Mix_Master")
  (`GameplayStatics.SetSoundMixClassOverride` "/Game/Audio/MixClasses/Mix_Music.Mix_Music" "/Engine/EngineSounds/Music.Music" (`self.MusicVolumeVal`) 1.0 0.0)
  (`GameplayStatics.PushSoundMixModifier` "/Game/Audio/MixClasses/Mix_Music.Mix_Music")
  (`GameplayStatics.SetSoundMixClassOverride` "/Game/Audio/MixClasses/Mix_SFX.Mix_SFX" "/Engine/EngineSounds/SFX.SFX" (`self.SFXVolumeVal`) 1.0 0.0)
  (`GameplayStatics.PushSoundMixModifier` "/Game/Audio/MixClasses/Mix_SFX.Mix_SFX")
  (`KismetSystemLibrary.ExecuteConsoleCommand` (`KismetStringLibrary.Concat_StrStr` "Gamma " (`KismetStringLibrary.Conv_DoubleToString` (`KismetMathLibrary.Lerp` 0.0 4.4 (`self.GammaSettingVal`)))) null))

(fn `Load Settings`
  (set `self.GammaSettingVal` (`/Game/Blueprints/Systems/BP_SettingsSaveGame.SavedGammaSetting` (`self.SettingsSaveGameRef`)))
  (set `self.MasterVolumeVal` (`/Game/Blueprints/Systems/BP_SettingsSaveGame.SavedMasterVolume` (`self.SettingsSaveGameRef`)))
  (set `self.MusicVolumeVal` (`/Game/Blueprints/Systems/BP_SettingsSaveGame.SavedMusicVolume` (`self.SettingsSaveGameRef`)))
  (set `self.SFXVolumeVal` (`/Game/Blueprints/Systems/BP_SettingsSaveGame.SavedSFXVolume` (`self.SettingsSaveGameRef`)))
  (`self.ApplySettings`))

(fn `SaveSettings`
  (set `/Game/Blueprints/Systems/BP_SettingsSaveGame.SavedGammaSetting` (`self.GammaSettingVal`) (`self.SettingsSaveGameRef`))
  (set `/Game/Blueprints/Systems/BP_SettingsSaveGame.SavedMasterVolume` (`self.MasterVolumeVal`) (`self.SettingsSaveGameRef`))
  (set `/Game/Blueprints/Systems/BP_SettingsSaveGame.SavedMusicVolume` (`self.MusicVolumeVal`) (`self.SettingsSaveGameRef`))
  (set `/Game/Blueprints/Systems/BP_SettingsSaveGame.SavedSFXVolume` (`self.SFXVolumeVal`) (`self.SettingsSaveGameRef`))
  (`self.Async Save Settings`))