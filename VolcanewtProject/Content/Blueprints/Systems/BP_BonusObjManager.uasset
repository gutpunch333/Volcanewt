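; BP_BonusObjManager is an actor that hands bonus objective settings to the Volcanewt game mode.
; On BeginPlay it casts the game mode to BPGM_Volcanewt and copies in its civilian and military objective arrays, plus bonus, intermediate and walker-guy timers.
; Empty loops over each array supply the index that sets that category's active bonus value on the game mode.
; It runs no objective logic itself.
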(event `self.ReceiveBeginPlay`
  (bind _as_bpgm_volcanewt (`self.As BPGM Volcanewt`))
  (bind _as_bpgm_volcanewt_2 (`self.As BPGM Volcanewt`))
  (bind _asbpgm_volcanewt (cast `/Game/Blueprints/Systems/BPGM_Volcanewt` (`GameplayStatics.GetGameMode`)))
  (set `self.As BPGM Volcanewt` _asbpgm_volcanewt)
  (set `/Game/Blueprints/Systems/BPGM_Volcanewt.CivillianBonusObjectives` (`self.ActiveCivillianBonusObjectives`) _as_bpgm_volcanewt)
  (set `/Game/Blueprints/Systems/BPGM_Volcanewt.MilitaryBonusObjectives` (`self.ActiveMilitaryBonusObjectives`) _as_bpgm_volcanewt)
  (for (_ _array_index) (`self.ActiveCivillianBonusObjectives`)
    _)
  (set `/Game/Blueprints/Systems/BPGM_Volcanewt.CivillianBonusActive#` _array_index _as_bpgm_volcanewt_2)
  (for (_ _array_index_2) (`self.ActiveMilitaryBonusObjectives`)
    _)
  (set `/Game/Blueprints/Systems/BPGM_Volcanewt.MilitaryBonusActive#` _array_index_2 _as_bpgm_volcanewt_2)
  (set `/Game/Blueprints/Systems/BPGM_Volcanewt.Bonus Timer` (`self.BonusTimer`) _as_bpgm_volcanewt_2)
  (set `/Game/Blueprints/Systems/BPGM_Volcanewt.Bonus Intermediate Timer` (`self.Bonus Intermediate Timer`) _as_bpgm_volcanewt_2)
  (set `/Game/Blueprints/Systems/BPGM_Volcanewt.WalkerGuysTimer` (`self.WalkerGuysTimer`) _as_bpgm_volcanewt_2))

(fn `UserConstructionScript`)