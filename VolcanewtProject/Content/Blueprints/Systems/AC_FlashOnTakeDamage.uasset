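; Actor component that flashes its owner whenever the owner takes any damage, using custom depth stencil values.
; On BeginPlay it caches the owner's components of a configurable class and binds to OnTakeAnyDamage.
; Each hit prints a debug string, writes the chosen stencil (noted as white or blue) to those primitives, then a short timer resets it to default.
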(event `self.ReceiveBeginPlay`
  ;[1 1 1] Setup
  (set `self.Owner` (`self.GetOwner`)) ; Pointer to actor this component\nis attached to
  (add `Actor.OnTakeAnyDamage` (`self.Owner`) (`|CreateDelegate` :!event `StartFlash`)) ; Bind to Owner's OnTakeAnyDamage dispacher.\nThis fires any time the owner recieves some damage.
  (set `self.Actor Components` (`Actor.K2_GetComponentsByClass` (`self.Owner`) (`self.Component Class to Search`))))

(event `StartFlash`
  (params (DamagedActor :type "Actor Object Reference") (Damage :type "Float (single-precision)") (DamageType :type "DamageType Object Reference") (InstigatedBy :type "Controller Object Reference") (DamageCauser :type "Actor Object Reference"))
  ;[1 1 1] Create Flash
  (`KismetSystemLibrary.PrintString` "flash")
  (for _array_element (`self.Actor Components`)
    (bind _asprimitive_component (cast `PrimitiveComponent` _array_element))
    (`/Engine/EditorBlueprintResources/StandardMacros.IsValid` _asprimitive_component
      (:`Is Valid`
        (`PrimitiveComponent.SetCustomDepthStencilValue` _asprimitive_component (`self.Stencil`)) ; Set each component to the stencil we want.\nCurrently:\nWhite = 1\nBlue = 2\nRed = 3
      )))
  (bind _returnvalue (`KismetSystemLibrary.K2_SetTimerDelegate` (`|CreateDelegate` :!event `Reset Stencil`) 0.1)) ; Set a timer to return stencil back to 0
  (set `self.Timer Handle` _returnvalue))

(event `Reset Stencil`
  ;[1 1 1] Reset to normal
  (for _array_element (`self.Actor Components`)
    (bind _asprimitive_component (cast `PrimitiveComponent` _array_element))
    (`PrimitiveComponent.SetCustomDepthStencilValue` _asprimitive_component 0) ; Returning actor stencil to default
  ))