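; BP_MoneyUISpawner is a short-lived actor that shows a floating money cost popup, apparently for hits, through its MoneyWidget component.
; On BeginPlay it passes InputMoneyCost to WBP_MoneycostUI and picks a random end point above its location with sideways scatter.
; The MoveT timeline lerps the actor to that point, then disables widget ticking and destroys the actor.
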(event `self.ReceiveBeginPlay`
  (bind _returnvalue (`self.K2_GetActorLocation`))
  ;[1 1 1] Setting variables in widget UI
  (bind _aswbp_moneycost_ui (cast `/Game/UI/Widgets/WBP_MoneycostUI` (`WidgetComponent.GetWidget` (`self.MoneyWidget`))))
  (set `/Game/UI/Widgets/WBP_MoneycostUI.OutputMoneyCostOnHit` (`self.InputMoneyCost`) _aswbp_moneycost_ui)
  ;[1 1 1] Setting location for the UI to travel between
  (set `self.StartTransform` (`KismetMathLibrary.MakeTransform` _returnvalue))
  (set `self.EndTransform` (`KismetMathLibrary.MakeTransform` (+ _returnvalue (`KismetMathLibrary.MakeVector` (`KismetMathLibrary.RandomFloatInRange` -3000.0 3000.0) (`KismetMathLibrary.RandomFloatInRange` -3000.0 3000.0) (`KismetMathLibrary.RandomFloatInRange` 1000.0 2000.0)))))
  ;[1 1 1] Moving the actor across its path before destroying it
  (bind (_direction _move_track) (`Timeline|MoveT` :!via `PlayFromStart`)
    (:`Update`
      (`self.K2_SetActorTransform` (`KismetMathLibrary.TLerp` (`self.StartTransform`) (`self.EndTransform`) _move_track)))
    (:`Finished`
      (`WidgetComponent.SetTickMode` (`self.MoneyWidget`) "Disabled")
      (`self.K2_DestroyActor`))))

(fn `UserConstructionScript`)