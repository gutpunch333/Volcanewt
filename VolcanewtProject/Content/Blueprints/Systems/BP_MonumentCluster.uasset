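; Monument cluster actor that awards a one-time destruction bonus when its little statues are destroyed.
; On BeginPlay it caches the Volcanewt game mode and collects every BP_LittleStatue in the level.
; LittleMonumentDestroyed removes the reported statue and tracks a remaining index in BuildingLeft.
; When that index is zero, it adds a bonus share of the level's monetary value to the game mode's destroyed total and HUD.
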(event `self.ReceiveBeginPlay`
  (`parent.ReceiveBeginPlay`)
  (bind _asbpgm_volcanewt (cast `/Game/Blueprints/Systems/BPGM_Volcanewt` (`GameplayStatics.GetGameMode`)))
  (set `self.As BPGM Volcanewt` _asbpgm_volcanewt)
  (bind _outactors (`GameplayStatics.GetAllActorsOfClass` "/Game/Blueprints/Building_Blueprints/BP_LittleStatue.BP_LittleStatue_C"))
  (for _array_element _outactors
    (`KismetArrayLibrary.Array_Add` (`self.AllLittleMonuments`) _array_element)))

(event `LittleMonumentDestroyed`
  (params (NewParam :type "/Game/Blueprints/Building_Blueprints/BP_LittleStatue Object Reference"))
  (bind _as_bpgm_volcanewt (`self.As BPGM Volcanewt`))
  (for (_array_element _array_index) (`self.AllLittleMonuments`)
    ;[1 1 1] Checks for the little monument ref in the array. Changes the 'building left' value to a non-zero number if it is not the building ref
    (if (== _array_element NewParam)
      (`KismetArrayLibrary.Array_Remove` (`self.AllLittleMonuments`) _array_index)
      (else
        (set `self.Building Left` _array_index))))
  ;[1 1 1] Checks if there are no buildings left. The index 0 is empty thus cannot be removed
  (if (and (== (`self.Building Left`) 0) (`self.Bonus Avaiable`))
    (set `self.Bonus Avaiable` false)
    (bind _output_get (set `/Game/Blueprints/Systems/BPGM_Volcanewt.LevelMonetaryValueDestroyed` (+ (* (`/Game/Blueprints/Systems/BPGM_Volcanewt.LevelMonetaryValue` _as_bpgm_volcanewt) 0.08) (`/Game/Blueprints/Systems/BPGM_Volcanewt.LevelMonetaryValueDestroyed` _as_bpgm_volcanewt)) _as_bpgm_volcanewt))
    (set `/Game/UI/Widgets/WBP_HUD.LevelDestroyedMonetaryValue` _output_get (`/Game/Blueprints/Systems/BPGM_Volcanewt.HUDWidget Ref` _as_bpgm_volcanewt))
    (`KismetSystemLibrary.PrintString` "Cluster Gone" true true (struct :`R` 1.0 :`G` 0.008924 :`A` 1.0) 20.0)))

(fn `UserConstructionScript`)