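; Game instance that persists the player's gamma and master, music and SFX volume settings across sessions.
; On Init it loads BP_SettingsSaveGame from its slot, or creates and saves one, then copies the values and applies them.
; ApplySettings pushes sound mix class overrides for volume and sends gamma, remapped by Lerp, as a console command.
; SaveSettings writes the current values back to the slot.
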(event `self.ReceiveInit`
  (`self.Load Settings`))

(fn `ApplySettings`
  (`KismetSystemLibrary.PrintString` "apply settings function")
  (`GameplayStatics.SetSoundMixClassOverride` "/Game/Audio/MixClasses/Mix_Master.Mix_Master" "/Engine/EngineSounds/Master.Master" (`self.MasterVolumeVal`) 1.0 0.0)
  (`GameplayStatics.PushSoundMixModifier` "/Game/Audio/MixClasses/Mix_Master.Mix_Master")
  (`GameplayStatics.SetSoundMixClassOverride` "/Game/Audio/MixClasses/Mix_Music.Mix_Music" "/Engine/EngineSounds/Music.Music" (`self.MusicVolumeVal`) 1.0 0.0)
  (`GameplayStatics.PushSoundMixModifier` "/Game/Audio/MixClasses/Mix_Music.Mix_Music")
  (`GameplayStatics.SetSoundMixClassOverride` "/Game/Audio/MixClasses/Mix_SFX.Mix_SFX" "/Engine/EngineSounds/SFX.SFX" (`self.SFXVolumeVal`) 1.0 0.0)
  (`GameplayStatics.PushSoundMixModifier` "/Game/Audio/MixClasses/Mix_SFX.Mix_SFX")
  (`KismetSystemLibrary.ExecuteConsoleCommand` (`KismetStringLibrary.Concat_StrStr` "Gamma " (`KismetStringLibrary.Conv_DoubleToString` (`KismetMathLibrary.Lerp` 0.0 4.4 (`self.GammaSettingVal`)))) null))

(fn `Load Settings`
  (`KismetSystemLibrary.PrintString` "load settings function")
  (bind _returnvalue (`GameplayStatics.DoesSaveGameExist` (`self.SettingsSaveGameName`)))
  (if _returnvalue
    (bind _returnvalue_2 (`GameplayStatics.LoadGameFromSlot` (`self.SettingsSaveGameName`)))
    (bind _asbp_settings_save_game (cast `/Game/Blueprints/BP_SettingsSaveGame` _returnvalue_2))
    (set `self.SettingsSaveGameRef` _asbp_settings_save_game)
    (else
      (bind _returnvalue_3 (`GameplayStatics.CreateSaveGameObject` "/Game/Blueprints/BP_SettingsSaveGame.BP_SettingsSaveGame_C"))
      (`GameplayStatics.SaveGameToSlot` _returnvalue_3 (`self.SettingsSaveGameName`))
      (set `self.SettingsSaveGameRef` _returnvalue_3)))
  (set `self.GammaSettingVal` (`/Game/Blueprints/BP_SettingsSaveGame.SavedGammaSetting` (`self.SettingsSaveGameRef`)))
  (set `self.MasterVolumeVal` (`/Game/Blueprints/BP_SettingsSaveGame.SavedMasterVolume` (`self.SettingsSaveGameRef`)))
  (set `self.MusicVolumeVal` (`/Game/Blueprints/BP_SettingsSaveGame.SavedMusicVolume` (`self.SettingsSaveGameRef`)))
  (set `self.SFXVolumeVal` (`/Game/Blueprints/BP_SettingsSaveGame.SavedSFXVolume` (`self.SettingsSaveGameRef`)))
  (`self.ApplySettings`))

(fn `SaveSettings`
  (`KismetSystemLibrary.PrintString` "save settings function")
  (`/Engine/EditorBlueprintResources/StandardMacros.IsValid` (`self.SettingsSaveGameRef`)
    (:`Is Valid`
      (set `/Game/Blueprints/BP_SettingsSaveGame.SavedGammaSetting` (`self.GammaSettingVal`) (`self.SettingsSaveGameRef`))
      (set `/Game/Blueprints/BP_SettingsSaveGame.SavedMasterVolume` (`self.MasterVolumeVal`) (`self.SettingsSaveGameRef`))
      (set `/Game/Blueprints/BP_SettingsSaveGame.SavedMusicVolume` (`self.MusicVolumeVal`) (`self.SettingsSaveGameRef`))
      (set `/Game/Blueprints/BP_SettingsSaveGame.SavedSFXVolume` (`self.SFXVolumeVal`) (`self.SettingsSaveGameRef`))
      (`GameplayStatics.SaveGameToSlot` (`self.SettingsSaveGameRef`) (`self.SettingsSaveGameName`)))
    (:`Is Not Valid`
      (`KismetSystemLibrary.PrintString` "No settings save file bruv"))))