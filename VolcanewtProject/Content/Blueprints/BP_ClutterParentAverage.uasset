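; BP_ClutterParentAverage is a destructible clutter actor that breaks apart when the player pawn overlaps it.
; The construction script adds one static mesh instance at the actor's transform as the intact, overlap-detecting mesh.
; On player overlap it destroys that mesh, enables physics on GCComponent, crumbles its cluster and destroys the actor after a delay.
; The one-shot Destroyed flag is set before the player check, so any first overlap consumes it.
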(event `self.ReceiveAnyDamage`
  (params (Damage :type "Float (single-precision)") (DamageType :type "DamageType Object Reference") (InstigatedBy :type "Controller Object Reference") (DamageCauser :type "Actor Object Reference")))

(event `self.InstancedStaticMesh.OnComponentBeginOverlap`
  (params (OverlappedComponent :type "PrimitiveComponent Object Reference") (OtherActor :type "Actor Object Reference") (OtherComp :type "PrimitiveComponent Object Reference") (OtherBodyIndex :type Integer) (bFromSweep :type Boolean) (SweepResult :type "HitResult Structure (by ref)"))
  (if (not (`self.Destroyed`))
    (set `self.Destroyed` true)
    (if (== OtherActor (`GameplayStatics.GetPlayerPawn` 0))
      (`PrimitiveComponent.SetSimulatePhysics` (`self.GC_Component`) true)
      (`ActorComponent.K2_DestroyComponent` (`self.InstancedStaticMesh`))
      (`GeometryCollectionComponent.CrumbleCluster` (`self.GC_Component`) 1)
      (`KismetSystemLibrary.Delay` 5.0)
      (`self.K2_DestroyActor`))))

(fn `UserConstructionScript`
  (`InstancedStaticMeshComponent.AddInstance` (`self.InstancedStaticMesh`) (`self.GetTransform`) true))