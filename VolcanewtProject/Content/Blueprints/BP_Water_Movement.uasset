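; BP_Water_Movement is a water volume that blocks ground spawning in Volcanewt while the newt is inside it.
; It caches the game mode on BeginPlay.
; Box overlaps with components tagged NewtDamagedCollider clear the game mode's CanSpawnGround flag on entry and restore it on exit.
; The player slowdown described by the graph comments is disconnected, so walk speed stays unchanged.
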(event `self.ReceiveBeginPlay`
  (bind _asbpgm_volcanewt (cast `/Game/Blueprints/Systems/BPGM_Volcanewt` (`GameplayStatics.GetGameMode`))))

(event `self.Box.OnComponentBeginOverlap`
  (params (OverlappedComponent :type "PrimitiveComponent Object Reference") (OtherActor :type "Actor Object Reference") (OtherComp :type "PrimitiveComponent Object Reference") (OtherBodyIndex :type Integer) (bFromSweep :type Boolean) (SweepResult :type "HitResult Structure (by ref)"))
  ;[1 1 1] Decrease player speed on water
  (if (`ActorComponent.ComponentHasTag` OtherComp "NewtDamagedCollider")
    (set `/Game/Blueprints/Systems/BPGM_Volcanewt.CanSpawnGround?` false (stale `self.ReceiveBeginPlay` _asbpgm_volcanewt))))

(event `self.Box.OnComponentEndOverlap`
  (params (OverlappedComponent :type "PrimitiveComponent Object Reference") (OtherActor :type "Actor Object Reference") (OtherComp :type "PrimitiveComponent Object Reference") (OtherBodyIndex :type Integer))
  ;[1 1 1] Return player speed to normal
  (if (`ActorComponent.ComponentHasTag` OtherComp "NewtDamagedCollider")
    (set `/Game/Blueprints/Systems/BPGM_Volcanewt.CanSpawnGround?` true (stale `self.ReceiveBeginPlay` _asbpgm_volcanewt))))

(fn `UserConstructionScript`)