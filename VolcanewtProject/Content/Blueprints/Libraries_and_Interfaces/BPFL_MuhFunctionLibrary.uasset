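; Blueprint function library of shared helpers for actor searches, enemy despawning, effects and visibility checks.
; FindNearestActorOfClass scans every actor of a class for the closest to a location, a costly operation.
; FindIfEnemyTooFar destroys an enemy at or beyond the despawn distance from player 0's pawn.
; Other helpers spawn a scaled Niagara system at an actor and test line of sight with a Visibility-channel multi line trace.
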(fn `FindIfEnemyTooFar`
  (params (EnemyRef :type "Actor Object Reference"))
  (returns (EnemyWasDestroyed :type Boolean))
  (locals (DespawnEnemyDistance :type "Float (double-precision)" :default 150000.0) (LocalEnemyRef :type "Actor Object Reference") (EnemyTooFar :type Boolean))
  ;[1 1 1] Finding distance between player and enemy location. If the difference is greater than 2000, destroy the enemy
  (bind _output_get (set `local.LocalEnemyRef` EnemyRef))
  (`/Engine/EditorBlueprintResources/StandardMacros.IsValid` _output_get
    (:`Is Valid`
      (bind _output_get_2 (set `local.EnemyTooFar` (>= (`KismetMathLibrary.VSize` (- (`Actor.K2_GetActorLocation` (`GameplayStatics.GetPlayerPawn` null)) (`Actor.K2_GetActorLocation` _output_get))) (`local.DespawnEnemyDistance`))))
      (if _output_get_2
        (`KismetSystemLibrary.PrintString` null "Enemy Too Far")
        (`Actor.K2_DestroyActor` (`local.LocalEnemyRef`))
        (return (`local.EnemyTooFar`))))))

(fn `FindNearestActorOfClass`
  (params (Class :type "Actor Class Reference") (TargetLocation :type "Vector Structure"))
  (returns (NearestDistance :type "Float (double-precision)") (NearestActor :type "Actor Object Reference"))
  (locals (Loc_NearestDistance :type "Float (double-precision)" :default 1000000000.0) (Loc_NearestActor :type "Actor Object Reference"))
  ;[1 1 1] Getting all actors of a class, expensive
  (bind _outactors (`GameplayStatics.GetAllActorsOfClass` null Class))
  ;[1 1 1] For every instance of this actor type in the scene, checking the distance between the input location and each actor.
  (for _array_element _outactors
    (bind _returnvalue (`KismetMathLibrary.Vector_Distance` (`Actor.K2_GetActorLocation` _array_element) (`local.TargetLocation`)))
    ;[1 1 1] If the distance from each actor is less than any prior one, the local nearest distance and actor are saved
    (if (< _returnvalue (`local.Loc_NearestDistance`))
      (set `local.Loc_NearestDistance` _returnvalue)
      (set `local.Loc_NearestActor` _array_element)))
  ;[1 1 1] Once every actor's distance has been checked, save the nearest and return
  (return (`local.Loc_NearestDistance`) (`local.Loc_NearestActor`)))

(fn `HasLineOfSight`
  (params (From :type "Vector Structure") (To :type "Vector Structure") (ActorsToIgnore :type "Array of Actor Object Reference (by ref)"))
  (returns (Result :type Boolean))
  ;[1 1 1] Checks if object has line of sight, returns true if line trace doesn't hit anything
  (bind (_outhits _returnvalue) (`KismetSystemLibrary.LineTraceMulti` null From To "TraceTypeQuery1" false ActorsToIgnore "None" false))
  (return (not _returnvalue)))

(fn `SpawnNiagaraAtActor`
  (params (ActorActivatedOn :type "Actor Object Reference") (ChosenParticle :type "NiagaraSystem Object Reference"))
  (`NiagaraFunctionLibrary.SpawnSystemAtLocation` null ChosenParticle (`Actor.K2_GetActorLocation` ActorActivatedOn) (struct) (8.0 8.0 1.0)))