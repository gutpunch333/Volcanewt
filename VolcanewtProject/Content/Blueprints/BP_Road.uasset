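; BP_Road is a spline road that moves a reference point along its length and tracks whether a bus occupies it.
; Tick advances distance by road speed, matches the point's location and rotation to the spline, and wraps when looping.
; Binding a bus marks the road occupied until that bus is destroyed.
; Spline mesh generation exists in the construction script graph but is disconnected, so no meshes are built.
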(event `BindBus&Road`
  (params (BoundBus :type "/Game/Enemies/BP_Bus Object Reference"))
  (add `self.OnDestroyed` BoundBus (delegate `ClearBoundBus`))
  (set `self.BusAlreadyOnRoad` true))

(event `ClearBoundBus` :!signature `self.OnDestroyed`
  (params (DestroyedActor :type "Actor Object Reference"))
  (set `self.BusAlreadyOnRoad` false))

(event `self.ReceiveTick`
  (params (DeltaSeconds :type "Float (single-precision)"))
  (bind (_returnvalue_location _returnvalue_rotation) (`KismetMathLibrary.BreakTransform` (`SplineComponent.GetTransformAtDistanceAlongSpline` (`self.Spline`) (`self.Distance`) "Local" false)))
  (set `self.Distance` (+ (* DeltaSeconds (`self.RoadSpeed`)) (`self.Distance`)))
  (`SceneComponent.K2_SetRelativeTransform` (`self.Reference Point`) (`KismetMathLibrary.MakeTransform` _returnvalue_location _returnvalue_rotation (`SceneComponent.RelativeScale3D` (`self.Reference Point`))) false false)
  (if (`self.IsLooping?`)
    (if (> (`self.Distance`) (`SplineComponent.GetSplineLength` (`self.Spline`)))
      (set `self.Distance` 0.0))))

(fn `UserConstructionScript`)