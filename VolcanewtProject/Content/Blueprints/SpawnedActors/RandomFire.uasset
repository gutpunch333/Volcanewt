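; RandomFire is a spawned fire hazard that damages overlapping actors and can spread nearby.
; BeginPlay activates its VFX and sets a looping timer, which clears itself on the first tick.
; That tick damages capsule overlaps not tagged Newt or Fire, or enables capsule gravity if nothing overlaps.
; With overlaps and spreading enabled, a percentage roll spawns another RandomFire at a random XY offset, passing on its settings.
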(event `FireReadyToTick`
  (bind _random_x_direction_distance (`self.Random X Direction Distance`))
  (bind _random_y_direction_distance (`self.Random Y Direction Distance`))
  (bind _overlappingactors (`PrimitiveComponent.GetOverlappingActors` (`self.Capsule`) null))
  (bind _returnvalue (`SceneComponent.K2_GetComponentToWorld` (`self.Capsule`)))
  (if (> (`KismetArrayLibrary.Array_Length` _overlappingactors) 0)
    (for _array_element _overlappingactors
      (if (`self.ActorHasTag` "Newt")
        _
        (elif (not (`self.ActorHasTag` "Fire"))
          (`GameplayStatics.ApplyDamage` _array_element (`self.FireDamagePerTick`) null self))))
    (if (`self.FireSpreads`)
      (if (<= (`KismetMathLibrary.RandomIntegerInRange` 1 100) (`self.Fire Chance To Spread`))
        (`|SpawnActorFromClass` "RandomFire_C" (`KismetMathLibrary.MakeTransform` (`KismetMathLibrary.MakeVector` (+ (.x (.location _returnvalue)) (`KismetMathLibrary.RandomFloatInRange` (* _random_x_direction_distance -1.0) _random_x_direction_distance)) (+ (.y (.location _returnvalue)) (`KismetMathLibrary.RandomFloatInRange` (* _random_y_direction_distance -1.0) _random_y_direction_distance)) (.z (.location _returnvalue))) (.rotation _returnvalue) (.scale _returnvalue)) "Undefined" "MultiplyWithRoot" null (`self.FireSpreads`) (`self.FireDamagePerTick`) (`self.Fire Tick Rate`) (`self.Fire Chance To Spread`) null)))
    (else
      (`PrimitiveComponent.SetEnableGravity` (`self.Capsule`) true)))
  (`KismetSystemLibrary.K2_ClearAndInvalidateTimerHandle` (stale `self.ReceiveBeginPlay` _returnvalue)))

(event `self.ReceiveBeginPlay`
  (`ActorComponent.SetActive` (`self.ChargeFX`) true true) ; FIRE TRAIL VFX
  (bind _returnvalue (`KismetSystemLibrary.K2_SetTimerDelegate` (delegate `FireReadyToTick`) (`self.Fire Tick Rate`) true)))

(fn `UserConstructionScript`)