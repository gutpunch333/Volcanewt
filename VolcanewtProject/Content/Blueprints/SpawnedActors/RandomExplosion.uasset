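; RandomExplosion is a spawned explosion actor that deals a one-time burst of damage when play begins.
; It damages each actor overlapping its Capsule, gated by checks on its own tags for neither "Newt" nor "Explosion".
; It then spawns a Niagara effect and plays a sound at the capsule's transform.
; Random X/Y offset calculations are present but unused, so the explosion position is not randomized here.
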(event `self.ReceiveBeginPlay`
  (bind _overlappingactors (`PrimitiveComponent.GetOverlappingActors` (`self.Capsule`) null))
  (bind (_returnvalue_location _returnvalue_rotation _returnvalue_scale) (`KismetMathLibrary.BreakTransform` (`SceneComponent.K2_GetComponentToWorld` (`self.Capsule`))))
  (if (> (`KismetArrayLibrary.Array_Length` _overlappingactors) 0)
    (for _array_element _overlappingactors
      (if (`self.ActorHasTag` "Newt")
        _
        (elif (not (`self.ActorHasTag` "Explosion"))
          (`GameplayStatics.ApplyDamage` _array_element (`self.DamageOfExplosion`) null self)))))
  (`NiagaraFunctionLibrary.SpawnSystemAtLocation` (`self.ExplosionNiagara`) _returnvalue_location _returnvalue_rotation _returnvalue_scale)
  (`GameplayStatics.PlaySoundAtLocation` (`self.ExplosionSfx`) _returnvalue_location _returnvalue_rotation 1.0 1.0 0.0 null null null null))

(fn `UserConstructionScript`)