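; Parent Blueprint for destructible buildings in Volcanewt that take damage, shake, collapse and report their monetary value to the game mode.
; Hits above small fractions of total health trigger a timeline shake and a money UI spawner, while damage reduces health and spawns Niagara effects.
; At zero health it removes the static mesh, crumbles the physics-simulated geometry collection with sound, then optionally fades its dynamic materials before destroying itself.
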(event `ShakeBuilding`
  ;[1 0.7696 0.2474 1 26] Handles Building Shake
  (`TimelineComponent.SetLooping` (`self.ShakeTimeline`) true)
  (switch `int` (`KismetMathLibrary.RandomInteger` 1)
    (:`0`
      (bind (_direction _shakevector) (`Timeline|ShakeTimeline` :!via `PlayFromStart` :!label _label)
        (:`Update`
          (`self.K2_SetActorLocation` (+ _shakevector (`self.ActorStartingLocaton`)) false true)
          (`KismetSystemLibrary.Delay` (`self.shakeTime`))
          (`TimelineComponent.SetLooping` (`self.ShakeTimeline`) false))
        (:`Finished`
          (`self.K2_SetActorLocation` (`self.ActorStartingLocaton`) false true))))
    (:`1`
      (goto _label :!via `ReverseFromEnd`))))

(event `self.ReceiveBeginPlay`
  (set `self.TotalHealth` (`self.Current Health`))
  (bind _asbpgm_volcanewt (cast `/Game/Blueprints/Systems/BPGM_Volcanewt` (`GameplayStatics.GetGameMode`)))
  (set `self.As BPGM Volcanewt_0` _asbpgm_volcanewt)
  (set `self.ActorStartingLocaton` (`self.K2_GetActorLocation`)))

(event `self.ReceiveAnyDamage`
  (params (Damage :type "Float (single-precision)") (DamageType :type "DamageType Object Reference") (InstigatedBy :type "Controller Object Reference") (DamageCauser :type "Actor Object Reference"))
  (bind _current_health (`self.Current Health`))
  (bind _gc_component (`self.GC_Component`))
  (bind _returnvalue (<= _current_health 0.0))
  ;[1 1 1] Checking damage percent to shake building or not
  (set `self.damageTaken` Damage)
  (if (> (/ (`self.damageTaken`) (`self.TotalHealth`)) 0.05)
    (`self.ShakeBuilding`) ; skip if too low damage
    ;[1 1 1] Checks if the building has any health, if above 0 itlll do damage stuff
    (`self.SpawnMoneyUI`) ; skip if too low damage
  )
  (if (not _returnvalue)
    (set `self.Current Health` (- _current_health (`self.damageTaken`)))
    (`/Game/Blueprints/Libraries_and_Interfaces/BPFL_MuhFunctionLibrary.SpawnNiagaraAtActor` self "/Game/VFX/Effects/FXS_BuildingDamage.FXS_BuildingDamage")
    (if _returnvalue
      (`/Game/Blueprints/Systems/BPGM_Volcanewt.BuildingDestroyed` (`self.As BPGM Volcanewt_0`) (`self.MonetaryValue`) self)
      (`ActorComponent.K2_DestroyComponent` (`self.Static Mesh Component`))
      ;[1 1 1] Sets physics to mesh and breaks apart the separate geometry mesh
      (`PrimitiveComponent.SetLightingChannels` (`self.GC_Component`) false true false)
      (`PrimitiveComponent.SetSimulatePhysics` _gc_component true)
      (`GeometryCollectionComponent.CrumbleCluster` _gc_component 0)
      (`GeometryCollectionComponent.CrumbleCluster` _gc_component 1)
      ;[1 1 1] Sound :)
      (`GameplayStatics.PlaySoundAtLocation` (`self.Destuction SFX`) (`self.K2_GetActorLocation`) (struct) 1.0 1.0 0.0 null null null null)
      (if (`self.Fade Out`)
        (`KismetSystemLibrary.Delay` 1.0)
        ;[1 1 1] Lerping the dynamic materials' parameter values to fade the building out
        (bind (_direction _fadealpha) (`Timeline|Timeline` :!via `PlayFromStart`)
          (:`Update`
            (bind _returnvalue_2 (`KismetMathLibrary.Lerp` 1.0 0.0 _fadealpha))
            (`MaterialInstanceDynamic.SetScalarParameterValue` (`self.DynamicMaterialInstanceIndex1`) "fadeOut" _returnvalue_2)
            (`MaterialInstanceDynamic.SetScalarParameterValue` (`self.DynamicMaterialInstanceIndex0`) "fadeOut" _returnvalue_2))
          (:`Finished`
            (`KismetSystemLibrary.Delay` 0.5)
            (`self.K2_DestroyActor`)))))))

(event `SpawnMoneyUI`
  (bind _returnvalue_location (`KismetMathLibrary.BreakTransform` (`self.GetTransform`)))
  (bind _damagetaken (`self.damageTaken`))
  ;[1 1 1] Spawn Money UI
  (if (>= _damagetaken (* (`self.TotalHealth`) 0.08))
    (`|SpawnActorFromClass` "/Game/Blueprints/Systems/BP_MoneyUISpawner.BP_MoneyUISpawner_C" (`KismetMathLibrary.MakeTransform` (+ _returnvalue_location (0.0 0.0 10.0))) "AlwaysSpawn" "MultiplyWithRoot" null (`self.MonetaryValue`) (`KismetMathLibrary.FTrunc` _damagetaken) (`KismetMathLibrary.FTrunc` (`self.TotalHealth`)) (`KismetMathLibrary.FTrunc` (`self.Current Health`)) null)))

(fn `UserConstructionScript`
  (bind _max_health (`self.Max Health`))
  (bind _gc_component (`self.GC_Component`))
  (bind _returnvalue (`PrimitiveComponent.CreateDynamicMaterialInstance` _gc_component 1 (`self.Source Material`) "None"))
  (set `self.DynamicMaterialInstanceIndex1` _returnvalue)
  (bind _returnvalue_2 (`PrimitiveComponent.CreateDynamicMaterialInstance` _gc_component 0 (`self.Source Material_0`) "None"))
  (set `self.DynamicMaterialInstanceIndex0` _returnvalue_2)
  (set `self.Current Health` _max_health)
  (set `self.TotalHealth` _max_health))