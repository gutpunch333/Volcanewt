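; Deep water hazard volume that repeatedly damages actors while they overlap its Box.
; Begin overlap adds the actor to a duplicate-free DrowningActors array, and a looping one-second timer applies heavy damage to every entry.
; End overlap removes the actor and clears DrowningTimer once the array is empty.
; The timer start guard checks DamageTimer while the handle is stored in DrowningTimer, so the two do not match.
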(event `self.ReceiveBeginPlay`)

(event `self.Box.OnComponentBeginOverlap`
  (params (OverlappedComponent :type "PrimitiveComponent Object Reference") (OtherActor :type "Actor Object Reference") (OtherComp :type "PrimitiveComponent Object Reference") (OtherBodyIndex :type Integer) (bFromSweep :type Boolean) (SweepResult :type "HitResult Structure (by ref)"))
  ;[1 1 1] Adds actor to array of actors to be damaged on timer. Does not add actor if already in list
  (set `self.Drowning Actor` OtherActor)
  (for _array_element (`self.Drowning Actors`)
    (if (== _array_element (`self.Drowning Actor`))
      (set `self.In List` true)
      (break)))
  (if (`self.In List`)
    (set `self.In List` false)
    (else
      (`KismetArrayLibrary.Array_Add` (`self.Drowning Actors`) (`self.Drowning Actor`))))
  ;[1 1 1] Starts a damage timer if one is not active when an actor enters the zone.
  (if (not (`KismetSystemLibrary.K2_IsValidTimerHandle` (`self.Damage Timer`)))
    (bind _returnvalue (`KismetSystemLibrary.K2_SetTimerDelegate` (delegate `Drowning`) 1.0 true))
    (set `self.Drowning Timer` _returnvalue)))

(event `Drowning`
  ;[1 1 1] Damages all actors in array on timer
  (for _array_element (`self.Drowning Actors`)
    (`GameplayStatics.ApplyDamage` _array_element 100.0)
    (`KismetSystemLibrary.PrintString` "Hello")))

(event `self.Box.OnComponentEndOverlap`
  (params (OverlappedComponent :type "PrimitiveComponent Object Reference") (OtherActor :type "Actor Object Reference") (OtherComp :type "PrimitiveComponent Object Reference") (OtherBodyIndex :type Integer))
  (bind _drowning_actors (`self.Drowning Actors`))
  ;[1 1 1] Removes actor from array if empty and disables the timer if no actors are left to be damaged
  (`KismetArrayLibrary.Array_RemoveItem` _drowning_actors OtherActor)
  (if (not (`KismetArrayLibrary.Array_IsNotEmpty` _drowning_actors))
    (`KismetSystemLibrary.K2_ClearAndInvalidateTimerHandle` (`self.Drowning Timer`))))

(fn `UserConstructionScript`)