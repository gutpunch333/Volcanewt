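; BP_TruckParent is a parent Blueprint for vehicle props that the player can flatten.
; The Construction Script picks a random mesh from an array and rolls a random MonetaryValue, so both can change whenever construction reruns.
; When the player pawn begins overlapping the mesh, the root is squashed vertically and physics simulation is enabled on the mesh.
; MonetaryValue is only set here, not read.
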(event `self.StaticMesh.OnComponentBeginOverlap`
  (params (OverlappedComponent :type "PrimitiveComponent Object Reference") (OtherActor :type "Actor Object Reference") (OtherComp :type "PrimitiveComponent Object Reference") (OtherBodyIndex :type Integer) (bFromSweep :type Boolean) (SweepResult :type "HitResult Structure (by ref)"))
  (if (== OtherActor (`GameplayStatics.GetPlayerPawn` 0))
    (`SceneComponent.SetWorldScale3D` (`self.DefaultSceneRoot`) (1.0 1.0 0.25))
    (`PrimitiveComponent.SetSimulatePhysics` (`self.StaticMesh`) true)))

(fn `UserConstructionScript`
  ;[1 1 1] Selects a random small vehicle static mesh and spawns it with the static mesh
  (`StaticMeshComponent.SetStaticMesh` (`self.StaticMesh`) (`|GetArrayItem` (`self.Static Mesh`) (`KismetMathLibrary.RandomInteger` 3)))
  ;[1 1 1] Sets a random value for the car
  (set `self.Monetary Value` (`KismetMathLibrary.RandomIntegerInRange` 5000 20000)))