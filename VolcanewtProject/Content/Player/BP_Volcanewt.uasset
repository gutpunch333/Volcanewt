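; Player character Volcanewt, which moves, jumps, shakes the camera on landing and attacks small buildings.
; Enhanced Input drives camera-relative movement, jumping and invertible pitch look, with horizontal look left disconnected.
; A and D set held flags that Tick turns into controller yaw input, computed from current actor yaw plus a small offset.
; Attack applies damage to every BP_SmallBuilding overlapping Box1 and prints its name.
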(event `self.ReceiveBeginPlay`
  (bind _returnvalue (pcsubsystem `EnhancedInputLocalPlayerSubsystem` (`GameplayStatics.GetPlayerController` 0)))
  (`/Engine/EditorBlueprintResources/StandardMacros.IsValid` _returnvalue
    (:`Is Valid`
      (`EnhancedInputSubsystemInterface.AddMappingContext` _returnvalue "/Game/Player/IMC_ThirdPerson.IMC_ThirdPerson" 0 (struct)))))

(event `self.OnLanded`
  (params (Hit :type "HitResult Structure (by ref)"))
  (`GameplayStatics.PlayWorldCameraShake` "/Game/Player/jumpShakeMatinee.jumpShakeMatinee_C" (`self.K2_GetActorLocation`) 0.0 333333.0))

(event `EnhancedInput|/Game/Player/INP_Jump`
  (params (ActionValue :type Boolean) (ElapsedSeconds :type "Float (double-precision)") (TriggeredSeconds :type "Float (double-precision)") (InputAction :type "InputAction Object Reference" :default "/Game/Player/INP_Jump.INP_Jump"))
  (:`Started`
    (`self.Jump`))
  (:`Completed`
    (`self.StopJumping`)))

(event `EnhancedInput|/Game/Player/INP_MoveAround`
  (params (ActionValue :type "Vector2D Structure") (ElapsedSeconds :type "Float (double-precision)") (TriggeredSeconds :type "Float (double-precision)") (InputAction :type "InputAction Object Reference" :default "/Game/Player/INP_MoveAround.INP_MoveAround"))
  (bind (_returnvalue_roll _returnvalue_pitch _returnvalue_yaw) (`KismetMathLibrary.BreakRotator` (`self.GetControlRotation`)))
  (:`Triggered`
    (`self.AddMovementInput` (`KismetMathLibrary.GetRightVector` (`self.GetControlRotation`)) ActionValue_X)
    (`self.AddMovementInput` (`KismetMathLibrary.GetForwardVector` (`KismetMathLibrary.MakeRotator` _returnvalue_roll 0.0 _returnvalue_yaw)) ActionValue_Y)))

(event `EnhancedInput|/Game/Player/INP_LookAround`
  (params (ActionValue :type "Vector2D Structure") (ElapsedSeconds :type "Float (double-precision)") (TriggeredSeconds :type "Float (double-precision)") (InputAction :type "InputAction Object Reference" :default "/Game/Player/INP_LookAround.INP_LookAround"))
  (:`Triggered`
    (`self.AddControllerPitchInput` (* ActionValue_Y (`KismetMathLibrary.SelectFloat` -1.0 1.0 (`self.InvertCameraY`))))))

(event `self.Box1.OnComponentBeginOverlap`
  (params (OverlappedComponent :type "PrimitiveComponent Object Reference") (OtherActor :type "Actor Object Reference") (OtherComp :type "PrimitiveComponent Object Reference") (OtherBodyIndex :type Integer) (bFromSweep :type Boolean) (SweepResult :type "HitResult Structure (by ref)")))

(event `EnhancedInput|/Game/Player/INP_Attack`
  (params (ActionValue :type Boolean) (ElapsedSeconds :type "Float (double-precision)") (TriggeredSeconds :type "Float (double-precision)") (InputAction :type "InputAction Object Reference" :default "/Game/Player/INP_Attack.INP_Attack"))
  (:`Started`
    (for _array_element (`PrimitiveComponent.GetOverlappingActors` (`self.Box1`) "/Game/Blueprints/BP_SmallBuilding.BP_SmallBuilding_C")
      (`GameplayStatics.ApplyDamage` _array_element 25.0)
      (`KismetSystemLibrary.PrintString` (`KismetSystemLibrary.GetDisplayName` _array_element)))))

(event `Key|A`
  (params (Key :type "Key Structure"))
  (:`Pressed`
    (set `self.A Key is Down` true))
  (:`Released`
    (set `self.A Key is Down` false)))

(event `Key|D`
  (params (Key :type "Key Structure"))
  (:`Pressed`
    (set `self.D Key is Down` true))
  (:`Released`
    (set `self.D Key is Down` false)))

(event `self.ReceiveTick`
  (params (DeltaSeconds :type "Float (single-precision)"))
  (bind (_returnvalue_roll _returnvalue_pitch _returnvalue_yaw) (`KismetMathLibrary.BreakRotator` (`self.K2_GetActorRotation`)))
  (`|ExecutionSequence`
    (:`then_0`
      (if (`self.A Key is Down`)
        (`self.AddControllerYawInput` (+ _returnvalue_yaw -0.1))))
    (:`then_1`
      (if (`self.D Key is Down`)
        (`self.AddControllerYawInput` (+ _returnvalue_yaw 0.1))))))

(fn `UserConstructionScript`)