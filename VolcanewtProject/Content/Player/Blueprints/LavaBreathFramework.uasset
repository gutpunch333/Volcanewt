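; Lava breath smoke hazard actor that activates its smoke effect on BeginPlay and deals damage to actors inside its capsule.
; A timer set to loop calls the damage pass, which checks for a "Newt" tag on the smoke actor itself rather than on each overlapping actor.
; That pass then clears the timer, so damage runs only once.
; A random spawn-chance check is present but unconnected.
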(event `SmokeReadyToTick`
  (bind _overlappingactors (`PrimitiveComponent.GetOverlappingActors` (`self.Capsule1`) null))
  (if (> (`KismetArrayLibrary.Array_Length` _overlappingactors) 0)
    (for _array_element _overlappingactors
      (if (`self.ActorHasTag` "Newt")
        (`GameplayStatics.ApplyDamage` _array_element (`self.SmokeDamagePerTick`) null self))))
  (`KismetSystemLibrary.K2_ClearAndInvalidateTimerHandle` (stale `self.ReceiveBeginPlay` _returnvalue)))

(event `self.ReceiveBeginPlay`
  (`ActorComponent.SetActive` (`self.SmokeFx`) true true)
  (bind _returnvalue (`KismetSystemLibrary.K2_SetTimerDelegate` (delegate `SmokeReadyToTick`) (`self.Smoke Tick Rate`) true)))

(fn `UserConstructionScript`)